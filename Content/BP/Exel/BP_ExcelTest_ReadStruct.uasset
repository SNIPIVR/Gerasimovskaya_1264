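; Test Blueprint that loads Tables/GameData.xlsx from the content directory on BeginPlay, prints its active sheet and watches it for changes.
; It sets a first-row/column header table format, and each change triggers RefreshActors.
; RefreshActors loops over sheet rows with an empty body; the struct-read logic that would update tagged actors' transforms is disconnected.
; BeginPlay also creates a separate workbook and saves it with an empty path.
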(event `self.ReceiveBeginPlay`
  (bind _returnvalue (`KismetStringLibrary.Concat_StrStr` "" "Tables/GameData.xlsx"))
  (`KismetSystemLibrary.PrintString` _returnvalue true true (struct :`G` 0.66 :`B` 1.0 :`A` 1.0) 20.0)
  (bind _returnvalue_2 (`DirectExcelLibrary.LoadExcel` _returnvalue "ProjectContentDir"))
  (bind _output_get (set `self.Workbook` _returnvalue_2))
  (bind _returnvalue_3 (`DirectExcelLibrary.CreateExcel`))
  (`DirectExcelLibrary.SaveExcel` _returnvalue_3)
  (`/Engine/EditorBlueprintResources/StandardMacros.IsValid` _output_get
    (:`Is Valid`
      (`|ExecutionSequence`
        (:`then_0`
          (`KismetSystemLibrary.PrintString` "LoadExcel Succeed!" true true (struct :`G` 0.66 :`B` 1.0 :`A` 1.0) 20.0)
          (`ExcelWorksheet.Print` (`ExcelWorkbook.ActiveSheet` (`self.Workbook`)) true (struct :`G` 0.66 :`B` 1.0 :`A` 1.0) 2.0)
          (`KismetSystemLibrary.PrintString` "Hello"))
        (:`then_1`
          (`ExcelWorksheet.SetTableFormat` (`ExcelWorkbook.ActiveSheet` (`self.Workbook`)) "TableWithFirstRowColumnHeader"))
        (:`then_2`
          (`self.RefreshActors`)
          (`ExcelWorkbook.StartWatch` (`self.Workbook`) (delegate `OnExcelChanged`) "ReloadWithOriginalTableHeaders" 1.0))))
    (:`Is Not Valid`
      (`KismetSystemLibrary.PrintString` "FailedOpen" true true (struct :`G` 0.66 :`B` 1.0 :`A` 1.0) 20.0))))

(event `OnExcelChanged`
  (params (workbook :type "ExcelWorkbook Object Reference"))
  (`self.RefreshActors`)
  (`KismetSystemLibrary.PrintString` "Excel Changed" true true (struct :`G` 0.66 :`B` 1.0 :`A` 1.0) 5.0))

(event `RefreshActors`
  (bind _returnvalue (`ExcelWorkbook.SheetAt` (`self.Workbook`) 0))
  (for _index (range (+ (`ExcelWorksheet.LowestRow` _returnvalue) 1) (+ (`ExcelWorksheet.HighestRow` _returnvalue) 1))
    _))

(fn `UserConstructionScript`)