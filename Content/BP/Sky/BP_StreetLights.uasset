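; BP_StreetLights is a street light actor whose spotlight switches on and off in response to lighting events from the game state.
; On BeginPlay it casts the game state to BP_CustomGameState, stores it and binds handlers to its LightsOn and LightsOff events.
; The handlers set the SpotLight intensity to NewIntensity for on and zero for off, so the light needs no Tick polling.
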(event `self.ReceiveBeginPlay`
  (bind _asbp_custom_game_state (cast `/Game/BP/Sky/BP_CustomGameState` (`GameplayStatics.GetGameState`)))
  (set `self.GameState` _asbp_custom_game_state)
  (add `/Game/BP/Sky/BP_CustomGameState.LightsOn` (`self.GameState`) (delegate `LightsOn`))
  (add `/Game/BP/Sky/BP_CustomGameState.LightsOff` (`self.GameState`) (delegate `LightsOff`)))

(event `LightsOff`
  (`LightComponent.SetIntensity` (`self.SpotLight`) 0.0))

(event `LightsOn`
  (`LightComponent.SetIntensity` (`self.SpotLight`) (`self.New Intensity`)))

(fn `UserConstructionScript`)