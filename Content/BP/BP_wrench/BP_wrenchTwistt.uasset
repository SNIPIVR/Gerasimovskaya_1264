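; BP_wrenchTwistt is a wrench that a motion controller can grab and twist.
; Grab stores the controller as the Hand if it is within the Sphere's radius, and Release clears it when that same controller lets go.
; While held, Tick takes the look-at pitch from hand to wrench, clamps it, and applies it as the wrench's world roll, keeping pitch and yaw.
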(event `self.ReceiveTick`
  (params (DeltaSeconds :type "Float (single-precision)"))
  (bind _hand (`self.Hand`))
  (bind _wrench (`self.Wrench`))
  (bind (_returnvalue_roll _returnvalue_pitch _returnvalue_yaw) (`KismetMathLibrary.BreakRotator` (`SceneComponent.K2_GetComponentRotation` _wrench)))
  (bind (_returnvalue_roll_2 _returnvalue_pitch_2) (`KismetMathLibrary.BreakRotator` (`KismetMathLibrary.FindLookAtRotation` (`SceneComponent.K2_GetComponentLocation` _hand) (`SceneComponent.K2_GetComponentLocation` _wrench))))
  ;[1 1 1] Set door rotate
  (`/Engine/EditorBlueprintResources/StandardMacros.IsValid` _hand
    (:`Is Valid`
      (`SceneComponent.K2_SetWorldRotation` _wrench (`KismetMathLibrary.MakeRotator` (`KismetMathLibrary.ClampAngle` _returnvalue_pitch_2 1.0 180.0) _returnvalue_pitch _returnvalue_yaw) false false))))

(event `/Game/BP/Door/BP_Grap.Release`
  (params (MotionController :type "MotionControllerComponent Object Reference"))
  (if (== MotionController (`self.Hand`))
    (set `self.Hand` null)))

(event `/Game/BP/Door/BP_Grap.Grab`
  (params (MotionController :type "MotionControllerComponent Object Reference"))
  (bind _sphere (`self.Sphere`))
  (if (== (`SceneComponent.K2_GetComponentLocation` MotionController) (`SceneComponent.K2_GetComponentLocation` _sphere) :`ErrorTolerance` (`SphereComponent.SphereRadius` _sphere))
    (set `self.Hand` MotionController)))

(fn `UserConstructionScript`)