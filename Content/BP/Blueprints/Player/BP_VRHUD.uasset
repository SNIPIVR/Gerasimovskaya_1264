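; VR HUD actor that floats an object info screen (WBP_ObjectInfoScreen) around the player, filled in through InitWidget.
; Each tick it follows the pawn camera in X/Y at its own height.
; When camera yaw drifts too far, a Gate runs an interpolated lazy turn until nearly aligned or a roll limit is hit.
; A timeline scales the widget open, and plays faster in reverse on close before destroying the actor.
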(event `self.ReceiveBeginPlay`
  (`TimelineComponent.SetPlayRate` (`self.Open/HideWidgetAnimTimeline`) (/ 1.0 0.3))
  (bind _asvrpawn (cast `/Game/VRTemplate/Blueprints/VRPawn` (`GameplayStatics.GetPlayerPawn` 0)))
  (set `self.VivePawnOwner` _asvrpawn))

(event `StartRotation`
  (bind _returnvalue_roll (`KismetMathLibrary.BreakRotator` (`self.K2_GetActorRotation`)))
  (bind (_returnvalue_roll_2 _returnvalue_pitch _returnvalue_yaw) (`KismetMathLibrary.BreakRotator` (`self.K2_GetActorRotation`)))
  (bind (_returnvalue_roll_3 _returnvalue_pitch_2 _returnvalue_yaw_2) (`KismetMathLibrary.BreakRotator` (`KismetMathLibrary.RInterpTo` (`self.K2_GetActorRotation`) (`SceneComponent.RelativeRotation` (`/Game/VRTemplate/Blueprints/VRPawn.Camera` (`self.VivePawnOwner`))) (`GameplayStatics.GetWorldDeltaSeconds`) 4.0)))
  (goto _label :!via `Open`))

(event `self.ReceiveTick`
  (params (DeltaSeconds :type "Float (single-precision)"))
  (bind _returnvalue_roll (`KismetMathLibrary.BreakRotator` (`self.K2_GetActorRotation`)))
  (bind (_returnvalue_x _returnvalue_y _returnvalue_z) (`KismetMathLibrary.BreakVector` (`self.K2_GetActorLocation`)))
  (bind (_returnvalue_roll_2 _returnvalue_pitch _returnvalue_yaw) (`KismetMathLibrary.BreakRotator` (`self.K2_GetActorRotation`)))
  (bind (_returnvalue_x_2 _returnvalue_y_2) (`KismetMathLibrary.BreakVector` (`SceneComponent.K2_GetComponentLocation` (`/Game/VRTemplate/Blueprints/VRPawn.Camera` (`self.VivePawnOwner`)))))
  (bind (_returnvalue_roll_3 _returnvalue_pitch_2 _returnvalue_yaw_2) (`KismetMathLibrary.BreakRotator` (`KismetMathLibrary.NormalizedDeltaRotator` (`SceneComponent.RelativeRotation` (`/Game/VRTemplate/Blueprints/VRPawn.Camera` (`self.VivePawnOwner`))) (`self.K2_GetActorRotation`))))
  (bind (_returnvalue_roll_4 _returnvalue_pitch_3 _returnvalue_yaw_3) (`KismetMathLibrary.BreakRotator` (`KismetMathLibrary.RInterpTo` (`self.K2_GetActorRotation`) (`SceneComponent.RelativeRotation` (`/Game/VRTemplate/Blueprints/VRPawn.Camera` (`self.VivePawnOwner`))) (`GameplayStatics.GetWorldDeltaSeconds`) 4.0)))
  (`/Engine/EditorBlueprintResources/StandardMacros.IsValid` (`self.VivePawnOwner`)
    (:`Is Valid`
      (`|ExecutionSequence`
        (:`then_0`
          (`/Engine/EditorBlueprintResources/StandardMacros.Gate` true :!label _label
            (:`Exit`
              (if (`KismetMathLibrary.NearlyEqual_FloatFloat` _returnvalue_roll 10.0 0.3)
                (`self.StopRotation` :!label _label_2)
                (set `self.bInRotation` false)
                (`KismetSystemLibrary.Delay` 0.5)
                (`self.K2_SetActorRotation` (`KismetMathLibrary.MakeRotator` 0.0 _returnvalue_pitch _returnvalue_yaw))
                (elif (`KismetMathLibrary.NearlyEqual_FloatFloat` _returnvalue_roll -10.0 0.3)
                  (goto _label_2)
                  (else
                    (`self.K2_SetActorRotation` (`KismetMathLibrary.MakeRotator` _returnvalue_roll_4 0.0 _returnvalue_yaw_3))
                    (if (== (`self.K2_GetActorRotation`) (`SceneComponent.RelativeRotation` (`/Game/VRTemplate/Blueprints/VRPawn.Camera` (`self.VivePawnOwner`))) :`ErrorTolerance` 5.0)
                      (`self.StopRotation`)
                      (set `self.bInRotation` false))))))))
        (:`then_1`
          (if (and (> (`KismetMathLibrary.Abs` _returnvalue_yaw_2) 25.0) (not (`self.bInRotation`)))
            (`self.StartRotation`)
            (set `self.bInRotation` true)))
        (:`then_2`
          (`self.K2_SetActorLocation` (`KismetMathLibrary.MakeVector` _returnvalue_x_2 _returnvalue_y_2 _returnvalue_z)))))))

(event `StopRotation`
  (goto _label :!via `Close`))

(event `PlayOpenAnim`
  (set `self.bOpen` true)
  (bind (_direction _alpha) (`Timeline|Open/HideWidgetAnimTimeline` :!via `PlayFromStart` :!label _label_3)
    (:`Update`
      (`SceneComponent.SetRelativeScale3D` (`self.Widget`) (`KismetMathLibrary.VLerp` (0.0 0.0 0.0) (0.035 0.035 0.035) _alpha)))
    (:`Finished`
      (if (not (`self.bOpen`))
        (`self.K2_DestroyActor`)))))

(event `PlayCloseAnim`
  (`TimelineComponent.SetPlayRate` (`self.Open/HideWidgetAnimTimeline`) (/ 1.0 0.1))
  (set `self.bOpen` false)
  (goto _label_3 :!via `ReverseFromEnd`))

(event `OnCloseButtonPressed`
  (`self.PlayCloseAnim`))

(fn `InitWidget`
  (params (VivePawn :type "/Game/VRTemplate/Blueprints/VRPawn Object Reference") (ObjectInfo :type "/Game/BP/Blueprints/Game/S_MirnayaObjectInfo Structure") (ID :type String))
  (set `self.VivePawnOwner` VivePawn)
  (set `self.ObjectInfo` ObjectInfo)
  (bind _aswbp_object_info_screen (cast `/Game/BP/Blueprints/UI/WBP_ObjectInfoScreen` (`WidgetComponent.GetUserWidgetObject` (`self.Widget`))))
  (`/Game/BP/Blueprints/UI/WBP_ObjectInfoScreen.ShowInfo` _aswbp_object_info_screen (`self.ObjectInfo`) ID)
  (`self.PlayOpenAnim`)
  (add `/Game/BP/Blueprints/UI/WBP_ObjectInfoScreen.ExitButtonPressed` _aswbp_object_info_screen (`|CreateDelegate` :!event `OnCloseButtonPressed`)))

(fn `UserConstructionScript`)