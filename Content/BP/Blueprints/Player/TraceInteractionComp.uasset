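; Player scene component that finds the interactable actor it points at and triggers interaction with it.
; Every tick it line traces far along its forward vector on the Visibility channel, ignoring its owner.
; The hit actor is stored as CurrentActor only if it implements the ITraceInteraction interface; otherwise the reference is cleared.
; StartInteract sends the interface's start-interact message to that actor when it is valid.
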(event `self.ReceiveTick`
  (params (DeltaSeconds :type "Float (single-precision)"))
  (bind _returnvalue (`self.K2_GetComponentLocation`))
  (bind (_outhit _returnvalue_2) (`KismetSystemLibrary.LineTraceSingle` _returnvalue (+ _returnvalue (* (`self.GetForwardVector`) 100000.0)) "TraceTypeQuery1" false (`|MakeArray` (`self.GetOwner`))))
  (if _returnvalue_2
    (bind (_bblockinghit _binitialoverlap _time _distance _location _impactpoint _normal _impactnormal _physmat _hitactor) (`GameplayStatics.BreakHitResult` _outhit))
    (if (`KismetSystemLibrary.DoesImplementInterface` _hitactor "/Game/Blueprints/Player/ITraceInteraction.ITraceInteraction_C")
      (set `self.CurrentActor` _hitactor)
      (else
        (set `self.CurrentActor` null :!label _label)))
    (else
      (goto _label))))

(event `StartInteract`
  (bind _currentactor (`self.CurrentActor`))
  (`/Engine/EditorBlueprintResources/StandardMacros.IsValid` _currentactor
    (:`Is Valid`
      (message `/Game/Blueprints/Player/ITraceInteraction.StartInteract` _currentactor))))