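; Blueprint function library for Mirnaya VR with a lookup that returns an object's info struct by ID.
; It gates on a DT_Objects row named by the ID, then searches a parsed JSON "Objects" array for the matching id and copies name, description, parameter and file name strings.
; The parser receives the literal "1" and the row data is unused.
; Failed parses, keys and searches display error messages.
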(fn `GetMirnayaObjectInfoByID`
  (params (ID :type String))
  (returns (ObjectInfo :type "/Game/BP/Blueprints/Game/S_MirnayaObjectInfo Structure") (bFind :type Boolean))
  (locals (L_FindedObject :type "LowEntryJsonObject Object Reference") (VivePawnOwner :type "/Game/VRTemplate/Blueprints/VRPawn Object Reference") (L_ObjectInfo :type "/Game/BP/Blueprints/Game/S_MirnayaObjectInfo Structure"))
  (`|GetDataTableRow` "/Game/BP/Blueprints/Utils/DT_Objects.DT_Objects" (`KismetStringLibrary.Conv_StringToName` ID)
    (:`then`
      (bind _returnjsonobjectvalue (`LowEntryJsonLibrary.Json_ParseJsonString` "1")
        (:`FoundObject`
          (bind _element (`/LowEntryJson/Blueprints/LowEntryJsonMacros.JsonArrayForEachLoopWithBreak` (`LowEntryJsonLibrary.Object_GetAsJsonArrayOrDefault` _returnjsonobjectvalue "Objects") :!label _label)
            (:`LoopBody`
              (bind _returnvalue (`LowEntryJsonLibrary.Value_GetAsJsonObjectOrDefault` _element))
              (bind _returnvalue_2 (`LowEntryJsonLibrary.Object_GetString` _returnvalue "id")
                (:`Success`
                  (if (`KismetStringLibrary.EqualEqual_StrStr` _returnvalue_2 (`local.ID`))
                    (set `local.L_FindedObject` _returnvalue)
                    (goto _label :!via `Break`)))
                (:`NotFound`
                  (`/Game/BP/Blueprints/Utils/BML_MirnayaVR.DisplayMessage` true "Cant Find ID Key in JSON Object"))
                (:`WrongType`
                  (`/Game/BP/Blueprints/Utils/BML_MirnayaVR.DisplayMessage` true "Wrong Type of Value In ID Key"))))
            (:`Completed`
              (`/Engine/EditorBlueprintResources/StandardMacros.IsValid` (`local.L_FindedObject`)
                (:`Is Valid`
                  (`|ExecutionSequence`
                    (:`then_0`
                      (bind _returnvalue_3 (`LowEntryJsonLibrary.Object_GetString` (`local.L_FindedObject`) "ObjectName")
                        (:`Success`
                          (setmembers `/Game/BP/Blueprints/Game/S_MirnayaObjectInfo` :`StructRef` (`local.L_ObjectInfo`) :`ObjectName` _returnvalue_3 :`ObjectDescription` "" :`ObjectParamsNames` "" :`ObjectParamsValues` "" :`FileName` ""))
                        (:`NotFound`
                          (`/Game/BP/Blueprints/Utils/BML_MirnayaVR.DisplayMessage` true "Cant Find ObjectName Key in JSON Object"))
                        (:`WrongType`
                          (`/Game/BP/Blueprints/Utils/BML_MirnayaVR.DisplayMessage` true "Wrong Type of Value In ObjectName Key"))))
                    (:`then_1`
                      (bind _returnvalue_4 (`LowEntryJsonLibrary.Object_GetString` (`local.L_FindedObject`) "ObjectDescription")
                        (:`Success`
                          (setmembers `/Game/BP/Blueprints/Game/S_MirnayaObjectInfo` :`StructRef` (`local.L_ObjectInfo`) :`ObjectName` "" :`ObjectDescription` _returnvalue_4 :`ObjectParamsNames` "" :`ObjectParamsValues` "" :`FileName` ""))
                        (:`NotFound`
                          (`/Game/BP/Blueprints/Utils/BML_MirnayaVR.DisplayMessage` true "Cant Find ObjectDescription Key in JSON Object"))
                        (:`WrongType`
                          (`/Game/BP/Blueprints/Utils/BML_MirnayaVR.DisplayMessage` true "Wrong Type of Value In ObjectDescription Key"))))
                    (:`then_2`
                      (bind _returnvalue_5 (`LowEntryJsonLibrary.Object_GetString` (`local.L_FindedObject`) "ObjectParamsNames")
                        (:`Success`
                          (setmembers `/Game/BP/Blueprints/Game/S_MirnayaObjectInfo` :`StructRef` (`local.L_ObjectInfo`) :`ObjectName` "" :`ObjectDescription` "" :`ObjectParamsNames` _returnvalue_5 :`ObjectParamsValues` "" :`FileName` ""))
                        (:`NotFound`
                          (`/Game/BP/Blueprints/Utils/BML_MirnayaVR.DisplayMessage` true "Cant Find ObjectParamsNames Key in JSON Object"))
                        (:`WrongType`
                          (`/Game/BP/Blueprints/Utils/BML_MirnayaVR.DisplayMessage` true "Wrong Type of Value In ObjectParamsNames Key"))))
                    (:`then_3`
                      (bind _returnvalue_6 (`LowEntryJsonLibrary.Object_GetString` (`local.L_FindedObject`) "ObjectParamsValues")
                        (:`Success`
                          (setmembers `/Game/BP/Blueprints/Game/S_MirnayaObjectInfo` :`StructRef` (`local.L_ObjectInfo`) :`ObjectName` "" :`ObjectDescription` "" :`ObjectParamsNames` "" :`ObjectParamsValues` _returnvalue_6 :`FileName` ""))
                        (:`NotFound`
                          (`/Game/BP/Blueprints/Utils/BML_MirnayaVR.DisplayMessage` true "Cant Find ObjectParamsValues Key in JSON Object"))
                        (:`WrongType`
                          (`/Game/BP/Blueprints/Utils/BML_MirnayaVR.DisplayMessage` true "Wrong Type of Value In ObjectParamsValues Key"))))
                    (:`then_4`
                      (bind _returnvalue_7 (`LowEntryJsonLibrary.Object_GetString` (`local.L_FindedObject`) "FileName")
                        (:`Success`
                          (setmembers `/Game/BP/Blueprints/Game/S_MirnayaObjectInfo` :`StructRef` (`local.L_ObjectInfo`) :`ObjectName` "" :`ObjectDescription` "" :`ObjectParamsNames` "" :`ObjectParamsValues` "" :`FileName` _returnvalue_7))
                        (:`NotFound`
                          (`/Game/BP/Blueprints/Utils/BML_MirnayaVR.DisplayMessage` true "Cant Find FileName Key in JSON Object"))
                        (:`WrongType`
                          (`/Game/BP/Blueprints/Utils/BML_MirnayaVR.DisplayMessage` true "Wrong Type of Value In FileName Key"))))
                    (:`then_5`
                      (return (`local.L_ObjectInfo`) true))))
                (:`Is Not Valid`
                  (`/Game/BP/Blueprints/Utils/BML_MirnayaVR.DisplayMessage` true "Cant Find Object By ID")
                  (return (struct) false))))))
        (:`StringIsEmpty`
          (`/Game/BP/Blueprints/Utils/BML_MirnayaVR.DisplayMessage` true "JSON String Is Empty"))
        (:`UnableToParse`
          (`/Game/BP/Blueprints/Utils/BML_MirnayaVR.DisplayMessage` true "Unable to Parse JSON String"))))))