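; BP_AnimatedObject is a world object that opens and closes by playing animations, driven by an electrical state from buttons.
; CurrentStateChange maps a true state to Open and a false state to Close, each playing its non-looping animation on Anim01.
; InAnimation and Open flags gate the calls, with a delay matching the animation length before the state updates.
; State changes arriving mid-animation are ignored rather than queued.
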(event `Open`
  (bind _openanim (`self.OpenAnim`))
  ;[1 1 1] Play Open/Close Animation
  (if (and (not (`self.bInAnimation`)) (not (`self.bOpen`)))
    (set `self.bInAnimation` true)
    (`SkeletalMeshComponent.PlayAnimation` (`self.Anim_01`) _openanim false)
    (`KismetSystemLibrary.Delay` (`AnimSequenceBase.SequenceLength` _openanim))
    (set `self.bInAnimation` false)
    (set `self.bOpen` true)))

(event `Close`
  (bind _closeanim (`self.CloseAnim`))
  ;[1 1 1] Play Open/Close Animation
  (if (and (not (`self.bInAnimation`)) (`self.bOpen`))
    (set `self.bInAnimation` true)
    (`SkeletalMeshComponent.PlayAnimation` (`self.Anim_01`) _closeanim false)
    (`KismetSystemLibrary.Delay` (`AnimSequenceBase.SequenceLength` _closeanim))
    (set `self.bInAnimation` false)
    (set `self.bOpen` false)))

(event `/Game/VRExpansion/Vive/Testing/Button/ElectricalObject.CurrentStateChange`
  (params (CurrentProvider :type "Object Object Reference") (ElectricalState :type Boolean) (CurrentFlow :type "Float (single-precision)"))
  ;[1 1 1] Events from buttons
  (if ElectricalState
    (`self.Open`)
    (else
      (`self.Close`))))

(fn `UserConstructionScript`)