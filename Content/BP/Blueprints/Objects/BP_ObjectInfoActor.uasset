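; BP_ObjectInfoActor is a VR trigger object that shows information about itself when something begins overlapping its static mesh.
; The overlap plays the close animation on any open BP_VRHUD actors, then looks up its ID in DT_Objects, displaying an error if missing.
; A found row spawns a new BP_VRHUD using the camera's relative X/Y and the pawn's Z, initialized with the pawn, row and ID.
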(event `self.ReceiveBeginPlay`
  (bind _asvrpawn (cast `/Game/VRTemplate/Blueprints/VRPawn` (`GameplayStatics.GetPlayerPawn` 0)))
  (set `self.Vive Pawn` _asvrpawn))

(event `self.StaticMesh.OnComponentBeginOverlap`
  (params (OverlappedComponent :type "PrimitiveComponent Object Reference") (OtherActor :type "Actor Object Reference") (OtherComp :type "PrimitiveComponent Object Reference") (OtherBodyIndex :type Integer) (bFromSweep :type Boolean) (SweepResult :type "HitResult Structure (by ref)"))
  (bind _id (`self.ID`))
  (bind _id_2 (`self.ID`))
  (bind _vive_pawn (`self.Vive Pawn`))
  (bind (_returnvalue_x _returnvalue_y _returnvalue_z) (`KismetMathLibrary.BreakVector` (`self.K2_GetActorLocation` _vive_pawn)))
  (bind (_relativelocation_x _relativelocation_y) (`KismetMathLibrary.BreakVector` (`SceneComponent.RelativeLocation` (`/Game/VRTemplate/Blueprints/VRPawn.Camera` _vive_pawn))))
  ;[1 1 1] Open object information in user interface
  (set `self.isHit?` (`.bInitialOverlap` (`GameplayStatics.BreakHitResult` SweepResult)))
  ;;[1 1 1] Close other widget with information
  (bind _outactors (`GameplayStatics.GetAllActorsOfClass` "/Game/BP/Blueprints/Player/BP_VRHUD.BP_VRHUD_C"))
  (if (> (`KismetArrayLibrary.Array_Length` _outactors) 0)
    (for _array_element _outactors
      (`/Game/BP/Blueprints/Player/BP_VRHUD.PlayCloseAnim` _array_element))
    ;;[1 1 1] Load and open new information
    (`KismetSystemLibrary.Delay` 0.1))
  (`|GetDataTableRow` "/Game/BP/Blueprints/Utils/DT_Objects.DT_Objects" (`KismetStringLibrary.Conv_StringToName` _id_2)
    (:`then`
      (bind _returnvalue (`|SpawnActorFromClass` "/Game/BP/Blueprints/Player/BP_VRHUD.BP_VRHUD_C" (`KismetMathLibrary.MakeTransform` (`KismetMathLibrary.MakeVector` _relativelocation_x _relativelocation_y _returnvalue_z)) "AlwaysSpawn" "OverrideRootScale" null null))
      (set `self.Hud_Info` _returnvalue)
      (bind _asvrpawn (cast `/Game/VRTemplate/Blueprints/VRPawn` (`GameplayStatics.GetPlayerPawn` 0)))
      (bind _returnvalue_2 (`|GetDataTableRow` "/Game/BP/Blueprints/Utils/DT_Objects.DT_Objects" (`KismetStringLibrary.Conv_StringToName` _id))
        (:`then`
          (`/Game/BP/Blueprints/Player/BP_VRHUD.InitWidget` (`self.Hud_Info`) _asvrpawn _returnvalue_2 _id))))
    (:`RowNotFound`
      (`/Game/BP/Blueprints/Utils/BML_MirnayaVR.DisplayMessage` true (`KismetStringLibrary.Concat_StrStr` "Object with ID: " _id_2 " dont found")))))

(fn `UserConstructionScript`)