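; Base interactable button actor whose empty OnButtonPress function serves as the hook for what a press does.
; StartInteract calls OnButtonPress and plays a timeline that lerps ButtonComp a short distance along its local X axis, with the play rate set on BeginPlay.
; ButtonComp's OnButtonStateChanged event also calls OnButtonPress, without playing the animation.
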(event `self.ReceiveBeginPlay`
  (`TimelineComponent.SetPlayRate` (`self.PressAnimTimeline`) (/ 1.0 0.3)))

(event `self.ButtonComp.OnButtonStateChanged`
  (params (ButtonState :type Boolean) (InteractingActor :type "Actor Object Reference") (InteractingComponent :type "PrimitiveComponent Object Reference"))
  (`self.OnButtonPress`))

(event `/Game/Blueprints/Player/ITraceInteraction.StartInteract`
  (`self.OnButtonPress`)
  (bind (_direction _alpha) (`Timeline|PressAnimTimeline` :!via `PlayFromStart`)
    (:`Update`
      (`SceneComponent.K2_SetRelativeLocation` (`self.ButtonComp`) (`KismetMathLibrary.VLerp` (0.0 0.0 0.0) (-1.5 0.0 0.0) _alpha) false false))))

(fn `OnButtonPress`)

(fn `UserConstructionScript`)