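; Scaffold door Blueprint that a motion controller can grab and swing when unlocked.
; Grab stores the controller as Hand if it is within the HandCollision sphere, and Release clears it.
; On Tick, the held door takes its world yaw from a hand-to-door look-at, clamped between -90 and 0 degrees.
; With no hand, a delayed reset snaps the door to zero rotation if its yaw is within tolerance.
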(event `self.ReceiveTick`
  (params (DeltaSeconds :type "Float (single-precision)"))
  (bind _hand (`self.Hand`))
  (bind _door (`self.Door`))
  (bind (_returnvalue_roll _returnvalue_pitch _returnvalue_yaw) (`KismetMathLibrary.BreakRotator` (`SceneComponent.K2_GetComponentRotation` _door)))
  (bind (_returnvalue_roll_2 _returnvalue_pitch_2 _returnvalue_yaw_2) (`KismetMathLibrary.BreakRotator` (`KismetMathLibrary.FindLookAtRotation` (`SceneComponent.K2_GetComponentLocation` _hand) (`SceneComponent.K2_GetComponentLocation` _door))))
  (`|ExecutionSequence`
    (:`then_1`
      ;[1 1 1] Set door rotate
      (if (not (`self.Locked`))
        (`/Engine/EditorBlueprintResources/StandardMacros.IsValid` _hand
          (:`Is Valid`
            (`SceneComponent.K2_SetWorldRotation` _door (`KismetMathLibrary.MakeRotator` 0.0 0.0 (`KismetMathLibrary.ClampAngle` (- _returnvalue_yaw_2 0.0) -90.0)) false false))
          (:`Is Not Valid`
            (if (`KismetMathLibrary.NearlyEqual_FloatFloat` _returnvalue_yaw 0.0 90.0)
              (`KismetSystemLibrary.Delay` 30.0)
              (`SceneComponent.K2_SetWorldRotation` :`self` _door))))))))

(event `/Game/BP/Door/BP_Grap.Release`
  (params (MotionController :type "MotionControllerComponent Object Reference"))
  (if (== MotionController (`self.Hand`))
    (set `self.Hand` null)))

(event `/Game/BP/Door/BP_Grap.Grab`
  (params (MotionController :type "MotionControllerComponent Object Reference"))
  (bind _handcollision (`self.HandCollision`))
  (if (== (`SceneComponent.K2_GetComponentLocation` MotionController) (`SceneComponent.K2_GetComponentLocation` _handcollision) :`ErrorTolerance` (`SphereComponent.SphereRadius` _handcollision))
    (set `self.Hand` MotionController)))

(fn `UserConstructionScript`)