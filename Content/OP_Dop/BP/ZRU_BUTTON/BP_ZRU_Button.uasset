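; BP_ZRU_Button is a colored push-button actor that animates when something overlaps its Button component.
; An overlap presses it and releases it after half a second, with the Botton_switch timeline playing and reversing to slide the component along local X.
; Tick also sets a random pressed state through a repeating one-second delay.
; The construction script applies ButtonColor through a dynamic material instance.
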(event `button_pressed`
  (params (On :type Boolean))
  (if On
    (bind (_direction _sw_graph) (`Timeline|Botton_switch` :!label _label)
      (:`Update`
        (`SceneComponent.K2_SetRelativeLocation` (`self.Button`) (`KismetMathLibrary.MakeVector` (`KismetMathLibrary.Lerp` _sw_graph (`KismetMathLibrary.Conv_BoolToDouble` On))) false false)))
    (else
      (goto _label :!via `Reverse`))))

(event `self.ReceiveTick`
  (params (DeltaSeconds :type "Float (single-precision)"))
  (`KismetSystemLibrary.Delay` 1.0)
  (`self.button_pressed` (`KismetMathLibrary.RandomBool`)))

(event `Button_SW`
  (`self.button_pressed` true)
  (`KismetSystemLibrary.Delay` 0.5)
  (`self.button_pressed` false))

(event `self.Button.OnComponentBeginOverlap`
  (params (OverlappedComponent :type "PrimitiveComponent Object Reference") (OtherActor :type "Actor Object Reference") (OtherComp :type "PrimitiveComponent Object Reference") (OtherBodyIndex :type Integer) (bFromSweep :type Boolean) (SweepResult :type "HitResult Structure (by ref)"))
  (`self.Button_SW`))

(fn `UserConstructionScript`
  (bind _returnvalue (`PrimitiveComponent.CreateDynamicMaterialInstance` (`self.Button`) 0 null "None"))
  (`MaterialInstanceDynamic.SetVectorParameterValue` _returnvalue "Param" (`self.Button Color`)))