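; Two-lamp LED indicator, apparently for ZRU switchgear, showing one of three work positions: disconnected (both grey), control position (green), or working position (red).
; The construction script creates dynamic material instances on two material slots of the LED body and applies the current position, so it previews in the editor.
; SetColor drives each lamp's Color and Emissive parameters, and is rerun on BeginPlay and through the Switch_work_position event.
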(event `self.ReceiveBeginPlay`
  (`self.Switch_work_position` (`self.Work_Position`)))

(event `self.ReceiveTick`
  (params (DeltaSeconds :type "Float (single-precision)")))

(event `Switch_work_position`
  (params (Work_position :type "/Game/OP_Dop/BP/ZRU_LED_SW/E_WORK_POSITION Enum" :default "NewEnumerator0"))
  (`self.Set_Color` Work_position))

(fn `Set_Color`
  (params (position :type "/Game/OP_Dop/BP/ZRU_LED_SW/E_WORK_POSITION Enum" :default "NewEnumerator0"))
  (bind _led_1 (`self.LED_1`))
  (bind _led_2 (`self.LED_2`))
  (bind _led_2_2 (`self.LED_2`))
  (bind _led_1_2 (`self.LED_1`))
  (switch `/Game/OP_Dop/BP/ZRU_LED_SW/E_WORK_POSITION` position
    (:`NewEnumerator0`
      (`MaterialInstanceDynamic.SetVectorParameterValue` _led_1_2 "Color" (struct :`R` 0.401042 :`G` 0.401042 :`B` 0.401042 :`A` 1.0))
      (`MaterialInstanceDynamic.SetScalarParameterValue` _led_1 "Emissive" 0.0)
      (`MaterialInstanceDynamic.SetVectorParameterValue` _led_2 "Color" (struct :`R` 0.401042 :`G` 0.401042 :`B` 0.401042 :`A` 1.0))
      (`MaterialInstanceDynamic.SetScalarParameterValue` _led_2_2 "Emissive" 0.0))
    (:`NewEnumerator1`
      (`MaterialInstanceDynamic.SetVectorParameterValue` _led_1_2 "Color" (struct :`G` 0.395833 :`B` 0.003296))
      (`MaterialInstanceDynamic.SetScalarParameterValue` _led_1 "Emissive" 1.0)
      (`MaterialInstanceDynamic.SetVectorParameterValue` _led_2 "Color" (struct :`R` 0.401042 :`G` 0.401042 :`B` 0.401042 :`A` 1.0))
      (`MaterialInstanceDynamic.SetScalarParameterValue` _led_2_2 "Emissive" 0.0))
    (:`NewEnumerator2`
      (`MaterialInstanceDynamic.SetVectorParameterValue` _led_1_2 "Color" (struct :`R` 0.401042 :`G` 0.401042 :`B` 0.401042 :`A` 1.0))
      (`MaterialInstanceDynamic.SetScalarParameterValue` _led_1 "Emissive" 0.0)
      (`MaterialInstanceDynamic.SetVectorParameterValue` _led_2 "Color" (struct :`R` 0.8 :`G` 0.003922))
      (`MaterialInstanceDynamic.SetScalarParameterValue` _led_2_2 "Emissive" 1.0))))

(fn `UserConstructionScript`
  (locals (NewLocalVar_0 :type "LinearColor Structure" :default (struct :`R` 0.684896 :`G` 0.684896 :`B` 0.684896)))
  (bind _led_body_0 (`self.LED_Body_0`))
  (bind _returnvalue (`PrimitiveComponent.CreateDynamicMaterialInstance` _led_body_0 2 null "None"))
  (set `self.LED_1` _returnvalue)
  (bind _returnvalue_2 (`PrimitiveComponent.CreateDynamicMaterialInstance` _led_body_0 3 null "None"))
  (set `self.LED_2` _returnvalue_2)
  (`self.Set_Color` (`self.Work_Position`)))