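; Switchgear LED indicator Blueprint (BP_ZRU_LED_GND) that displays a work position: off (grey), control (green) or working (red).
; The construction script creates a dynamic material on the LED body and applies the current position.
; Set_Color maps each position to color and emissive parameters, glowing only for green and red.
; BeginPlay and the Switch_work_position event refresh it, while an unconnected delayed randomizer never runs.
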(event `self.ReceiveTick`
  (params (DeltaSeconds :type "Float (single-precision)")))

(event `self.ReceiveBeginPlay`
  (`self.Switch_work_position` (`self.Work_Position`)))

(event `Switch_work_position`
  (params (Work_position :type "/Game/OP_Dop/BP/ZRU_LED_SW/E_WORK_POSITION Enum" :default "NewEnumerator0"))
  (`self.Set_Color` Work_position))

(fn `Set_Color`
  (params (Posirion :type "/Game/OP_Dop/BP/ZRU_LED_SW/E_WORK_POSITION Enum" :default "NewEnumerator0"))
  (bind _color_work_position (`self.Color_work_position`))
  (bind _color_work_position_2 (`self.Color_work_position`))
  (switch `/Game/OP_Dop/BP/ZRU_LED_SW/E_WORK_POSITION` Posirion
    (:`NewEnumerator0`
      (`MaterialInstanceDynamic.SetVectorParameterValue` _color_work_position "Color" (struct :`R` 0.401042 :`G` 0.401042 :`B` 0.401042 :`A` 1.0))
      (`MaterialInstanceDynamic.SetScalarParameterValue` _color_work_position_2 "Emissive" 0.0))
    (:`NewEnumerator1`
      (`MaterialInstanceDynamic.SetVectorParameterValue` _color_work_position "Color" (struct :`G` 0.395833 :`B` 0.003296))
      (`MaterialInstanceDynamic.SetScalarParameterValue` _color_work_position_2 "Emissive" 1.0 :!label _label))
    (:`NewEnumerator2`
      (`MaterialInstanceDynamic.SetVectorParameterValue` _color_work_position "Color" (struct :`R` 0.8 :`G` 0.003922))
      (goto _label))))

(fn `UserConstructionScript`
  (locals (NewLocalVar_0 :type "LinearColor Structure" :default (struct :`R` 0.684896 :`G` 0.684896 :`B` 0.684896)))
  (bind _returnvalue (`PrimitiveComponent.CreateDynamicMaterialInstance` (`self.LED_Body_0`) 2 null "None"))
  (set `self.Color_work_position` _returnvalue)
  (`self.Set_Color` (`self.Work_Position`)))