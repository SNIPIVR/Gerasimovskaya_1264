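; BP_AVMeter is an analog meter actor, apparently an ammeter/voltmeter, with a needle mesh and text labels for unit and range.
; The construction script fills the labels and applies the initial value.
; SetValue clamps the value to MIN–MAX and rolls the arrow linearly, scaled by range width without subtracting MIN.
; The Change_CurrentValue event drives SetValue at runtime, while a delayed random-value test is left unconnected.
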(event `self.ReceiveTick`
  (params (DeltaSeconds :type "Float (single-precision)")))

(event `Change_CurrentValue`
  (params (Val :type "Float (double-precision)"))
  (`self.Set_Value` Val))

(fn `Set_Value`
  (params (Val :type "Float (double-precision)"))
  (bind _output_get (set `self.Current_Value` (`KismetMathLibrary.FClamp` Val (`self.MIN`) (`self.MAX`))))
  (`SceneComponent.K2_SetRelativeRotation` (`self.SM_AVmeter_Arrow`) (`KismetMathLibrary.MakeRotator` (- (* _output_get (/ -78.0 (- (`self.MAX`) (`self.MIN`)))) 282.0)) false false))

(fn `UserConstructionScript`
  (`TextRenderComponent.K2_SetText` (`self.TR_Measure`) (`self.Measure`))
  (`TextRenderComponent.K2_SetText` (`self.TR_MIN`) (`KismetTextLibrary.Conv_DoubleToText` (`self.MIN`) "HalfToEven"))
  (`TextRenderComponent.K2_SetText` (`self.TR_MAX`) (`KismetTextLibrary.Conv_DoubleToText` (`self.MAX`) "HalfToEven"))
  (`self.Set_Value` (`self.Current_Value`)))