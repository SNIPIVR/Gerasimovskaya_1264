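; Excel reporter that records a person's run through one of the numbered scenarios.
; CreateXLS loads the scenario's template from the project, fills in date, full name and position, and saves it under a hardcoded D: results path named by timestamp, scenario and person.
; SendToLog writes timestamped object, value and ID rows to the "Выполнение" sheet, saving each time; consecutive entries for the same object overwrite one row.
; SaveAgain is an empty stub.
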(event `SendToLog`
  (params (LogObject :type String) (LogValue :type String) (LogID :type String))
  (bind _sheetlog_number (`self.SheetLog_Number`))
  (bind _sheetlog (`self.SheetLog`))
  (set `self.SheetLog_Value` LogValue)
  (if (not (`KismetStringLibrary.EqualEqual_StrStr` LogObject (`self.SheetLog_Object`)))
    (`/Engine/EditorBlueprintResources/StandardMacros.IncrementInt` (`self.SheetLog_Number`)
      (:`  `
        _)))
  (if (not (`KismetStringLibrary.IsEmpty` (`self.XlsFullName`)))
    (set `self.SheetLog_Id` LogID)
    (set `self.SheetLog_Object` LogObject)
    (bind _output_get (set `self.SheetLog` (`ExcelWorkbook.SheetWithTitle` (`self.Workbook`) "Выполнение")))
    (`ExcelWorksheet.SetStringAt` _output_get (`KismetStringLibrary.Conv_IntToString` (- _sheetlog_number 1)) 1 _sheetlog_number)
    (bind _output_get_2 (set `self.date_format` (`ExcelCell.GetFormat` (`ExcelWorksheet.CellAt` (`self.SheetLog`) 2 2))))
    (`ExcelWorksheet.SetDateTimeAt` _sheetlog (`KismetMathLibrary.Now`) 2 (`self.SheetLog_Number`))
    (`ExcelCell.SetFormat` (`ExcelWorksheet.CellAt` _sheetlog 2 (`self.SheetLog_Number`)) _output_get_2)
    (`ExcelWorksheet.SetStringAt` (`self.SheetLog`) (`self.SheetLog_Object`) 3 _sheetlog_number)
    (`ExcelWorksheet.SetStringAt` (`self.SheetLog`) (`self.SheetLog_Value`) 4 _sheetlog_number)
    (`ExcelWorksheet.SetStringAt` (`self.SheetLog`) (`self.SheetLog_Id`) 5 _sheetlog_number)
    (`DirectExcelLibrary.SaveExcel` (`self.Workbook`) (`self.XlsFullName`))))

(event `SaveAgain`
  (params (ScenarN :type "/Game/BP/Blueprints/UI/MainMenu/ChoiceScenar Enum" :default "NewEnumerator0") (FIO :type Text) (`Doljnost'` :type Text)))

(event `CreateXLS`
  (params (ScenarN :type "/Game/BP/Blueprints/UI/MainMenu/ChoiceScenar Enum" :default "NewEnumerator0") (FIO :type Text) (`Doljnost'` :type Text))
  (bind (_year _month _day _hour _minute) (`KismetMathLibrary.BreakDateTime` (`KismetMathLibrary.Now`)))
  (bind _returnvalue (`ExcelWorksheet.CellAt` (`self.Sheet`) 2 2))
  (set `self.ScenarN` ScenarN)
  (set `self.FIO` (`KismetTextLibrary.Conv_TextToString` FIO))
  (set `self.Doljnost'` (`KismetTextLibrary.Conv_TextToString` `Doljnost'`))
  (set `self.XlsFullName` (`KismetStringLibrary.Concat_StrStr` "d:/Результаты/" (`KismetStringLibrary.Conv_IntToString` _year) "_" (`self.DayTo2Digital` _month) "_" (`self.DayTo2Digital` _day) "/" (`self.DayTo2Digital` _hour) "-" (`self.DayTo2Digital` _minute) (select `/Game/BP/Blueprints/UI/MainMenu/ChoiceScenar` (`self.ScenarN`) :`NewEnumerator0` ". Сценарий 1. " :`NewEnumerator1` ". Сценарий 2. " :`NewEnumerator2` ". Сценарий 3. " :`NewEnumerator3` ". Сценарий 4. " :`NewEnumerator4` ". Сценарий 5. " :`NewEnumerator5` ". Сценарий 6. " :`NewEnumerator6` ". Сценарий 7. ") (`self.FIO`) " (" (`self.Doljnost'`) ").xlsx"))
  (bind _returnvalue_2 (`DirectExcelLibrary.LoadExcel` (`KismetStringLibrary.Concat_StrStr` "/Шаблоны/" (`|GetEnumeratorNameAsString` (`self.ScenarN`)) ".xlsx") "ProjectDir"))
  (bind _output_get (set `self.Workbook` _returnvalue_2))
  (`DirectExcelLibrary.SaveExcel` _output_get (`self.XlsFullName`))
  (set `self.Sheet` (`ExcelWorkbook.ActiveSheet` (`self.Workbook`)))
  (bind _output_get_2 (set `self.date_format` (`ExcelCell.GetFormat` _returnvalue)))
  (`ExcelWorksheet.SetDateTimeAt` (`self.Sheet`) (`KismetMathLibrary.Now`) 2 2)
  (`ExcelCell.SetFormat` _returnvalue _output_get_2)
  (`ExcelWorksheet.SetStringAt` (`self.Sheet`) (`self.FIO`) 2 3)
  (`ExcelWorksheet.SetStringAt` (`self.Sheet`) (`self.Doljnost'`) 2 4)
  (`DirectExcelLibrary.SaveExcel` (`self.Workbook`) (`self.XlsFullName`)))

(fn `UserConstructionScript`)