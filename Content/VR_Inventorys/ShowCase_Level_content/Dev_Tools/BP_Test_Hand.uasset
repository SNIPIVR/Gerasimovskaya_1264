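; BP_Test_Hand is a dev test actor that simulates a right VR hand interacting with inventory slots.
; On BeginPlay it caches its own BP_VRM_GrabComponent as the held component.
; The RightHandDetect overlap tracks one actor tagged "slot", deactivating any previous slot and activating the new one with the held component and right motion controller.
; Leaving the tracked slot deactivates and clears it.
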(event `self.ReceiveBeginPlay`
  ;[1 1 1] Test for held actor
  (set `self.HeldComponentRight` (`self.GetComponentByClass` "/Game/VR_Inventorys/Blueprints/BP_VRM_GrabComponent.BP_VRM_GrabComponent_C")) ; Held Actor!
)

(event `self.Right Hand Detect.OnComponentBeginOverlap`
  (params (OverlappedComponent :type "PrimitiveComponent Object Reference") (OtherActor :type "Actor Object Reference") (OtherComp :type "PrimitiveComponent Object Reference") (OtherBodyIndex :type Integer) (bFromSweep :type Boolean) (SweepResult :type "HitResult Structure (by ref)"))
  (if (`self.ActorHasTag` OtherActor "slot")
    (bind _detected_slot_rh (`self.Detected Slot RH`) ; Previously Set Slot?
      (:`then`
        (message `/Game/VR_Inventorys/Blueprints/BPI_InventorySlot_Interface.Deactivate Slot` _detected_slot_rh (`self.HeldComponentRight`)))
      (:`else`
        _))
    (bind _output_get (set `self.Detected Slot RH` OtherActor)) ; New detect!
    (message `/Game/VR_Inventorys/Blueprints/BPI_InventorySlot_Interface.Activate Slot` _output_get (`self.HeldComponentRight`) (`self.MotionControllerRight`))))

(event `self.Right Hand Detect.OnComponentEndOverlap`
  (params (OverlappedComponent :type "PrimitiveComponent Object Reference") (OtherActor :type "Actor Object Reference") (OtherComp :type "PrimitiveComponent Object Reference") (OtherBodyIndex :type Integer))
  (if (== OtherActor (`self.Detected Slot RH`))
    (message `/Game/VR_Inventorys/Blueprints/BPI_InventorySlot_Interface.Deactivate Slot` (`self.Detected Slot RH`) (`self.HeldComponentRight`))
    (set `self.Detected Slot RH` null) ; Reset Slot
  ))

(fn `UserConstructionScript`)