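; Promotional display version of a VR inventory slot that can mimic the hand-hover interaction in a showcase level.
; BeginPlay creates dynamic materials for slot and ring, applies visibility and colors from SlotConfiguration, and sets the description text.
; With PromoAnimate enabled, Tick uses a one-second Delay and FlipFlop to alternately play and reverse the hover timeline.
; That timeline optionally lerps the slot mesh's scale and material opacity.
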(event `self.ReceiveBeginPlay`
  (bind _slot_dynamic_mat (`self.Slot Dynamic Mat`))
  (bind _ring_dynamic_mat (`self.Ring Dynamic Mat`))
  (bind (_slot_configuration_dontshowouterring _slot_configuration_dontshowslottext _slot_configuration_showemptysloticon _slot_configuration_sizescalingoninteraction _slot_configuration_slotscaleupsize _slot_configuration_scaleupslotteditem _slot_configuration_opacityscalingoninteraction _slot_configuration_rotationoninteraction _slot_configuration_slotcolor _slot_configuration_outerringcolor) (break `/Game/VR_Inventorys/Blueprints/Struct_Slot_Config` (`self.Slot configuration`)))
  (`|ExecutionSequence`
    (:`then_0`
      (set `self.Current 3D Scale` (`SceneComponent.RelativeScale3D` (`self.Slot mesh`)))
      ;[1 1 1] Use Dynamic Material, Allows Control of  Material Paramaters
      (bind _returnvalue (`PrimitiveComponent.CreateDynamicMaterialInstance` (`self.Slot mesh`) 0 null "None"))
      (set `self.Slot Dynamic Mat` _returnvalue)
      (bind _returnvalue_2 (`PrimitiveComponent.CreateDynamicMaterialInstance` (`self.Ring mesh`) 0 null "None"))
      (set `self.Ring Dynamic Mat` _returnvalue_2)
      (`PrimitiveComponent.SetMaterial` (`self.Slot mesh`) 0 (`self.Slot Dynamic Mat`))
      (`PrimitiveComponent.SetMaterial` (`self.Ring mesh`) 0 (`self.Ring Dynamic Mat`)))
    (:`then_1`
      ;[0.8853 1 0] Slot CONFIG
      (`SceneComponent.SetHiddenInGame` (`self.Ring mesh`) _slot_configuration_dontshowouterring false) ; Hide Outer Ring
      (`SceneComponent.SetHiddenInGame` (`self.Empty Icon`) _slot_configuration_showemptysloticon false) ; Hide Empty Icon
      (`SceneComponent.SetHiddenInGame` (`self.TextRender`) _slot_configuration_dontshowslottext false) ; Hide Slot Info Text
      (`/Engine/EditorBlueprintResources/StandardMacros.IsValid` _slot_dynamic_mat
        (:`Is Valid`
          (`MaterialInstanceDynamic.SetVectorParameterValue` _slot_dynamic_mat "Color" _slot_configuration_slotcolor)
          (`/Engine/EditorBlueprintResources/StandardMacros.IsValid` _ring_dynamic_mat
            (:`Is Valid`
              (`MaterialInstanceDynamic.SetVectorParameterValue` _ring_dynamic_mat "Color" _slot_configuration_outerringcolor))))))
    (:`then_3`
      (`TextRenderComponent.K2_SetText` (`self.Text Discription`) (`self.Promo Discription text`)))))

(event `self.ReceiveTick`
  (params (DeltaSeconds :type "Float (single-precision)"))
  (bind (_slot_configuration_dontshowouterring _slot_configuration_dontshowslottext _slot_configuration_showemptysloticon _slot_configuration_sizescalingoninteraction _slot_configuration_slotscaleupsize _slot_configuration_scaleupslotteditem _slot_configuration_opacityscalingoninteraction) (break `/Game/VR_Inventorys/Blueprints/Struct_Slot_Config` (`self.Slot configuration`)))
  ;[1 1 1] Potential Slot Interaction when Hand Hover over slot
  ;;[1 1 1] Scale Up and down
  (if (`self.Promo Animate`)
    (`KismetSystemLibrary.Delay` 1.0)
    (`/Engine/EditorBlueprintResources/StandardMacros.FlipFlop`
      (:`A`
        (bind (_direction _lerp) (`Timeline|Hand Hover Slot Interaction` :!label _label)
          (:`Update`
            (if _slot_configuration_sizescalingoninteraction
              ;;[1 1 1] Scale Up Slot Mesh, On Hover (relative to its parent actor
              (`SceneComponent.SetRelativeScale3D` (`self.Slot mesh`) (`KismetMathLibrary.VLerp` (`self.Current 3D Scale`) (* (`self.Current 3D Scale`) (1.2 1.2 1.2)) _lerp)))
            ;;[1 1 1] Highlight On Hover
            (if _slot_configuration_opacityscalingoninteraction
              (`MaterialInstanceDynamic.SetScalarParameterValue` (`self.Slot Dynamic Mat`) "MinOpacity" (`KismetMathLibrary.Lerp` 0.1 0.3 _lerp))))))
      (:`B`
        (goto _label :!via `Reverse`)))))

(fn `UserConstructionScript`)