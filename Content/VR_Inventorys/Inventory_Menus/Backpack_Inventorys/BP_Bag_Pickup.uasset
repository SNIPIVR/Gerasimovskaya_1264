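; VR backpack inventory actor that the player grabs by physics constraint, with a weight readout in kg.
; Grabbing snaps GrabPoint to the motion controller, constrains the bag to the hand and swaps in a pre-authored left hand mesh.
; Releasing breaks the constraint and parks the bag below the origin with physics off, a temporary solution.
; Weight events update the text; mass is set only at BeginPlay, and the slot-based recalculation is never called.
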(event `self.ReceiveBeginPlay`
  (bind _backpack_weight (`self.BackPack Weight`))
  ;[0.3772 1 0] Set Weight of object at runtime
  (`PrimitiveComponent.SetMassOverrideInKg` (`self.StaticMeshComponent`) "None" _backpack_weight true)
  (`TextRenderComponent.K2_SetText` (`self.Weight Info`) (`|FormatText` "{Weight} kg" (`KismetTextLibrary.Conv_DoubleToText` _backpack_weight "HalfToEven"))))

(event `/Game/VR_Inventorys/Interfaces/BPI_Backpack.Remove Weight`
  (params (Item :type "Actor Object Reference") (Weight :type "Float (double-precision)"))
  ;[0.3772 1 0] Dynamically Adjust The BackPacks Weight
  (set `self.BackPack Weight` (- (`self.BackPack Weight`) Weight))
  ;;[0.3772 1 0] Update Text
  (`TextRenderComponent.K2_SetText` (`self.Weight Info`) (`|FormatText` "{Weight} kg" (`KismetTextLibrary.Conv_DoubleToText` (`self.BackPack Weight`) "HalfToEven")) :!label _label))

(event `/Game/VR_Inventorys/Interfaces/BPI_Backpack.Add Weight`
  (params (Item :type "Actor Object Reference") (Weight :type "Float (double-precision)"))
  ;[0.3772 1 0] Dynamically Adjust The BackPacks Weight
  (set `self.BackPack Weight` (+ (`self.BackPack Weight`) Weight))
  (goto _label))

(event `Grab Backpack Inventory`
  (params (`Track Hand` :type "BoxComponent Object Reference") (`Hand Mesh` :type "SkeletalMeshComponent Object Reference") (MotionController :type "MotionControllerComponent Object Reference"))
  (bind (_returnvalue_location _returnvalue_rotation) (`KismetMathLibrary.BreakTransform` (`KismetMathLibrary.ComposeTransforms` (`KismetMathLibrary.InvertTransform` (`SceneComponent.GetRelativeTransform` (`self.grab Point`))) (`SceneComponent.K2_GetComponentToWorld` MotionController))))
  (bind (_returnvalue_location_2 _returnvalue_rotation_2) (`KismetMathLibrary.BreakTransform` (`KismetMathLibrary.TLerp` (`self.GetTransform`) (`KismetMathLibrary.MakeTransform` _returnvalue_location _returnvalue_rotation) 1.0)))
  ;[1 1 1] Grab Backpack
  (`|ExecutionSequence`
    (:`then_0`
      (`/Engine/EditorBlueprintResources/StandardMacros.IsValid` `Hand Mesh`
        (:`Is Valid`
          (`SceneComponent.SetHiddenInGame` `Hand Mesh` true false)
          (set `self.Track Hand` `Track Hand`)
          ;;[1 1 1] Re-Enable Physics if  Inventory Bag was re-Grabbed
          (`PrimitiveComponent.SetSimulatePhysics` (`self.StaticMeshComponent`) true)
          (`PrimitiveComponent.SetCollisionResponseToChannel` (`self.StaticMeshComponent`) "ECC_Pawn" "ECR_Ignore")
          (`self.K2_SetActorTransform` (`KismetMathLibrary.MakeTransform` _returnvalue_location_2 _returnvalue_rotation_2) false true)
          (`PhysicsConstraintComponent.SetConstrainedComponents` (`self.Primary Grab Constraint`) (`self.Track Hand`) "None" (`self.StaticMeshComponent`) "None")
          (`PlayerController.PlayHapticEffect` (`GameplayStatics.GetPlayerController` 0) null "Left" 1.0 false))))
    (:`then_1`
      (`SceneComponent.SetHiddenInGame` (`self.Pre Autherd Hand mesh Left`) false false))))

(event `Release BackPack`
  ;[1 1 1] Release BackPack
  (`|ExecutionSequence`
    (:`then_0`
      (`/Engine/EditorBlueprintResources/StandardMacros.IsValid` (stale `Grab Backpack Inventory` `Hand Mesh`)
        (:`Is Valid`
          (`SceneComponent.SetHiddenInGame` (stale `Grab Backpack Inventory` `Hand Mesh`) false false)
          (`PhysicsConstraintComponent.BreakConstraint` (`self.Primary Grab Constraint`))
          ;;[1 1 1] Teleport Inventory Bag to a Location (Temp Solution, Until i Find A Better One)
          (`self.K2_SetActorLocation` (0.0 0.0 -1000.0) false true)
          (`PrimitiveComponent.SetSimulatePhysics` (`self.StaticMeshComponent`) false))))
    (:`then_1`
      (`SceneComponent.SetHiddenInGame` (`self.Pre Autherd Hand mesh Left`) true false))))

(fn `Re Evaluate Weight `
  (returns (`Weight Out` :type "Float (double-precision)"))
  (locals (`Temp Weight` :type "Float (double-precision)"))
  (set `local.Temp Weight` 0.0) ; Clear
  (for _array_element (`self.GetAllChildActors` false)
    (bind _asbp_inventory_slot_base (cast `/Game/VR_Inventorys/Slots/BASE_SLOT/BP_Inventory_Slot_BASE` _array_element))
    (bind _slotted_actor (`/Game/VR_Inventorys/Slots/BASE_SLOT/BP_Inventory_Slot_BASE.Slotted Actor` _asbp_inventory_slot_base)
      (:`then`
        (set `local.Temp Weight` (+ (`local.Temp Weight`) (`/Game/VR_Inventorys/Blueprints/BP_VRM_GrabComponent.Item Weight` (`self.GetComponentByClass` _slotted_actor "/Game/VR_Inventorys/Blueprints/BP_VRM_GrabComponent.BP_VRM_GrabComponent_C")))))
      (:`else`)))
  (return (`local.Temp Weight`)))

(fn `UserConstructionScript`)