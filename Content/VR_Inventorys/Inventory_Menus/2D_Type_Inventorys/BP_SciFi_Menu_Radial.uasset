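; Sci-fi radial menu actor for the VR inventory, which keeps itself turned toward the player.
; Every Tick, unless PromoExample is set, it aims at the cached VR camera with a look-at rotation, flipping yaw and clamping pitch to a narrow range.
; While no camera is cached, Tick searches for BP_VRPawn and stores its Camera.
; The graph holds only this facing logic, with no menu selection or item handling.
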(event `self.ReceiveBeginPlay`)

(event `self.ReceiveTick`
  (params (DeltaSeconds :type "Float (single-precision)"))
  (bind (_returnvalue_roll _returnvalue_pitch _returnvalue_yaw) (`KismetMathLibrary.BreakRotator` (`KismetMathLibrary.FindLookAtRotation` (`SceneComponent.K2_GetComponentLocation` (`self.VR Player Camera`)) (`self.K2_GetActorLocation`))))
  (if (not (`self.Promo Example?`))
    ;[1 1 1] Keep Inventory FACING Player
    (`self.VR Player Camera` ; Happens ONLY once
      (:`then`
        (bind _result (`/Engine/EditorBlueprintResources/StandardMacros.NegateFloat` _returnvalue_pitch)
          (:`  `
            (`self.K2_SetActorRotation` (`KismetMathLibrary.MakeRotator` 0.0 (`KismetMathLibrary.ClampAngle` _result -20.0 20.0) (+ _returnvalue_yaw 180.0))))))
      (:`else`
        ;[1 1 1] Search for Players Vr Camera
        (bind _returnvalue (`GameplayStatics.GetActorOfClass` "/Game/VR_Inventorys/VRTemplate/Blueprints/BP_VRPawn.BP_VRPawn_C"))
        (`/Engine/EditorBlueprintResources/StandardMacros.IsValid` _returnvalue
          (:`Is Valid`
            (set `self.VR Player Camera` (`/Game/VR_Inventorys/VRTemplate/Blueprints/BP_VRPawn.Camera` _returnvalue))))))))

(fn `UserConstructionScript`)