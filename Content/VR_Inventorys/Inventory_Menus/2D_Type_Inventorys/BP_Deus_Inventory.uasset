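; VR 2D-type Deus inventory menu actor that turns to face the player's VR camera.
; It rotates on menu open or appear, gated by a DoOnce that close or disappear resets, and every Tick unless PromoExample is set.
; Yaw follows a look-at from the camera with a quarter-turn offset, and pitch is clamped.
; The camera is lazily found on BP_VRPawn and cached.
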(event Custom|On%20Open%20Menu
  ;[1 1 1] Keep Inventory FACING Player
  (Utilities|FlowControl|DoOnce false
    (:Completed
      (Variables|Default|GetVR%20Player%20Camera ; Happens ONLY once
        (:then
          (Transformation|SetActorRotation (Math|Rotator|MakeRotator 0.0 (Math|Float|ClampAngle (stale _result) -2e+01 2e+01) (+ (.yaw (Math|Rotator|FindLookatRotation (Transformation|GetWorldLocation (Variables|Default|GetVR%20Player%20Camera)) (Transformation|GetActorLocation))) -9e+01))))
        (:else
          ;[1 1 1] Search for Players Vr Camera
          (bind _returnvalue (Actor|GetActorOfClass "/Game/VR_Inventorys/VRTemplate/Blueprints/BP_VRPawn.BP_VRPawn_C"))
          (Utilities|IsValid _returnvalue
            (:Is%20Valid
              (Variables|Default|SetVR%20Player%20Camera (Variables|/Game/VR_Inventorys/VRTemplate/Blueprints/BP_VRPawn.BP_VRPawn_C|GetCamera _returnvalue)))))))))

(event Custom|On%20Close%20Menu
  ;[1 1 1] Keep Inventory FACING Player
  (Utilities|FlowControl|DoOnce false) ; enters at Reset
)

(event EventBeginPlay)

(event EventInventoryDissappear
  ;[1 1 1] Keep Inventory FACING Player
  (Utilities|FlowControl|DoOnce false) ; enters at Reset
)

(event EventTick
  (params (DeltaSeconds :type Float%20%28single-precision%29))
  ;[1 1 1] Keep Inventory FACING Player
  (if (not (Variables|Default|GetPromo%20Example?))
    (Variables|Default|GetVR%20Player%20Camera ; Happens ONLY once
      (:then
        (Transformation|SetActorRotation (Math|Rotator|MakeRotator 0.0 (Math|Float|ClampAngle (stale _result) -2e+01 2e+01) (+ (.yaw (Math|Rotator|FindLookatRotation (Transformation|GetWorldLocation (Variables|Default|GetVR%20Player%20Camera)) (Transformation|GetActorLocation))) -9e+01))))
      (:else
        ;[1 1 1] Search for Players Vr Camera
        (bind _returnvalue (Actor|GetActorOfClass "/Game/VR_Inventorys/VRTemplate/Blueprints/BP_VRPawn.BP_VRPawn_C"))
        (Utilities|IsValid _returnvalue
          (:Is%20Valid
            (Variables|Default|SetVR%20Player%20Camera (Variables|/Game/VR_Inventorys/VRTemplate/Blueprints/BP_VRPawn.BP_VRPawn_C|GetCamera _returnvalue))))))))

(event EventInventoryAppear
  ;[1 1 1] Keep Inventory FACING Player
  (Utilities|FlowControl|DoOnce false
    (:Completed
      (Variables|Default|GetVR%20Player%20Camera ; Happens ONLY once
        (:then
          (Transformation|SetActorRotation (Math|Rotator|MakeRotator 0.0 (Math|Float|ClampAngle (stale _result) -2e+01 2e+01) (+ (.yaw (Math|Rotator|FindLookatRotation (Transformation|GetWorldLocation (Variables|Default|GetVR%20Player%20Camera)) (Transformation|GetActorLocation))) -9e+01))))
        (:else
          ;[1 1 1] Search for Players Vr Camera
          (bind _returnvalue (Actor|GetActorOfClass "/Game/VR_Inventorys/VRTemplate/Blueprints/BP_VRPawn.BP_VRPawn_C"))
          (Utilities|IsValid _returnvalue
            (:Is%20Valid
              (Variables|Default|SetVR%20Player%20Camera (Variables|/Game/VR_Inventorys/VRTemplate/Blueprints/BP_VRPawn.BP_VRPawn_C|GetCamera _returnvalue)))))))))

(fn ConstructionScript)