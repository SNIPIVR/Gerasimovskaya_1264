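; Component that opens and hides a VR inventory menu in one of several styles (Half-Life Alyx, Dead Space, Deus Ex, three radial).
; CallInventory spawns the class mapped to the chosen style beside the hand, ahead of the camera or at a passed-in component.
; A single cached menu is reused regardless of later style selection, then messaged to appear.
; HideInventory messages it to disappear and parks it below the world origin after a delay; older per-style chains are unwired.
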(event `Call Inventory`
  (params (`Players VR Hand` :type "SkeletalMeshComponent Object Reference") (`Players VR Camera` :type "CameraComponent Object Reference") (`Any scene Component` :type "SceneComponent Object Reference") (Selection :type "/Game/VR_Inventorys/Blueprints/Enum_Inventory_Menu_Type_enum Enum" :default "NewEnumerator0"))
  (bind _players_vr_hand (`self.Players VR Hand`))
  (bind _players_vr_camera (`self.Players VR Camera`))
  (bind _returnvalue (`SceneComponent.K2_GetComponentLocation` (`self.Any Scene Component`)))
  (bind (_value _returnvalue_2) (`BlueprintMapLibrary.Map_Find` (`self.Actor ref`) (`self.Inventory Type`)))
  (bind _returnvalue_3 (+ (`SceneComponent.K2_GetComponentLocation` _players_vr_camera) (* (`SceneComponent.GetForwardVector` _players_vr_camera) 70.0)))
  (bind _returnvalue_4 (select `/Game/VR_Inventorys/Blueprints/Enum_Inventory_Menu_Type_enum` (`self.Inventory Type`) :`NewEnumerator0` (+ (`SceneComponent.K2_GetComponentLocation` _players_vr_hand) (* (`SceneComponent.GetRightVector` _players_vr_hand) 30.0)) :`NewEnumerator1` _returnvalue_3 :`NewEnumerator3` _returnvalue_3 :`NewEnumerator2` _returnvalue :`NewEnumerator4` _returnvalue :`NewEnumerator5` _returnvalue))
  (set `self.Players VR Hand` `Players VR Hand`)
  (set `self.Any Scene Component` `Any scene Component`)
  (set `self.Players VR Camera` `Players VR Camera`)
  (set `self.Inventory Type` Selection)
  (`self.Menu Ref`
    (:`then`
      (`Actor.K2_SetActorLocation` (`self.Menu Ref`) _returnvalue_4 false true)
      (message `/Game/VR_Inventorys/Blueprints/BPI_InventorySlot_Interface.Inventory Appear` (`self.Menu Ref`)))
    (:`else`
      ;[0.3772 1 0] add \show inventory
      (if _returnvalue_2
        (bind _returnvalue_5 (`|SpawnActorFromClass` (`|ConvertAsset` _value) (`KismetMathLibrary.MakeTransform` _returnvalue_4) "Undefined" "OverrideRootScale" null null))
        (set `self.Menu Ref` _returnvalue_5)))))

(event `Hide Inventory`
  ;[0.3772 1 0] Hide
  (bind _menu_ref (`self.Menu Ref`)
    (:`then`
      (message `/Game/VR_Inventorys/Blueprints/BPI_InventorySlot_Interface.Inventory Dissappear` _menu_ref)
      (`KismetSystemLibrary.Delay` 1.5)
      (`Actor.K2_SetActorLocation` _menu_ref (0.0 0.0 -500.0) false true))
    (:`else`)))