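; Inventory component that saves and restores the items held in its owner's slot child actors, apparently a VR backpack.
; On BeginPlay it caches the game instance, the auto-store slot and every inventory slot among the owner's child actors.
; SaveItems appends slotted actor classes to an uncleared array and writes it to the save game.
; LoadItems clears all slots, spawns saved classes at the auto-store slot and passes each to it for storing.
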(event `self.ReceiveBeginPlay`
  (bind _childactors (`Actor.GetAllChildActors` (`self.GetOwner`) true))
  (`|ExecutionSequence`
    (:`then_0`
      ;[0.1424 0.2864 1] Save data
      (bind _asbp_game_instance (cast `/Game/VR_Inventorys/Blueprints/Save/BP_Game_Instance` (`GameplayStatics.GetGameInstance`)))
      (set `self.As BP Game Instance` _asbp_game_instance))
    (:`then_1`
      (for _array_element _childactors
        (bind _asbp_auto_store_slot (cast `/Game/VR_Inventorys/Slots/BP_Auto_Store_Slot` _array_element))
        (set `self.As BP Auto Store Slot Ref` _asbp_auto_store_slot))
      (for _array_element_2 _childactors
        (bind _asbp_inventory_slot_base (cast `/Game/VR_Inventorys/Slots/BASE_SLOT/BP_Inventory_Slot_BASE` _array_element_2))
        (`KismetArrayLibrary.Array_Add` (`self.Slot Array`) _asbp_inventory_slot_base)))))

(event `Load Items`
  (bind _slot_array (`self.Slot Array`))
  ;[1 1 1] Clear ALL SLOTS First!
  (for _index (range (+ (`KismetArrayLibrary.Array_Length` _slot_array) 1))
    (bind _asbp_inventory_slot_base (cast `/Game/VR_Inventorys/Slots/BASE_SLOT/BP_Inventory_Slot_BASE` (`|GetArrayItem` _slot_array _index)))
    (`/Game/VR_Inventorys/Slots/BASE_SLOT/BP_Inventory_Slot_BASE.Quick Clear Slot` _asbp_inventory_slot_base))
  ;[1 1 1] Load Items from SAVED ?
  (for (_array_element _array_index) (`/Game/VR_Inventorys/Blueprints/Save/BP_SaveGame.BackPack Array Invetory items` (`/Game/VR_Inventorys/Blueprints/Save/BP_Game_Instance.As BP Save Game` (`self.As BP Game Instance`)))
    (bind _returnvalue (`|SpawnActorFromClass` _array_element (`KismetMathLibrary.MakeTransform` (`Actor.K2_GetActorLocation` (`self.As BP Auto Store Slot Ref`))) "Undefined" "MultiplyWithRoot" null null))
    (`/Engine/EditorBlueprintResources/StandardMacros.IsValid` _returnvalue
      (:`Is Valid`
        (message `/Game/VR_Inventorys/Blueprints/BPI_InventorySlot_Interface.Auto Store` (`self.As BP Auto Store Slot Ref`) _returnvalue null)
        (`KismetSystemLibrary.PrintString` (`KismetStringLibrary.Concat_StrStr` (`KismetSystemLibrary.GetDisplayName` _returnvalue) ".............................    Loaded"))))))

(event `Save Items`
  (bind _slot_array (`self.Slot Array`))
  (bind _as_bp_game_instance (`self.As BP Game Instance`))
  (bind _as_bp_save_game (`/Game/VR_Inventorys/Blueprints/Save/BP_Game_Instance.As BP Save Game` _as_bp_game_instance))
  ;[0.3772 1 0] save items
  (for _index (range (+ (`KismetArrayLibrary.Array_Length` _slot_array) 1))
    (bind _asbp_inventory_slot_base (cast `/Game/VR_Inventorys/Slots/BASE_SLOT/BP_Inventory_Slot_BASE` (`|GetArrayItem` _slot_array _index)))
    (`KismetArrayLibrary.Array_Add` (`self.Slotted actors Array`) (`GameplayStatics.GetObjectClass` (`/Game/VR_Inventorys/Slots/BASE_SLOT/BP_Inventory_Slot_BASE.Slotted Actor` _asbp_inventory_slot_base))))
  (`/Game/VR_Inventorys/Blueprints/Save/BP_SaveGame.Save Backpack Items` _as_bp_save_game (`self.Slotted actors Array`))
  (`GameplayStatics.SaveGameToSlot` _as_bp_save_game (`/Game/VR_Inventorys/Blueprints/Save/BP_Game_Instance.Save Slot Name` _as_bp_game_instance))
  (`/Game/VR_Inventorys/Blueprints/Save/BP_SaveGame.Show Backpack Saved Data` _as_bp_save_game))