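; Game instance for the VR inventory system that holds the session's BP_SaveGame reference.
; On Init it loads the save from its slot if one exists, printing an error when the cast fails, or otherwise creates a new save object without writing it to disk.
; SaveData and LoadData are empty stubs, and a backpack saved-data display call is left unconnected.
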(event `self.ReceiveInit`
  ;[0.3772 1 0] setup save Data
  (bind _returnvalue (`GameplayStatics.DoesSaveGameExist` (`self.Save Slot Name`)))
  (if _returnvalue
    (bind _returnvalue_2 (`GameplayStatics.LoadGameFromSlot` (`self.Save Slot Name`)))
    (bind _asbp_save_game (cast `/Game/VR_Inventorys/Blueprints/Save/BP_SaveGame` _returnvalue_2)
      (:`then`
        (set `self.As BP Save Game` _asbp_save_game)
        (bind _as_bp_save_game (`self.As BP Save Game`)
          (:`then`)
          (:`else`)))
      (:`CastFailed`
        (`KismetSystemLibrary.PrintString` "FAILED TO GET SAVE GAME FROM GAME INSTANCE")))
    (else
      (bind _returnvalue_3 (`GameplayStatics.CreateSaveGameObject` "/Game/VR_Inventorys/Blueprints/Save/BP_SaveGame.BP_SaveGame_C"))
      (set `self.As BP Save Game` _returnvalue_3))))

(fn `Load Data`)

(fn `Save Data`)