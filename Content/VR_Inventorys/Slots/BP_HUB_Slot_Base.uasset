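; BP_HUB_Slot_Base is a VR inventory hub slot that shows a label and reveals its child sub-slots when a hand hovers over it.
; Appear and Disappear scale the hub with a timeline, while dynamic materials color the slot and ring from its config.
; A tagged VR hand overlap plays a hover timeline that raises opacity and scales up the sub-slots and unhides their items.
; Leaving starts a short timer that reverses the timeline, hiding slotted items when finished.
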(event `self.ReceiveBeginPlay`
  (bind (_hub_slot_config_dontshowouterring _hub_slot_config_dontshowslottext _hub_slot_config_showemptysloticon _hub_slot_config_sizescalingoninteraction _hub_slot_config_slotscaleupsize _hub_slot_config_scaleupslotteditem _hub_slot_config_opacityscalingoninteraction _hub_slot_config_rotationoninteraction _hub_slot_config_slotcolor _hub_slot_config_outerringcolor) (break `/Game/VR_Inventorys/Blueprints/Struct_Slot_Config` (`self.HUB slot config`)))
  (`|ExecutionSequence`
    (:`then_0`
      (`TextRenderComponent.K2_SetText` (`self.Hub text`) (`self.Name of HUB`))
      (set `self.SubSlots Array` (`self.GetAllChildActors` true)))
    (:`then_1`
      ;[1 1 1] Use Dynamic Material, Allows Control of  Material Paramaters
      (bind _returnvalue (`PrimitiveComponent.CreateDynamicMaterialInstance` (`self.Slot mesh`) 0 null "None"))
      (set `self.Slot Dynamic Mat` _returnvalue)
      (bind _returnvalue_2 (`PrimitiveComponent.CreateDynamicMaterialInstance` (`self.Ring mesh`) 0 null "None"))
      (set `self.Ring Dynamic Mat` _returnvalue_2)
      (`PrimitiveComponent.SetMaterial` (`self.Slot mesh`) 0 (`self.Slot Dynamic Mat`))
      (`PrimitiveComponent.SetMaterial` (`self.Ring mesh`) 0 (`self.Ring Dynamic Mat`))
      (`self.SetActorHiddenInGame` (`self.SubSlots Array`) true) ; Hidden By default
    )
    (:`then_2`
      (`MaterialInstanceDynamic.SetVectorParameterValue` (`self.Slot Dynamic Mat`) "Color" _hub_slot_config_slotcolor)
      (`MaterialInstanceDynamic.SetVectorParameterValue` (`self.Ring Dynamic Mat`) "Color" _hub_slot_config_outerringcolor))))

(event `Appear`
  ;[1 1 1] On Appear Scale Up Main Slot ( Initial Anim Transition)
  (`self.SetActorHiddenInGame` false)
  (bind (_direction _lerp) (`Timeline|Scale UP` :!via `PlayFromStart` :!label _label)
    (:`Update`
      ;;[1 1 1] Scale Up
      (`self.SetActorScale3D` (`KismetMathLibrary.VLerp` (0.0 0.0 0.0) (1.0 1.0 1.0) _lerp)))
    (:`Finished`
      ;;[1 1 1] Hide after scale down
      (switch `ETimelineDirection` _direction
        (:`Backward`
          (`self.SetActorHiddenInGame` true))))))

(event `Disappear`
  ;[1 1 1] On Appear Scale Up Main Slot ( Initial Anim Transition)
  (goto _label :!via `ReverseFromEnd`))

(event `self.Trigger.OnComponentBeginOverlap`
  (params (OverlappedComponent :type "PrimitiveComponent Object Reference") (OtherActor :type "Actor Object Reference") (OtherComp :type "PrimitiveComponent Object Reference") (OtherBodyIndex :type Integer) (bFromSweep :type Boolean) (SweepResult :type "HitResult Structure (by ref)"))
  ;[1 1 1] Potential Slot Interaction when Hand Hover over slot
  (if (`ActorComponent.ComponentHasTag` OtherComp "VR Hand")
    (set `self.Active` true)
    (bind (_direction _lerp) (`Timeline|Hand Hover Slot Interaction` :!label _label_2)
      (:`Update`
        ;;[1 1 1] Highlight HUB SLOT On Hover
        (`MaterialInstanceDynamic.SetScalarParameterValue` (`self.Slot Dynamic Mat`) "MinOpacity" (`KismetMathLibrary.Lerp` 0.1 0.3 _lerp))
        (for _array_element (`self.SubSlots Array`)
          (`self.SetActorHiddenInGame` _array_element false)
          (`|ExecutionSequence`
            (:`then_0`
              ;;[1 1 1] Scale
              (`self.SetActorRelativeScale3D` _array_element (`KismetMathLibrary.VLerp` (0.0 0.0 0.0) (0.4 0.4 0.4) _lerp)))
            (:`then_1`
              (bind _slotted_actor (`/Game/VR_Inventorys/Slots/BASE_SLOT/BP_Inventory_Slot_BASE.Slotted Actor` (cast `/Game/VR_Inventorys/Slots/BASE_SLOT/BP_Inventory_Slot_BASE` _array_element :!pure true))
                (:`then`
                  (`self.SetActorHiddenInGame` _slotted_actor false))
                (:`else`))))))
      (:`Finished`
        (switch `ETimelineDirection` _direction
          (:`Backward`
            (for _array_element_2 (`self.SubSlots Array`)
              (bind _slotted_actor_2 (`/Game/VR_Inventorys/Slots/BASE_SLOT/BP_Inventory_Slot_BASE.Slotted Actor` (cast `/Game/VR_Inventorys/Slots/BASE_SLOT/BP_Inventory_Slot_BASE` _array_element_2 :!pure true))
                (:`then`
                  (`self.SetActorHiddenInGame` _slotted_actor_2 true)
                  (`KismetSystemLibrary.K2_ClearAndInvalidateTimerHandle` (stale `self.Trigger.OnComponentEndOverlap` _returnvalue)))
                (:`else`)))))))))

(event `SubSlot Timer`
  ;[1 1 1] Potential Slot Interaction when Hand Hover over slot
  (goto _label_2 :!via `Reverse`))

(event `self.Trigger.OnComponentEndOverlap`
  (params (OverlappedComponent :type "PrimitiveComponent Object Reference") (OtherActor :type "Actor Object Reference") (OtherComp :type "PrimitiveComponent Object Reference") (OtherBodyIndex :type Integer))
  ;[1 1 1] Potential Slot Interaction when Hand Hover over slot
  (if (`ActorComponent.ComponentHasTag` OtherComp "VR Hand")
    (set `self.Active` false)
    (bind _returnvalue (`KismetSystemLibrary.K2_SetTimerDelegate` (delegate `SubSlot Timer`) 1.0))))

(fn `UserConstructionScript`)