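; Base VR inventory slot that stores, releases or clears actors with a VRM grab component, optionally autospawning one.
; Storing checks occupancy and slot type, then attaches the item with its slotted or holster transform, or flashes red.
; Item weight changes are reported to a backpack parent through BPI_Backpack.
; The SlotConfiguration struct drives appearance and hand-hover feedback: haptics, dynamic-material opacity, timeline scaling and rotation.
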(event `self.Detect Box.OnComponentBeginOverlap`
  (params (OverlappedComponent :type "PrimitiveComponent Object Reference") (OtherActor :type "Actor Object Reference") (OtherComp :type "PrimitiveComponent Object Reference") (OtherBodyIndex :type Integer) (bFromSweep :type Boolean) (SweepResult :type "HitResult Structure (by ref)"))
  ;[0.3772 1 0] Slot Self Detect method ( But how will it know that another slot is also active? )
)

(event `self.Activate Slot`
  (params (`Held component` :type "/Game/VR_Inventorys/Blueprints/BP_VRM_GrabComponent Object Reference") (`Motion Controller` :type "MotionControllerComponent Object Reference"))
  ;[0.3772 1 0] Handle Hand Detection
  (`self.Slot Active` `Held component` `Motion Controller`) ; Under construction!
)

(event `self.ReceiveBeginPlay`
  (bind ((`DontShowOuterRing_22_0AE457FE48FA48AFF242A79EA7264EFB` _dontshowouterring) (`DontShowSlotText_16_A843240A44E1648E2778B6A6BD7969CB` _dontshowslottext) (`ShowEmptySlotIcon_79_BFEDBC684B17D2BE30463896FD1CEC38` _showemptysloticon) (`SlotscaleUpsize_73_923574E5446D1230387D65851947F746` _slotscaleupsize) (`ScaleUpslotteditem_78_288B1C1444F3DFCA92281CBACC80B9EE` _scaleupslotteditem) (`OpacityScalingonInteraction_54_626E165C46B421ACC1644CBC32353E97` _opacityscalingoninteraction) (`SlotColor_14_EB50064648D0C41894A6C2A6BB08A0B2` _slotcolor) (`OuterRingColor_19_8FF1BC5B4073314D19DA069D1BDD081B` _outerringcolor) (`SlotType_25_B885963C4CDDD7F1300C869D53443260` _slottype) (`Holster_66_6E7327ED475D062B7ECE4397204B82E3` _holster) (`SlottedHapticEffect_57_8DAD73DD4AAF1E0168E4B290C4412D53` _slottedhapticeffect) (`InteractionHapticEffect_60_4027F5D946295B12C954F7B6713BD3FB` _interactionhapticeffect)) (break `/Game/VR_Inventorys/Blueprints/Struct_Slot_Config` (`self.Slot configuration`)))
  (`|ExecutionSequence`
    (:`then_0`
      ;[0.1424 0.2864 1] Save data
      (bind _asbp_game_instance (cast `/Game/VR_Inventorys/Blueprints/Save/BP_Game_Instance` (`GameplayStatics.GetGameInstance`)))
      (set `self.As BP Game Instance` _asbp_game_instance))
    (:`then_1`
      (set `self.Actors Relative 3D Scale` (`self.GetActorRelativeScale3D`))
      (set `self.Mesh Relative 3D Scale` (`SceneComponent.RelativeScale3D` (`self.Slot mesh`)))
      ;[1 1 1] Use Dynamic Material, Allows Control of  Material Paramaters
      (bind _returnvalue (`PrimitiveComponent.CreateDynamicMaterialInstance` (`self.Slot mesh`) 0 null "None"))
      (set `self.Slot Dynamic Mat` _returnvalue)
      (bind _returnvalue_2 (`PrimitiveComponent.CreateDynamicMaterialInstance` (`self.Ring mesh`) 0 null "None"))
      (set `self.Ring Dynamic Mat` _returnvalue_2)
      (`PrimitiveComponent.SetMaterial` (`self.Slot mesh`) 0 (`self.Slot Dynamic Mat`))
      (`PrimitiveComponent.SetMaterial` (`self.Ring mesh`) 0 (`self.Ring Dynamic Mat`))
      ;[0.8853 1 0] Slot CONFIG
      (`self.Slot  config` _dontshowouterring _showemptysloticon _dontshowslottext _slotcolor _outerringcolor _opacityscalingoninteraction _slottype _holster _interactionhapticeffect _slottedhapticeffect)
      ;[1 1 1] Set up Rotation mesh
      (`MovementComponent.SetUpdatedComponent` (`self.RotatingMovement`) (`self.Slot mesh`))
      (`self.Autospawn`))))

(event `self.Detect Box.OnComponentEndOverlap`
  (params (OverlappedComponent :type "PrimitiveComponent Object Reference") (OtherActor :type "Actor Object Reference") (OtherComp :type "PrimitiveComponent Object Reference") (OtherBodyIndex :type Integer))
  ;[0.3772 1 0] Slot Self Detect method ( But how will it know that another slot is also active? )
)

(event `self.Deactivate Slot`
  (params (`Held Component` :type "/Game/VR_Inventorys/Blueprints/BP_VRM_GrabComponent Object Reference"))
  ;[0.3772 1 0] Handle Hand Detection
  (`self.Slot Deactivate` `Held Component`))

(event `Quick Clear Slot`
  (bind _returnvalue (`self.GetAttachParentActor`))
  ;[0.3772 1 0] Quick Clear Slot
  (`self.Slotted Actor`
    (:`then`
      (if (`KismetSystemLibrary.DoesImplementInterface` _returnvalue "/Game/VR_Inventorys/Interfaces/BPI_Backpack.BPI_Backpack_C")
        (message `/Game/VR_Inventorys/Interfaces/BPI_Backpack.Remove Weight` _returnvalue (`self.Slotted Actor`) (`/Game/VR_Inventorys/Blueprints/BP_VRM_GrabComponent.Item Weight` (`self.GetComponentByClass` (`self.Slotted Actor`) "/Game/VR_Inventorys/Blueprints/BP_VRM_GrabComponent.BP_VRM_GrabComponent_C")))
        (`self.K2_DestroyActor` (`self.Slotted Actor`))
        (set `self.Slotted Actor` null)
        (set `self.Primitive Component` null)
        (set `self.Slotted Actors Grab Component` null)
        (set `self.Slot in Use` false)))
    (:`else`)))

(event `self.InventoryQuickGrab`
  (params (`Motion Controller` :type "MotionControllerComponent Object Reference") (Hand :type "EControllerHand Enum" :default "Left"))
  (bind _returnvalue (`self.GetAttachParentActor`))
  (bind ((`ShowEmptySlotIcon_79_BFEDBC684B17D2BE30463896FD1CEC38` _showemptysloticon) (`OpacityScalingonInteraction_54_626E165C46B421ACC1644CBC32353E97` _opacityscalingoninteraction)) (break `/Game/VR_Inventorys/Blueprints/Struct_Slot_Config` (`self.Slot configuration`)))
  ;[0.3772 1 0] Quick Grab Slotted Item
  (bind _slotted_actor (`self.Slotted Actor`)
    (:`then`
      (`/Game/VR_Inventorys/Blueprints/BP_VRM_GrabComponent.Try Grab` (`self.GetComponentByClass` _slotted_actor "/Game/VR_Inventorys/Blueprints/BP_VRM_GrabComponent.BP_VRM_GrabComponent_C") `Motion Controller`)
      (`self.SetActorScale3D` (`self.Slotted Actor`) (`self.Actors Original scale`)) ; Set actor to correct scale before grabbing
      (bind _primitive_component (`self.Primitive Component`)
        (:`then`
          (`PrimitiveComponent.SetCollisionResponseToAllChannels` _primitive_component "ECR_Block") ; Prevent collision issues when slotted
          (`PrimitiveComponent.SetCastShadow` _primitive_component true) ; dont want Slotted Items casting shadows
          (`|ExecutionSequence`
            (:`then_0`
              (set `self.Slot in Use` false)
              (if (not _showemptysloticon)
                (`SceneComponent.SetHiddenInGame` (`self.Empty Icon`) false false))
              (if _opacityscalingoninteraction
                (`self.Update Slot Opacity` 0.1))
              (set `/Game/VR_Inventorys/Blueprints/BP_VRM_GrabComponent.Slotted?` false (`self.Slotted Actors Grab Component`))
              ;[0.3772 1 0] Reduce BackPack Inventory Weight
              (if (`KismetSystemLibrary.DoesImplementInterface` _returnvalue "/Game/VR_Inventorys/Interfaces/BPI_Backpack.BPI_Backpack_C")
                (message `/Game/VR_Inventorys/Interfaces/BPI_Backpack.Remove Weight` _returnvalue (`self.Slotted Actor`) (`/Game/VR_Inventorys/Blueprints/BP_VRM_GrabComponent.Item Weight` (`self.GetComponentByClass` (`self.Slotted Actor`) "/Game/VR_Inventorys/Blueprints/BP_VRM_GrabComponent.BP_VRM_GrabComponent_C")))))
            (:`then_1`
              ;;[1 1 1] Clear refs
              (set `self.Primitive Component` null)
              (set `self.Slotted Actor` null)
              (set `self.Slotted Actors Grab Component` null))))
        (:`else`)))
    (:`else`)))

(event `Wrong slot Timer`
  ;[0.2865 0.2865 0.2865] Slot  / Store Actor
  ;;[1 0.002493 0] Trun Red Or Any Other Colour On wrong slot type, for The set time
  (`MaterialInstanceDynamic.SetVectorParameterValue` (`self.Slot Dynamic Mat`) "Color" (`.SlotColor_14_EB50064648D0C41894A6C2A6BB08A0B2` (break `/Game/VR_Inventorys/Blueprints/Struct_Slot_Config` (`self.Slot configuration`)))) ; Restore to Original Color
  (`KismetSystemLibrary.K2_ClearAndInvalidateTimerHandle` (stale `self.InventoryQuickStore` _returnvalue_4)))

(event `self.InventoryQuickStore`
  (params (ACTOR :type "Actor Object Reference") (`Motion Controller` :type "MotionControllerComponent Object Reference"))
  (bind _returnvalue (`self.GetAttachParentActor`))
  (bind _slotted_actor (`self.Slotted Actor`))
  (bind ((`OpacityScalingonInteraction_54_626E165C46B421ACC1644CBC32353E97` _opacityscalingoninteraction) (`SlotColor_14_EB50064648D0C41894A6C2A6BB08A0B2` _slotcolor) (`SlottedSoundEffect_62_A403BB3942C74031103D6081FE9930B9` _slottedsoundeffect)) (break `/Game/VR_Inventorys/Blueprints/Struct_Slot_Config` (`self.Slot configuration`)))
  (bind ((`ShowEmptySlotIcon_79_BFEDBC684B17D2BE30463896FD1CEC38` _showemptysloticon) (`SlotscaleUpsize_73_923574E5446D1230387D65851947F746` _slotscaleupsize) (`ScaleUpslotteditem_78_288B1C1444F3DFCA92281CBACC80B9EE` _scaleupslotteditem) (`SlotType_25_B885963C4CDDD7F1300C869D53443260` _slottype) (`Holster_66_6E7327ED475D062B7ECE4397204B82E3` _holster)) (break `/Game/VR_Inventorys/Blueprints/Struct_Slot_Config` (`self.Slot configuration`)))
  (bind _returnvalue_2 (`self.GetComponentByClass` (`self.Slotted Actor`) "/Game/VR_Inventorys/Blueprints/BP_VRM_GrabComponent.BP_VRM_GrabComponent_C"))
  (bind _returnvalue_3 (`self.GetComponentByClass` (`self.Slotted Actor`) "/Game/VR_Inventorys/Blueprints/BP_VRM_GrabComponent.BP_VRM_GrabComponent_C"))
  ;[0.2865 0.2865 0.2865] Slot  / Store Actor
  ;;[0.3772 1 0] Quick store
  ;;;[0.0625 0.0625 0.0625] Set Refs
  (set `self.Slotted Actor` ACTOR)
  (set `self.Motion Controller ref` `Motion Controller`) ; For Haptic Effect!
  (`/Engine/EditorBlueprintResources/StandardMacros.IsValid` _returnvalue_2
    (:`Is Valid`
      (set `self.Slotted Actors Grab Component` _returnvalue_2) ; Create Ref to slotted actors Grab Component
      (set `self.Actors Original scale` (`/Game/VR_Inventorys/Blueprints/BP_VRM_GrabComponent.Default World scale` _returnvalue_2)) ; Used To restore actor to proper size on Slot grab
      (set `self.Item Slot Type` (`/Game/VR_Inventorys/Blueprints/BP_VRM_GrabComponent.SlotType` _returnvalue_2))
      (set `self.Primitive Component` (`self.GetComponentByClass` (`self.Slotted Actor`) "/Script/Engine.PrimitiveComponent"))
      (if (`self.Slot in Use`)
        ;;[1 0.002493 0] Trun Red Or Any Other Colour On wrong slot type, for The set time
        (bind _returnvalue_4 (`KismetSystemLibrary.K2_SetTimerDelegate` (delegate `Wrong slot Timer`) 1.0 :!label _label))
        (`MaterialInstanceDynamic.SetVectorParameterValue` (`self.Slot Dynamic Mat`) "Color" (struct :`R` 1.0 :`A` 1.0))
        (`/Game/VR_Inventorys/Blueprints/BP_VRM_GrabComponent.Try Release` (`self.Slotted Actors Grab Component`))
        (else
          ;;[0.3772 1 0] Slot Type Check
          (if (== (`self.Item Slot Type`) _slottype)
            (bind _primitive_component (`self.Primitive Component`)
              (:`then`
                (`PrimitiveComponent.SetCollisionResponseToAllChannels` _primitive_component "ECR_Ignore") ; Prevent collision issues when slotted
                (`PrimitiveComponent.SetCastShadow` _primitive_component false) ; dont want Slotted Items casting shadows
                (`self.K2_AttachToComponent` (`self.Slotted Actor`) (`self.AttachPoint`) "None" "KeepWorld" "KeepWorld" "KeepWorld" true)
                (if _holster
                  (`self.K2_SetActorRelativeTransform` _slotted_actor (`/Game/VR_Inventorys/Blueprints/BP_VRM_GrabComponent.Holster Transform` _returnvalue_3) false false)
                  (else
                    (`self.K2_SetActorRelativeTransform` _slotted_actor (`/Game/VR_Inventorys/Blueprints/BP_VRM_GrabComponent.Slotted Transfrom` _returnvalue_3) false false)))
                (if (not (`.ShowEmptySlotIcon_79_BFEDBC684B17D2BE30463896FD1CEC38` (break `/Game/VR_Inventorys/Blueprints/Struct_Slot_Config` (`self.Slot configuration`))))
                  (`SceneComponent.SetHiddenInGame` (`self.Empty Icon`) true false))
                (`self.Play Haptic Effect On correct hand` 1.0)
                (set `self.Slot in Use` true)
                ;;[1 1 1] Set slot to default colour when in use (to compensate for detect grab component slot type   changing the color to green.
                (`MaterialInstanceDynamic.SetVectorParameterValue` (`self.Slot Dynamic Mat`) "Color" _slotcolor)
                (if _opacityscalingoninteraction
                  (`self.Update Slot Opacity` 1.0))
                (set `/Game/VR_Inventorys/Blueprints/BP_VRM_GrabComponent.Slotted?` true (`self.Slotted Actors Grab Component`))
                (`self.Slot Sound` _slottedsoundeffect)
                ;[0.3772 1 0] Increase BackPack Inventory Weight
                (if (`KismetSystemLibrary.DoesImplementInterface` _returnvalue "/Game/VR_Inventorys/Interfaces/BPI_Backpack.BPI_Backpack_C")
                  (message `/Game/VR_Inventorys/Interfaces/BPI_Backpack.Add Weight` _returnvalue (`self.Slotted Actor`) (`/Game/VR_Inventorys/Blueprints/BP_VRM_GrabComponent.Item Weight` (`self.GetComponentByClass` (`self.Slotted Actor`) "/Game/VR_Inventorys/Blueprints/BP_VRM_GrabComponent.BP_VRM_GrabComponent_C")))))
              (:`else`))
            (else
              (goto _label))))))))

(event `Slot Sound`
  (params (Sound :type "SoundBase Object Reference"))
  ;[1 1 1] Play a Sound at slot location
  (`GameplayStatics.SpawnSoundAtLocation` Sound (`SceneComponent.K2_GetComponentLocation` (`self.AttachPoint`)) (struct) 1.0 1.0 0.0 null null))

(event `Appear`
  ;[1 1 1] On Appear Scale Up Slots ( Initial Anim Transition FOR Inventory Menu Spawn )
  (`self.SetActorHiddenInGame` false)
  (bind (_direction _lerp) (`Timeline|Scale UP` :!via `PlayFromStart` :!label _label_2)
    (:`Update`
      ;;[1 1 1] Scale
      (`self.SetActorRelativeScale3D` (`KismetMathLibrary.VLerp` (0.0 0.0 0.0) (`self.Actors Relative 3D Scale`) _lerp)))
    (:`Finished`
      ;;[1 1 1] Hide after scale down
      (switch `ETimelineDirection` _direction
        (:`Backward`
          (`self.SetActorHiddenInGame` true))))))

(event `Scale Up Slot`
  (bind _actors_relative_3d_scale (`self.Actors Relative 3D Scale`))
  (bind _mesh_relative_3d_scale (`self.Mesh Relative 3D Scale`))
  (bind ((`SlotscaleUpsize_73_923574E5446D1230387D65851947F746` _slotscaleupsize) (`ScaleUpslotteditem_78_288B1C1444F3DFCA92281CBACC80B9EE` _scaleupslotteditem)) (break `/Game/VR_Inventorys/Blueprints/Struct_Slot_Config` (`self.Slot configuration`)))
  ;[1 1 1] Potential Slot Interaction when Hand Hover over Occupied slot
  (bind (_direction _lerp) (`Timeline|Hand Hover Slot Interaction` :!label _label_3)
    (:`Update`
      ;;[0.3772 1 0] Scale Up Slot Mesh, On Hover (relative to its parent actor
      (if _scaleupslotteditem
        (`self.SetActorRelativeScale3D` (`KismetMathLibrary.VLerp` _actors_relative_3d_scale (* _actors_relative_3d_scale _slotscaleupsize) _lerp)) ; Using this will scale the whole actor including any slotted items
        (else
          (`SceneComponent.SetRelativeScale3D` (`self.Slot mesh`) (`KismetMathLibrary.VLerp` _mesh_relative_3d_scale (* _mesh_relative_3d_scale _slotscaleupsize) _lerp)))))))

(event `Disappear`
  ;[1 1 1] On Appear Scale Up Slots ( Initial Anim Transition FOR Inventory Menu Spawn )
  (goto _label_2 :!via `ReverseFromEnd`))

(event `Scale Down Slot`
  ;[1 1 1] Potential Slot Interaction when Hand Hover over Occupied slot
  (goto _label_3 :!via `Reverse`))

(event `Rotate Slot`
  ;[1 1 1] Slot rotatation
  (`ActorComponent.Activate` (`self.RotatingMovement`) false))

(event `Stop Slot rotation`
  ;[1 1 1] Slot rotatation
  (`ActorComponent.Deactivate` (`self.RotatingMovement`)))

(fn `Autospawn`
  (bind ((`ShowEmptySlotIcon_79_BFEDBC684B17D2BE30463896FD1CEC38` _showemptysloticon) (`SlotscaleUpsize_73_923574E5446D1230387D65851947F746` _slotscaleupsize) (`ScaleUpslotteditem_78_288B1C1444F3DFCA92281CBACC80B9EE` _scaleupslotteditem) (`AutospawnActor_69_6E6A4563479C91BB989B54A3BE2B461A` _autospawnactor)) (break `/Game/VR_Inventorys/Blueprints/Struct_Slot_Config` (`self.Slot configuration`)))
  (if (`KismetSystemLibrary.IsValidClass` _autospawnactor)
    (bind _returnvalue (`|SpawnActorFromClass` _autospawnactor (`KismetMathLibrary.MakeTransform` (0.0 0.0 0.0)) "AlwaysSpawn" "SelectDefaultAtRuntime" null null))
    (bind _returnvalue_2 (`self.GetComponentByClass` _returnvalue "/Game/VR_Inventorys/Blueprints/BP_VRM_GrabComponent.BP_VRM_GrabComponent_C"))
    (`/Engine/EditorBlueprintResources/StandardMacros.IsValid` _returnvalue_2
      (:`Is Valid`
        (setmembers `/Game/VR_Inventorys/Blueprints/Struct_Slot_Config` :`StructRef` (`self.Slot configuration`) :`Slot Type` (`/Game/VR_Inventorys/Blueprints/BP_VRM_GrabComponent.SlotType` _returnvalue_2))
        (`self.InventoryQuickStore` _returnvalue)
        (return))
      (:`Is Not Valid`
        (`KismetSystemLibrary.PrintString` "D'oh!  The chosen Autospawn Actor has No VRM Grab Component! ( PLEASE ADD ONE ! FOR FULL FUNCTIONALITY ) and free doughnuts ; )" true true (struct :`R` 1.0 :`A` 1.0) 5.0) ; You selected a autospawn actor with no VRM GRAB COMPONENT  Doh!
      ))
    (else
      (return))))

(fn `Play Haptic Effect On correct hand`
  (params (Scale :type "Float (single-precision)") (`Motion Controller` :type "MotionControllerComponent Object Reference"))
  (`/Engine/EditorBlueprintResources/StandardMacros.IsValid` `Motion Controller`
    (:`Is Valid`
      (`PlayerController.PlayHapticEffect` (`GameplayStatics.GetPlayerController` 0) (`.InteractionHapticEffect_60_4027F5D946295B12C954F7B6713BD3FB` (break `/Game/VR_Inventorys/Blueprints/Struct_Slot_Config` (`self.Slot configuration`))) (select `bool` (== (`MotionControllerComponent.MotionSource` `Motion Controller`) "Left") :`false` "Right" :`true` "Left" :!type "EControllerHand Enum") Scale false))))

(fn `Slot  config`
  (params (`Hide Outer ring ` :type Boolean) (`Hide Empty slot Icon` :type Boolean) (`Hide Slot text` :type Boolean) (`Slot color` :type "LinearColor Structure") (`Outer Ring Color` :type "LinearColor Structure") (`Slot Mat Opacity` :type Boolean) (`Slot Type` :type "/Game/VR_Inventorys/Blueprints/Enum_Inventory_slotType Enum" :default "NewEnumerator0") (Holster :type Boolean) (`Slot Detect Haptic` :type "HapticFeedbackEffect_Base Object Reference") (`Store Item Haptic` :type "HapticFeedbackEffect_Base Object Reference"))
  (bind _slot_dynamic_mat (`self.Slot Dynamic Mat`))
  (bind _ring_dynamic_mat (`self.Ring Dynamic Mat`))
  (`|ExecutionSequence`
    (:`then_0`
      (`SceneComponent.SetHiddenInGame` (`self.Ring mesh`) `Hide Outer ring ` false) ; Hide Outer Ring
    )
    (:`then_1`
      (`SceneComponent.SetHiddenInGame` (`self.Empty Icon`) `Hide Empty slot Icon` false) ; Hide Empty Icon
    )
    (:`then_2`
      (`SceneComponent.SetHiddenInGame` (`self.TextRender`) `Hide Slot text` false) ; Hide Slot Info Text
    )
    (:`then_3`
      (`/Engine/EditorBlueprintResources/StandardMacros.IsValid` _slot_dynamic_mat
        (:`Is Valid`
          (`MaterialInstanceDynamic.SetVectorParameterValue` _slot_dynamic_mat "Color" `Slot color`))))
    (:`then_4`
      (`/Engine/EditorBlueprintResources/StandardMacros.IsValid` _ring_dynamic_mat
        (:`Is Valid`
          (`MaterialInstanceDynamic.SetVectorParameterValue` _ring_dynamic_mat "Color" `Outer Ring Color`))))
    (:`then_5`
      (if `Slot Mat Opacity`
        (`MaterialInstanceDynamic.SetScalarParameterValue` (`self.Slot Dynamic Mat`) "MinOpacity" 0.1)))
    (:`then_7`
      ;[1 1 1] Set Haptic effects from slot Config, If nonthing is set Use a Default Haptic effect to avoid the accessed None error!
      (`/Engine/EditorBlueprintResources/StandardMacros.IsValid` `Store Item Haptic`
        (:`Is Valid`
          (set `self.Slot Configuration Slotted Haptic Effect` `Store Item Haptic`))
        (:`Is Not Valid`
          (set `self.Slot Configuration Slotted Haptic Effect` "/Game/VR_Inventorys/VRTemplate/Haptics/HolsterSelectionHover.HolsterSelectionHover"))))
    (:`then_8`
      (`/Engine/EditorBlueprintResources/StandardMacros.IsValid` `Slot Detect Haptic`
        (:`Is Valid`
          (set `self.Slot Configuration Interaction Haptic Effect` `Slot Detect Haptic`))
        (:`Is Not Valid`
          (set `self.Slot Configuration Interaction Haptic Effect` "/Game/VR_Inventorys/VRTemplate/Haptics/SelectionHover.SelectionHover"))))))

(fn `Slot Active`
  (params (`Held Actors VRM component` :type "/Game/VR_Inventorys/Blueprints/BP_VRM_GrabComponent Object Reference") (`Motion Controller Component` :type "MotionControllerComponent Object Reference"))
  (bind _slot_in_use (`self.Slot in Use`))
  (bind ((`ShowEmptySlotIcon_79_BFEDBC684B17D2BE30463896FD1CEC38` _showemptysloticon) (`SizeScalingonInteraction_55_BAA059FB41407982711FEBBA1F6F84F4` _sizescalingoninteraction) (`SlotscaleUpsize_73_923574E5446D1230387D65851947F746` _slotscaleupsize) (`ScaleUpslotteditem_78_288B1C1444F3DFCA92281CBACC80B9EE` _scaleupslotteditem) (`OpacityScalingonInteraction_54_626E165C46B421ACC1644CBC32353E97` _opacityscalingoninteraction) (`RotationOnInteraction_56_D74C80B8485B45923B87E8B283B08BA6` _rotationoninteraction)) (break `/Game/VR_Inventorys/Blueprints/Struct_Slot_Config` (`self.Slot configuration`)))
  (`/Engine/EditorBlueprintResources/StandardMacros.IsValid` `Held Actors VRM component` ; Is Holding Object?
    (:`Is Valid`
      (if _slot_in_use
        (return)
        (elif (`|EnumEquality` (`/Game/VR_Inventorys/Blueprints/BP_VRM_GrabComponent.SlotType` `Held Actors VRM component`) (`.SlotType_25_B885963C4CDDD7F1300C869D53443260` (break `/Game/VR_Inventorys/Blueprints/Struct_Slot_Config` (`self.Slot configuration`))))
          _
          (else
            (return)))))
    (:`Is Not Valid`
      (if _slot_in_use
        _
        (else
          (return)))))
  (`self.Play Haptic Effect On correct hand` 1.0 `Motion Controller Component`)
  (`|ExecutionSequence`
    (:`then_0`
      (if _sizescalingoninteraction
        (`self.Scale Up Slot`)))
    (:`then_1`
      (if _opacityscalingoninteraction
        (`MaterialInstanceDynamic.SetScalarParameterValue` (`self.Slot Dynamic Mat`) "MinOpacity" 1.0)))
    (:`then_2`
      (if _rotationoninteraction
        (`self.Rotate Slot`)))))

(fn `Slot Deactivate`
  (params (`Held Component` :type "/Game/VR_Inventorys/Blueprints/BP_VRM_GrabComponent Object Reference"))
  (bind _slot_in_use (`self.Slot in Use`))
  (bind ((`SizeScalingonInteraction_55_BAA059FB41407982711FEBBA1F6F84F4` _sizescalingoninteraction) (`OpacityScalingonInteraction_54_626E165C46B421ACC1644CBC32353E97` _opacityscalingoninteraction) (`RotationOnInteraction_56_D74C80B8485B45923B87E8B283B08BA6` _rotationoninteraction)) (break `/Game/VR_Inventorys/Blueprints/Struct_Slot_Config` (`self.Slot configuration`)))
  (`/Engine/EditorBlueprintResources/StandardMacros.IsValid` `Held Component`
    (:`Is Valid`
      (if (not _slot_in_use)
        (`|ExecutionSequence` :!label _label
          (:`then_0`
            (if _opacityscalingoninteraction
              (`MaterialInstanceDynamic.SetScalarParameterValue` (`self.Slot Dynamic Mat`) "MinOpacity" 0.1)))
          (:`then_1`
            (if _rotationoninteraction
              (`self.Stop Slot rotation`)))
          (:`then_2`
            (if _sizescalingoninteraction
              (`self.Scale Down Slot`))))))
    (:`Is Not Valid`
      (if _slot_in_use
        (goto _label)))))

(fn `Update Slot Colour`
  (params (`Correct Colour` :type "LinearColor Structure") (`Wrong Colour` :type "LinearColor Structure"))
  (bind (_slot_configuration_dontshowouterring _slot_configuration_dontshowslottext _slot_configuration_showemptysloticon _slot_configuration_sizescalingoninteraction _slot_configuration_slotscaleupsize _slot_configuration_scaleupslotteditem _slot_configuration_opacityscalingoninteraction _slot_configuration_rotationoninteraction _slot_configuration_slotcolor _slot_configuration_outerringcolor _slot_configuration_slottype) (break `/Game/VR_Inventorys/Blueprints/Struct_Slot_Config` (`self.Slot configuration`)))
  (bind _slot_dynamic_mat (`self.Slot Dynamic Mat`))
  ;[0 0 0] Check slot type and change color for player Clue!
  (if (`|EnumEquality` (`/Game/VR_Inventorys/Blueprints/BP_VRM_GrabComponent.SlotType` (`self.Detected Item`)) _slot_configuration_slottype)
    (`MaterialInstanceDynamic.SetVectorParameterValue` _slot_dynamic_mat "Color" `Correct Colour`)
    (else
      (`MaterialInstanceDynamic.SetVectorParameterValue` _slot_dynamic_mat "Color" `Wrong Colour`)))
  (return))

(fn `Update Slot Opacity`
  (params (Value :type "Float (single-precision)"))
  (bind (_slot_configuration_dontshowouterring _slot_configuration_dontshowslottext _slot_configuration_showemptysloticon _slot_configuration_sizescalingoninteraction _slot_configuration_slotscaleupsize _slot_configuration_scaleupslotteditem _slot_configuration_opacityscalingoninteraction) (break `/Game/VR_Inventorys/Blueprints/Struct_Slot_Config` (`self.Slot configuration`)))
  (if _slot_configuration_opacityscalingoninteraction
    (`MaterialInstanceDynamic.SetScalarParameterValue` (`self.Slot Dynamic Mat`) "MinOpacity" Value)))

(fn `UserConstructionScript`)