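; Hatchete_bp is a VR inventory example item that, despite its name, serves as a grounding placard (TableGround) for training scenarios.
; When TableGround ends overlap with MainTable or Scenario 2, 6 or 7, it snap-attaches to that actor's ground point.
; Near-identical per-scenario graphs pick among three points by GroundTable flags, clearing them and TableInDrop after a delay.
; Scenario 7's second point also logs the "Grounded" placard step once to BP_Excel.
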(event `self.ReceiveBeginPlay`
  ;[1 1 1] Set Slot type
)

(event `self.TableGround.OnComponentEndOverlap`
  (params (OverlappedComponent :type "PrimitiveComponent Object Reference") (OtherActor :type "Actor Object Reference") (OtherComp :type "PrimitiveComponent Object Reference") (OtherBodyIndex :type Integer))
  (`|ExecutionSequence`
    (:`then_0`
      (bind _asscenario_2 (cast `/Game/BP/Scenario/Scenario_2` OtherActor))
      (`|ExecutionSequence`
        (:`then_0`
          (if (`self.GroundTable1`)
            (set `self.TableInDrop` true)
            (`SceneComponent.K2_AttachToComponent` (`self.TableGround`) (`/Game/BP/Scenario/Scenario_2.GroundPoint` _asscenario_2) "None" "SnapToTarget" "SnapToTarget" "KeepWorld" true)
            (`KismetSystemLibrary.Delay` 2.0)
            (set `self.GroundTable1` false)
            (set `self.TableInDrop` false)))
        (:`then_1`
          (if (`self.GroundTable2`)
            (set `self.TableInDrop` true)
            (`SceneComponent.K2_AttachToComponent` (`self.TableGround`) (`/Game/BP/Scenario/Scenario_2.GroundPoint1` _asscenario_2) "None" "SnapToTarget" "SnapToTarget" "KeepWorld" true)
            (`KismetSystemLibrary.Delay` 2.0)
            (set `self.GroundTable2` false)
            (set `self.TableInDrop` false)))
        (:`then_2`
          (if (`self.GroundTable3`)
            (set `self.TableInDrop` true)
            (`SceneComponent.K2_AttachToComponent` (`self.TableGround`) (`/Game/BP/Scenario/Scenario_2.GroundPoint2` _asscenario_2) "None" "SnapToTarget" "SnapToTarget" "KeepWorld" true)
            (`KismetSystemLibrary.Delay` 2.0)
            (set `self.GroundTable3` false)
            (set `self.TableInDrop` false)))))
    (:`then_1`
      (bind _asmain_table (cast `/Game/BP/Scenario/MainTable` OtherActor))
      (if (`self.GroundTable`)
        (`SceneComponent.K2_AttachToComponent` (`self.TableGround`) (`/Game/BP/Scenario/MainTable.MainTouchBoxGround` _asmain_table) "None" "SnapToTarget" "SnapToTarget" "KeepWorld" true)
        (set `self.GroundTable` false)
        (set `self.TableInDrop` false)))
    (:`then_2`
      (bind _asscenario_6 (cast `/Game/BP/Scenario/Scenario_6` OtherActor))
      (`|ExecutionSequence`
        (:`then_0`
          (if (`self.GroundTable1`)
            (set `self.TableInDrop` true)
            (`SceneComponent.K2_AttachToComponent` (`self.TableGround`) (`/Game/BP/Scenario/Scenario_6.GroundPoint` _asscenario_6) "None" "SnapToTarget" "SnapToTarget" "KeepWorld" true)
            (`KismetSystemLibrary.Delay` 2.0)
            (set `self.GroundTable1` false)
            (set `self.TableInDrop` false)))
        (:`then_1`
          (if (`self.GroundTable2`)
            (set `self.TableInDrop` true)
            (`SceneComponent.K2_AttachToComponent` (`self.TableGround`) (`/Game/BP/Scenario/Scenario_6.GroundPoint1` _asscenario_6) "None" "SnapToTarget" "SnapToTarget" "KeepWorld" true)
            (`KismetSystemLibrary.Delay` 2.0)
            (set `self.GroundTable2` false)
            (set `self.TableInDrop` false)))
        (:`then_2`
          (if (`self.GroundTable3`)
            (set `self.TableInDrop` true)
            (`SceneComponent.K2_AttachToComponent` (`self.TableGround`) (`/Game/BP/Scenario/Scenario_6.GroundPoint2` _asscenario_6) "None" "SnapToTarget" "SnapToTarget" "KeepWorld" true)
            (`KismetSystemLibrary.Delay` 2.0)
            (set `self.GroundTable3` false)
            (set `self.TableInDrop` false)))))
    (:`then_3`
      (bind _asscenario_7 (cast `/Game/BP/Scenario/Scenario_7` OtherActor))
      (`|ExecutionSequence`
        (:`then_0`
          (if (`self.GroundTable1`)
            (set `self.TableInDrop` true)
            (`SceneComponent.K2_AttachToComponent` (`self.TableGround`) (`/Game/BP/Scenario/Scenario_7.GroundPoint` _asscenario_7) "None" "SnapToTarget" "SnapToTarget" "KeepWorld" true)
            (`KismetSystemLibrary.Delay` 2.0)
            (set `self.GroundTable1` false)
            (set `self.TableInDrop` false)))
        (:`then_1`
          (if (`self.GroundTable2`)
            (set `self.TableInDrop` true)
            (`SceneComponent.K2_AttachToComponent` (`self.TableGround`) (`/Game/BP/Scenario/Scenario_7.GroundPoint1` _asscenario_7) "None" "SnapToTarget" "SnapToTarget" "KeepWorld" true)
            (`KismetSystemLibrary.Delay` 2.0)
            (set `self.GroundTable2` false)
            (set `self.TableInDrop` false)
            (`/Engine/EditorBlueprintResources/StandardMacros.DoOnce` false
              (:`Completed`
                (bind _outactors (`GameplayStatics.GetAllActorsOfClass` "/Game/Excel/BP_Excel.BP_Excel_C"))
                (`/Game/Excel/BP_Excel.SendToLog` (`|GetArrayItem` _outactors) "На привод ЛР 110 Алексеевская вывесить плакат «Заземлено»." "0")))))
        (:`then_2`
          (if (`self.GroundTable3`)
            (set `self.TableInDrop` true)
            (`SceneComponent.K2_AttachToComponent` (`self.TableGround`) (`/Game/BP/Scenario/Scenario_7.GroundPoint2` _asscenario_7) "None" "SnapToTarget" "SnapToTarget" "KeepWorld" true)
            (`KismetSystemLibrary.Delay` 2.0)
            (set `self.GroundTable3` false)
            (set `self.TableInDrop` false)))))))

(fn `UserConstructionScript`)