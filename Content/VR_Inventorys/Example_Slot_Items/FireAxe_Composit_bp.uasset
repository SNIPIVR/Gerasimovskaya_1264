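; FireAxe composite is a grabbable VR fire axe, one of the inventory system's example slot items.
; On BeginPlay it registers itself as the ActorKey of its Gloves widget.
; C_GrabComponent's first-hand grab shows that widget and messages the HandLeft or HandRight child actor, chosen by MotionSource, to snap the hand mesh into position.
; Dropping the first hand hides the widget again.
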(event `self.ReceiveBeginPlay`
  ;[0.5028 1 0] Set Slot Type & Initial SETUP for Custom slotted and Holstered Transfroms (BR)
  (`|ExecutionSequence`
    (:`then_1`
      (bind _asgloves_widget (cast `/Game/BP/Gloves/Gloves_widget` (`WidgetComponent.GetUserWidgetObject` (`self.Widget`))))
      (set `/Game/BP/Gloves/Gloves_widget.ActorKey` self _asgloves_widget))))

(event `/Game/BP/Gloves/GlovesControl.Gloves`
  (params (CheckGloves :type Boolean) (PutOnGloves :type Boolean) (TakeOffGloves :type Boolean)))

(event `self.C_GrabComponent.FirstHandGrabbed`
  (params (`Motion Controller` :type "MotionControllerComponent Object Reference") (SkeltalMeshHand :type "SkeletalMeshComponent Object Reference") (`Motion Controller Aim` :type "MotionControllerComponent Object Reference"))
  (`SceneComponent.SetVisibility` (`self.Widget`) true false)
  (if (== (`MotionControllerComponent.MotionSource` `Motion Controller`) "Left")
    (message `/Game/GDXR_VR_Template/Blueprints/Interfaces/BPI_HandSnapping.SnapHandPosition` (`ChildActorComponent.ChildActor` (`self.HandLeft`)) SkeltalMeshHand null)
    (else
      (message `/Game/GDXR_VR_Template/Blueprints/Interfaces/BPI_HandSnapping.SnapHandPosition` (`ChildActorComponent.ChildActor` (`self.HandRight`)) SkeltalMeshHand null))))

(event `self.C_GrabComponent.FirstHandDropped`
  (params (`Original Hand Location` :type "Transform Structure") (`Motion Controller` :type "MotionControllerComponent Object Reference") (`Skeletal Mesh Hand` :type "SkeletalMeshComponent Object Reference"))
  (`SceneComponent.SetVisibility` (`self.Widget`) false false))

(fn `UserConstructionScript`)