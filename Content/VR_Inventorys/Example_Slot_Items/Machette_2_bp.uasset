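; VR grabbable blocking key (named Machette_2_bp) that locks into interlock holes on disconnect knives and cell doors.
; When the first hand drops it, a chain of Attach flags selects the target and snaps BlockKey to its AttractionPoint.
; Knife branches set stop-rotate flags on hard-indexed ActorKnife entries; the door branch runs three scenario macros.
; Flags clear after short delays, and some branches log the insertion once to BP_Excel.
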(event `self.ReceiveBeginPlay`
  ;[1 1 1] Set Slot type
)

(event `self.ReceiveTick`
  (params (DeltaSeconds :type "Float (single-precision)")))

(event `self.BlockKey.OnComponentEndOverlap`
  (params (OverlappedComponent :type "PrimitiveComponent Object Reference") (OtherActor :type "Actor Object Reference") (OtherComp :type "PrimitiveComponent Object Reference") (OtherBodyIndex :type Integer)))

(event `self.BlockKey.OnComponentBeginOverlap`
  (params (OverlappedComponent :type "PrimitiveComponent Object Reference") (OtherActor :type "Actor Object Reference") (OtherComp :type "PrimitiveComponent Object Reference") (OtherBodyIndex :type Integer) (bFromSweep :type Boolean) (SweepResult :type "HitResult Structure (by ref)")))

(event `self.C_GrabComponent.FirstHandDropped`
  (params (`Original Hand Location` :type "Transform Structure") (`Motion Controller` :type "MotionControllerComponent Object Reference") (`Skeletal Mesh Hand` :type "SkeletalMeshComponent Object Reference"))
  (if (`self.Attach?`)
    (bind _ashole_block_key (cast `/Game/StaticObject/DopObject/BlockKey/HoleBlockKey` (`|GetArrayItem` (`self.ActorBlock`))))
    (`SceneComponent.K2_AttachToComponent` (`self.BlockKey`) (`/Game/StaticObject/DopObject/BlockKey/HoleBlockKey.AttractionPoint` _ashole_block_key) "None" "SnapToTarget" "SnapToTarget" "KeepWorld" true)
    (`/Engine/EditorBlueprintResources/StandardMacros.DoOnce` false :!label _label
      (:`Completed`
        (`|ExecutionSequence`
          (:`then_0`
            (bind _asdisconnect_knives (cast `/Game/BP/DisconnectKnives/DisconnectKnives` (`|GetArrayItem` (`self.ActorKnife`))))
            (set `/Game/BP/DisconnectKnives/DisconnectKnives.StopRotate` true _asdisconnect_knives))
          (:`then_1`
            (`KismetSystemLibrary.Delay` 0.2)
            (`|ExecutionSequence`
              (:`then_0`
                (set `self.Attach?` false)
                (goto _label :!via `Reset`))
              (:`then_1`
                (`/Engine/EditorBlueprintResources/StandardMacros.DoOnce` false
                  (:`Completed`
                    (bind _outactors (`GameplayStatics.GetAllActorsOfClass` "/Game/Excel/BP_Excel.BP_Excel_C"))
                    (`/Game/Excel/BP_Excel.SendToLog` (`|GetArrayItem` _outactors) "Вставить блокировочный ключ." "0"))))))
          (:`then_2`
            (bind _asdisconnect_knives_2 (cast `/Game/BP/DisconnectKnives/DisconnectKnives` (`|GetArrayItem` (`self.ActorKnife`) 1)))
            (set `/Game/BP/DisconnectKnives/DisconnectKnives.StopRotate` true _asdisconnect_knives_2))
          (:`then_3`
            (bind _asdisconnect_knives_3 (cast `/Game/BP/DisconnectKnives/DisconnectKnives` (`|GetArrayItem` (`self.ActorKnife`) 7)))
            (set `/Game/BP/DisconnectKnives/DisconnectKnives.StopRotate` true _asdisconnect_knives_3)))))
    (elif (`self.AttachDoor?`)
      (`|ExecutionSequence`
        (:`then_0`
          (bind _ascell_input_door_2sceanari (cast `/Game/cupboard/ZRU_Cell_DOOR/Cell_Input_Door_2Sceanari` (`|GetArrayItem` (`self.ActorBlock`) 1)))
          (`SceneComponent.K2_AttachToComponent` (`self.BlockKey`) (`/Game/cupboard/ZRU_Cell_DOOR/Cell_Input_Door_2Sceanari.AttractionPoint` _ascell_input_door_2sceanari) "None" "SnapToTarget" "SnapToTarget" "KeepWorld" true)
          (`KismetSystemLibrary.Delay` 0.2)
          (`|ExecutionSequence`
            (:`then_0`
              (`KismetSystemLibrary.Delay` 2.0)
              (set `self.AttachDoor?` false))
            (:`then_1`
              (`/Engine/EditorBlueprintResources/StandardMacros.DoOnce` false
                (:`Completed`
                  (bind _outactors_2 (`GameplayStatics.GetAllActorsOfClass` "/Game/Excel/BP_Excel.BP_Excel_C"))
                  (`/Game/Excel/BP_Excel.SendToLog` (`|GetArrayItem` _outactors_2) "Вставить блокировочный ключ." "0"))))))
        (:`then_1`
          (bind _ascell_input_door_2sceanari_1 (cast `/Game/cupboard/ZRU_Cell_DOOR/Cell_Input_Door_2Sceanari1` (`|GetArrayItem` (`self.ActorBlock`) 5)))
          (`SceneComponent.K2_AttachToComponent` (`self.BlockKey`) (`/Game/cupboard/ZRU_Cell_DOOR/Cell_Input_Door_2Sceanari1.AttractionPoint` _ascell_input_door_2sceanari_1) "None" "SnapToTarget" "SnapToTarget" "KeepWorld" true)
          (`|ExecutionSequence`
            (:`then_0`
              (`KismetSystemLibrary.Delay` 2.0)
              (set `self.AttachDoor?` false))
            (:`then_1`
              (`/Engine/EditorBlueprintResources/StandardMacros.DoOnce` false
                (:`Completed`
                  (bind _outactors_3 (`GameplayStatics.GetAllActorsOfClass` "/Game/Excel/BP_Excel.BP_Excel_C"))
                  (`/Game/Excel/BP_Excel.SendToLog` (`|GetArrayItem` _outactors_3) "Вставить блокировочный ключ." "0"))))))
        (:`then_2`
          (bind _ascell_input_door_2sceanari_6 (cast `/Game/cupboard/ZRU_Cell_DOOR/Scenar6/Cell_Input_Door_2Sceanari6` (`|GetArrayItem` (`self.ActorBlock`) 6)))
          (`SceneComponent.K2_AttachToComponent` (`self.BlockKey`) (`/Game/cupboard/ZRU_Cell_DOOR/Scenar6/Cell_Input_Door_2Sceanari6.AttractionPoint` _ascell_input_door_2sceanari_6) "None" "SnapToTarget" "SnapToTarget" "KeepWorld" true)
          (`KismetSystemLibrary.Delay` 0.2)
          (`|ExecutionSequence`
            (:`then_0`
              (`KismetSystemLibrary.Delay` 2.0)
              (set `self.AttachDoor?` false)))))
      (elif (`self.Attach35?`)
        (bind _ashole_block_key_35 (cast `/Game/StaticObject/DopObject/BlockKey/HoleBlockKey35` (`|GetArrayItem` (`self.ActorBlock`) 2)))
        (`SceneComponent.K2_AttachToComponent` (`self.BlockKey`) (`/Game/StaticObject/DopObject/BlockKey/HoleBlockKey35.AttractionPoint` _ashole_block_key_35) "None" "SnapToTarget" "SnapToTarget" "KeepWorld" true)
        (`/Engine/EditorBlueprintResources/StandardMacros.DoOnce` false :!label _label_2
          (:`Completed`
            (`|ExecutionSequence`
              (:`then_0`
                (bind _as3_1_a3 (cast `/Game/BP/DisconnectKnives/3_1_A3` (`|GetArrayItem` (`self.ActorKnife`) 2)))
                (set `/Game/BP/DisconnectKnives/3_1_A3.StopRotate` true _as3_1_a3))
              (:`then_1`
                (`KismetSystemLibrary.Delay` 0.2)
                (`|ExecutionSequence`
                  (:`then_0`
                    (set `self.Attach35?` false)
                    (goto _label_2 :!via `Reset`))
                  (:`then_1`
                    (`/Engine/EditorBlueprintResources/StandardMacros.DoOnce` false
                      (:`Completed`
                        (bind _outactors_4 (`GameplayStatics.GetAllActorsOfClass` "/Game/Excel/BP_Excel.BP_Excel_C"))
                        (`/Game/Excel/BP_Excel.SendToLog` (`|GetArrayItem` _outactors_4) "Вставить блокировочный ключ." "0"))))))
              (:`then_2`
                (bind _as3_1_a3_2 (cast `/Game/BP/DisconnectKnives/3_1_A3` (`|GetArrayItem` (`self.ActorKnife`) 3)))
                (set `/Game/BP/DisconnectKnives/3_1_A3.StopRotate` true _as3_1_a3_2))
              (:`then_3`
                (bind _as3_1_a3_3 (cast `/Game/BP/DisconnectKnives/3_1_A3` (`|GetArrayItem` (`self.ActorKnife`) 6)))
                (set `/Game/BP/DisconnectKnives/3_1_A3.StopRotate` true _as3_1_a3_3)))))
        (elif (`self.AttachSHR?`)
          (bind _ashole_block_shr (cast `/Game/StaticObject/DopObject/BlockKey/HoleBlockSHR` (`|GetArrayItem` (`self.ActorBlock`) 3)))
          (`SceneComponent.K2_AttachToComponent` (`self.BlockKey`) (`/Game/StaticObject/DopObject/BlockKey/HoleBlockSHR.AttractionPoint` _ashole_block_shr) "None" "SnapToTarget" "SnapToTarget" "KeepWorld" true)
          (`/Engine/EditorBlueprintResources/StandardMacros.DoOnce` false :!label _label_3
            (:`Completed`
              (bind _as3_1_a3_scenar_3 (cast `/Game/BP/DisconnectKnives/3_1_A3_Scenar3` (`|GetArrayItem` (`self.ActorKnife`) 4)))
              (set `/Game/BP/DisconnectKnives/3_1_A3_Scenar3.StopRotate` true _as3_1_a3_scenar_3)
              (`KismetSystemLibrary.Delay` 0.2)
              (`|ExecutionSequence`
                (:`then_0`
                  (set `self.AttachSHR?` false)
                  (goto _label_3 :!via `Reset`)))))
          (elif (`self.AttachLR?`)
            (bind _ashole_block_lr (cast `/Game/StaticObject/DopObject/BlockKey/HoleBlockLR` (`|GetArrayItem` (`self.ActorBlock`) 4)))
            (`SceneComponent.K2_AttachToComponent` (`self.BlockKey`) (`/Game/StaticObject/DopObject/BlockKey/HoleBlockLR.AttractionPoint` _ashole_block_lr) "None" "SnapToTarget" "SnapToTarget" "KeepWorld" true)
            (`/Engine/EditorBlueprintResources/StandardMacros.DoOnce` false :!label _label_4
              (:`Completed`
                (bind _as3_2_a3_scenar_3 (cast `/Game/BP/DisconnectKnives/3_2_A3_Scenar3` (`|GetArrayItem` (`self.ActorKnife`) 5)))
                (set `/Game/BP/DisconnectKnives/3_2_A3_Scenar3.StopRotate` true _as3_2_a3_scenar_3)
                (`KismetSystemLibrary.Delay` 0.2)
                (`|ExecutionSequence`
                  (:`then_0`
                    (set `self.AttachLR?` false)
                    (goto _label_4 :!via `Reset`)))))
            (elif (`self.AttachTH1`)
              (bind _ashole_block_th1 (cast `/Game/StaticObject/DopObject/BlockKey/HoleBlockTH1` (`|GetArrayItem` (`self.ActorBlock`) 7)))
              (`SceneComponent.K2_AttachToComponent` (`self.BlockKey`) (`/Game/StaticObject/DopObject/BlockKey/HoleBlockTH1.AttractionPoint` _ashole_block_th1) "None" "SnapToTarget" "SnapToTarget" "KeepWorld" true)
              (`/Engine/EditorBlueprintResources/StandardMacros.DoOnce` false :!label _label_5
                (:`Completed`
                  (bind _as03_04_th1 (cast `/Game/BP/DisconnectKnives/03_04_TH1` (`|GetArrayItem` (`self.ActorKnife`) 8)))
                  (set `/Game/BP/DisconnectKnives/03_04_TH1.StopRotate2` true _as03_04_th1)
                  (`KismetSystemLibrary.Delay` 0.2)
                  (`|ExecutionSequence`
                    (:`then_0`
                      (set `self.AttachTH1` false)
                      (goto _label_5 :!via `Reset`)))))
              (elif (`self.AttachLRAex`)
                (bind _ashole_block_key_lralex_110 (cast `/Game/StaticObject/DopObject/BlockKey/HoleBlockKeyLRAlex110` (`|GetArrayItem` (`self.ActorBlock`) 8)))
                (`SceneComponent.K2_AttachToComponent` (`self.BlockKey`) (`/Game/StaticObject/DopObject/BlockKey/HoleBlockKeyLRAlex110.AttractionPoint` _ashole_block_key_lralex_110) "None" "SnapToTarget" "SnapToTarget" "KeepWorld" true)
                (`/Engine/EditorBlueprintResources/StandardMacros.DoOnce` false :!label _label_6
                  (:`Completed`
                    (bind _asdisconnect_knives_lr110alex (cast `/Game/BP/DisconnectKnives/DisconnectKnivesLR110Alex` (`|GetArrayItem` (`self.ActorKnife`) 9)))
                    (set `/Game/BP/DisconnectKnives/DisconnectKnivesLR110Alex.StopRotate2` true _asdisconnect_knives_lr110alex)
                    (`KismetSystemLibrary.Delay` 0.2)
                    (`|ExecutionSequence`
                      (:`then_0`
                        (set `self.AttachLRAex` false)
                        (goto _label_6 :!via `Reset`)))))))))))))

(event `self.C_GrabComponent.PhysicsVolumeChangedDelegate`
  (params (NewVolume :type "PhysicsVolume Object Reference")))

(fn `UserConstructionScript`)