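; Grabbable VR prop, named as a flashlight, that acts as a video recorder the player switches on by hand.
; Grabbing it snaps the matching left or right hand pose after a short delay.
; A VR hand touching ActivateReg sets emissive camera materials and, once only, turns the indicator green and logs activation to BP_Excel.
; The Box overlap FlipFlop drives nothing, and slot setup and weapon input-mapping logic are unwired.
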(event `self.C_GrabComponent.FirstHandGrabbed`
  (params (`Motion Controller` :type "MotionControllerComponent Object Reference") (SkeltalMeshHand :type "SkeletalMeshComponent Object Reference") (`Motion Controller Aim` :type "MotionControllerComponent Object Reference"))
  (`KismetSystemLibrary.Delay` 0.1)
  (if (== (`MotionControllerComponent.MotionSource` `Motion Controller`) "Left")
    (message `/Game/GDXR_VR_Template/Blueprints/Interfaces/BPI_HandSnapping.SnapHandPosition` (`ChildActorComponent.ChildActor` (`self.HandLeft`)) SkeltalMeshHand null)
    (else
      (message `/Game/GDXR_VR_Template/Blueprints/Interfaces/BPI_HandSnapping.SnapHandPosition` (`ChildActorComponent.ChildActor` (`self.HandRight`)) SkeltalMeshHand null))))

(event `self.TriggerPressed`)

(event `self.Box.OnComponentBeginOverlap`
  (params (OverlappedComponent :type "PrimitiveComponent Object Reference") (OtherActor :type "Actor Object Reference") (OtherComp :type "PrimitiveComponent Object Reference") (OtherBodyIndex :type Integer) (bFromSweep :type Boolean) (SweepResult :type "HitResult Structure (by ref)"))
  (if (`self.ActorHasTag` OtherActor "VR Hand")
    (`/Engine/EditorBlueprintResources/StandardMacros.FlipFlop`)))

(event `self.C_GrabComponent.FirstHandDropped`
  (params (`Original Hand Location` :type "Transform Structure") (`Motion Controller` :type "MotionControllerComponent Object Reference") (`Skeletal Mesh Hand` :type "SkeletalMeshComponent Object Reference")))

(event `self.ActivateReg.OnComponentBeginOverlap`
  (params (OverlappedComponent :type "PrimitiveComponent Object Reference") (OtherActor :type "Actor Object Reference") (OtherComp :type "PrimitiveComponent Object Reference") (OtherBodyIndex :type Integer) (bFromSweep :type Boolean) (SweepResult :type "HitResult Structure (by ref)"))
  (if (`ActorComponent.ComponentHasTag` OtherComp "VR Hand")
    (`PrimitiveComponent.SetMaterial` (`self.Camera`) 2 "/Game/StaticObject/ScenarioObject/Camera/Material_Imissive.Material_Imissive")
    (`/Engine/EditorBlueprintResources/StandardMacros.DoOnce` false
      (:`Completed`
        (`PrimitiveComponent.SetMaterial` (`self.Camera`) 5 "/Game/cupboard/Materials/Green_Light_Emissive.Green_Light_Emissive")
        (bind _outactors (`GameplayStatics.GetAllActorsOfClass` "/Game/Excel/BP_Excel.BP_Excel_C"))
        (`/Game/Excel/BP_Excel.SendToLog` (`|GetArrayItem` _outactors) "ОПУ_Видеорегистратор" "default_activate" "")))))

(fn `UserConstructionScript`)