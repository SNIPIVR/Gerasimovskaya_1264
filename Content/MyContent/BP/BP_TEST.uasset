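; BP_TEST is a test Blueprint that changes the material on its Cube component to show one of five scenarios.
; Five scenario events, whose BI prefix suggests Blueprint Interface calls, each set a different fixed material on the cube's first slot.
; The first event also prints a debug string, and the construction script is empty.
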(event `/Game/BP/Blueprints/UI/MainMenu/BPI_Menu.BI_Scenar1`
  (`KismetSystemLibrary.PrintString` "WORK1")
  (`PrimitiveComponent.SetMaterial` (`self.Cube`) 0 "/Game/Materials/Metal/Alumin.Alumin"))

(event `/Game/BP/Blueprints/UI/MainMenu/BPI_Menu.BI_Scenar2`
  (`PrimitiveComponent.SetMaterial` (`self.Cube`) 0 "/Game/StaticObject/05_softORY/Alumosteel_Cable.Alumosteel_Cable"))

(event `/Game/BP/Blueprints/UI/MainMenu/BPI_Menu.BI_Scenar3`
  (`PrimitiveComponent.SetMaterial` (`self.Cube`) 0 "/Game/VR_Inventorys/Example_Slot_Items/Example_PickUp_Items_source/MeleeWeapons/Materials/Baseball_bat_Blue_metal_mat.Baseball_bat_Blue_metal_mat"))

(event `/Game/BP/Blueprints/UI/MainMenu/BPI_Menu.BI_Scenar4`
  (`PrimitiveComponent.SetMaterial` (`self.Cube`) 0 "/Game/StaticObject/DopObject/Interior/Phone/Cisco_Phone_CP_6941_labels.Cisco_Phone_CP_6941_labels"))

(event `/Game/BP/Blueprints/UI/MainMenu/BPI_Menu.BI_Scenar5`
  (`PrimitiveComponent.SetMaterial` (`self.Cube`) 0 "/Game/VR_Inventorys/Example_Slot_Items/Example_PickUp_Items_source/MeleeWeapons/Materials/FireAxe_mat.FireAxe_mat"))

(fn `UserConstructionScript`)