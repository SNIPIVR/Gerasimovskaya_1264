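; VR body item storage that acts as a holster rig following the player.
; On BeginPlay it enables touch-button input and, if AutoAttachToPlayer is set, attaches to the player character and starts a looping timer.
; The timer keeps the root under the camera, snapping horizontally while easing yaw and height.
; Right A toggles the mesh between its origin and far below; code spawning default items into child storage slots is unwired.
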(event `EnhancedInput|/Game/GDXR_VR_Template/Input/Actions/IA_TouchButtonRightA`
  (params (ActionValue :type Boolean) (ElapsedSeconds :type "Float (double-precision)") (TriggeredSeconds :type "Float (double-precision)") (InputAction :type "InputAction Object Reference" :default "/Game/GDXR_VR_Template/Input/Actions/IA_TouchButtonRightA.IA_TouchButtonRightA"))
  (bind _staticmesh (`self.StaticMesh`))
  (:`Started`
    (`/Engine/EditorBlueprintResources/StandardMacros.FlipFlop`
      (:`A`
        (`SceneComponent.K2_SetRelativeLocation` _staticmesh (0.0 0.0 -500.0) false false))
      (:`B`
        (`SceneComponent.K2_SetRelativeLocation` _staticmesh (0.0 0.0 0.0) false false)))))

(event `self.ReceiveBeginPlay`
  (bind _returnvalue (`GameplayStatics.GetPlayerCharacter` 0))
  (`|ExecutionSequence`
    (:`then_0`
      (`self.EnableInput` (`GameplayStatics.GetPlayerController` 0))
      (`EnhancedInputSubsystemInterface.AddMappingContext` (pcsubsystem `EnhancedInputLocalPlayerSubsystem` (`GameplayStatics.GetPlayerController` 0)) "/Game/GDXR_VR_Template/Input/IMC_TouchButton.IMC_TouchButton" 0 (struct)))
    (:`then_1`
      (if (`self.AutoAttachToPlayer?`)
        (`/Engine/EditorBlueprintResources/StandardMacros.IsValid` _returnvalue
          (:`Is Valid`
            (`self.K2_AttachToActor` _returnvalue "None" "SnapToTarget" "SnapToTarget" "SnapToTarget")
            (bind _returnvalue_2 (`KismetSystemLibrary.K2_SetTimerDelegate` (delegate `Update Holster Rotation`) 0.02 true))))))))

(event `self.ReceiveTick`
  (params (DeltaSeconds :type "Float (single-precision)")))

(event `Update Holster Rotation`
  (bind _defaultsceneroot (`self.DefaultSceneRoot`))
  (bind _returnvalue (`self.GetComponentByClass` (`GameplayStatics.GetPlayerCharacter` 0) "/Script/Engine.CameraComponent"))
  (bind (_returnvalue_x _returnvalue_y _returnvalue_z) (`KismetMathLibrary.BreakVector` (`SceneComponent.K2_GetComponentLocation` (`self.DefaultSceneRoot`))))
  (bind (_returnvalue_x_2 _returnvalue_y_2 _returnvalue_z_2) (`KismetMathLibrary.BreakVector` (`SceneComponent.K2_GetComponentLocation` _returnvalue)))
  (bind _returnvalue_2 (`KismetSystemLibrary.K2_GetTimerElapsedTimeHandle` (stale `self.ReceiveBeginPlay` _returnvalue_2)))
  (bind (_returnvalue_roll _returnvalue_pitch _returnvalue_yaw) (`KismetMathLibrary.BreakRotator` (`KismetMathLibrary.RInterpTo` (`SceneComponent.K2_GetComponentRotation` _defaultsceneroot) (`SceneComponent.K2_GetComponentRotation` _returnvalue) _returnvalue_2 0.15)))
  (`SceneComponent.K2_SetWorldRotation` _defaultsceneroot (`KismetMathLibrary.MakeRotator` 0.0 0.0 _returnvalue_yaw) false false)
  (`SceneComponent.K2_SetWorldLocation` _defaultsceneroot (`KismetMathLibrary.MakeVector` _returnvalue_x_2 _returnvalue_y_2 (`KismetMathLibrary.FInterpTo` _returnvalue_z (- _returnvalue_z_2 70.0) _returnvalue_2 0.15)) true false))

(fn `UserConstructionScript`)