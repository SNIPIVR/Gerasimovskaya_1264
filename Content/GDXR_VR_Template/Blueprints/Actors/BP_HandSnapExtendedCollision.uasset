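; VR hand snap point with a box collision that locks a hand mesh to an authored pose, optionally acting as a climbable grip.
; At BeginPlay it removes its static mesh and, when CanClimb is set, switches the box to a custom object channel with query and physics collision.
; SnapHandPosition messages the player character to attach the hand at the Arrow component with a custom blend space, then calls HandAttached.
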(event `self.ReceiveBeginPlay`
  (bind _box_collision (`self.Box Collision`))
  (`ActorComponent.K2_DestroyComponent` (`self.StaticMesh`))
  (if (`self.CanClimb?`)
    (`PrimitiveComponent.SetCollisionObjectType` _box_collision "ECC_GameTraceChannel4")
    (`PrimitiveComponent.SetCollisionEnabled` _box_collision "QueryAndPhysics")))

(event `self.SnapHandPosition`
  (params (`Hand Skeletal Mesh` :type "SkeletalMeshComponent Object Reference") (`Motion Controller` :type "MotionControllerComponent Object Reference"))
  (bind _arrow (`self.Arrow`))
  (message `/Game/GDXR_VR_Template/Blueprints/Interfaces/BPI_HandSnapping.AttachHandToObject` (`GameplayStatics.GetPlayerCharacter` 0) (`SceneComponent.K2_GetComponentToWorld` _arrow) `Hand Skeletal Mesh` (`self.Custom Anim Blend Space`) _arrow `Motion Controller`)
  (`self.Hand Attached`))

(fn `UserConstructionScript`)