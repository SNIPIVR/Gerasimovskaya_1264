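; BP_KeyCard_03 is a grabbable VR key card actor.
; When first grabbed, it checks the motion controller's hand and messages the matching left or right snap child actor to position the hand mesh on the card.
; When dropped, it sets mesh physics simulation according to StatePhys.
; The Activation and StateOfPhys events are present but have no logic attached.
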(event `self.Activation`
  (params (State :type Boolean))
  ;[1 1 1] has key card been activated.
)

(event `self.C_GrabComponent.FirstHandGrabbed`
  (params (`Motion Controller` :type "MotionControllerComponent Object Reference") (SkeltalMeshHand :type "SkeletalMeshComponent Object Reference") (`Motion Controller Aim` :type "MotionControllerComponent Object Reference"))
  ;[1 1 1] Snap Hand to location
  (if (== (`MotionControllerComponent.MotionSource` `Motion Controller`) "Left")
    (message `/Game/GDXR_VR_Template/Blueprints/Interfaces/BPI_HandSnapping.SnapHandPosition` (`ChildActorComponent.ChildActor` (`self.SnapHandLeft`)) SkeltalMeshHand null)
    (else
      (message `/Game/GDXR_VR_Template/Blueprints/Interfaces/BPI_HandSnapping.SnapHandPosition` (`ChildActorComponent.ChildActor` (`self.SnapHandRight`)) SkeltalMeshHand null))))

(event `self.C_GrabComponent.FirstHandDropped`
  (params (`Original Hand Location` :type "Transform Structure") (`Motion Controller` :type "MotionControllerComponent Object Reference") (`Skeletal Mesh Hand` :type "SkeletalMeshComponent Object Reference"))
  (if (stale `self.StateOfPhys` StatePhys)
    (`PrimitiveComponent.SetSimulatePhysics` (`self.StaticMesh`) true)
    (else
      (`PrimitiveComponent.SetSimulatePhysics` (`self.StaticMesh`) false))))

(event `self.StateOfPhys`
  (params (StatePhys :type Boolean)))

(fn `UserConstructionScript`)