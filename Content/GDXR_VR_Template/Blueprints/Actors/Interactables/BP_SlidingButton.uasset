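; VR sliding button that drives the text, and in one step the image material, of a TV_Guide screen.
; While a component overlaps the collider, a looping timer moves the mesh to that component's closest point on the line between two spline points.
; Reaching the far point fires once, using a MultiGate indexed by a counter to select the guide step and toggle the mesh's visibility.
; Ending overlap pauses the timer, slides the mesh back and re-arms the trigger.
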(event `self.Col.OnComponentBeginOverlap`
  (params (OverlappedComponent :type "PrimitiveComponent Object Reference") (OtherActor :type "Actor Object Reference") (OtherComp :type "PrimitiveComponent Object Reference") (OtherBodyIndex :type Integer) (bFromSweep :type Boolean) (SweepResult :type "HitResult Structure (by ref)"))
  (set `self.Other Comp` OtherComp)
  (bind _returnvalue (`KismetSystemLibrary.K2_SetTimerDelegate` (delegate `Update Draw Position`) 0.02 true))
  (set `self.TimerHandle` _returnvalue))

(event `Update Draw Position`
  (bind _spline (`self.Spline`))
  (bind _returnvalue (`SplineComponent.GetLocationAtSplinePoint` _spline 1 "World"))
  (bind _returnvalue_2 (`KismetMathLibrary.FindClosestPointOnSegment` (`SceneComponent.K2_GetComponentLocation` (`self.Other Comp`)) (`SplineComponent.GetLocationAtSplinePoint` _spline 0 "World") _returnvalue))
  (bind _returnvalue_3 (`KismetMathLibrary.VInterpTo` _returnvalue_2 _returnvalue_2 (`KismetMathLibrary.FClamp` (* (`KismetSystemLibrary.K2_GetTimerElapsedTimeHandle` (`self.TimerHandle`)) 1.5)) 2.0))
  (`SceneComponent.K2_SetWorldLocation` (`self.StaticMesh`) _returnvalue_3 true false)
  (if (== _returnvalue_3 _returnvalue :`ErrorTolerance` 0.05)
    (`/Engine/EditorBlueprintResources/StandardMacros.DoOnce` false :!label _label
      (:`Completed`
        (`KismetSystemLibrary.K2_PauseTimer` null "Update Draw Position")
        (set `self.Other Comp` null)
        (bind _astv_guide (cast `/Game/TrainingRoom/TV_Guide` (`self.BP_TV`)))
        (`|MultiGate` false false (`self.Num`) :!label _label_2
          (:`Out 1`
            (bind _text_guide (`/Game/TrainingRoom/TV_Guide.Text_Guide` _astv_guide))
            (`TextRenderComponent.K2_SetText` _text_guide (`self.Text_2`))
            (`SceneComponent.SetVisibility` (`self.StaticMesh`) true false)
            (`PrimitiveComponent.SetMaterial` (`/Game/TrainingRoom/TV_Guide.Guid_Img` _astv_guide) 0 (`self.Material`))
            (`KismetSystemLibrary.Delay` 0.1)
            (`/Engine/EditorBlueprintResources/StandardMacros.IncrementInt` (`self.Num`)
              (:`  `
                (goto _label_2 :!via `Reset`))))
          (:`Out 2`
            (`TextRenderComponent.K2_SetText` _text_guide (`self.Text_3`))
            (`SceneComponent.SetVisibility` (`self.StaticMesh`) false false)
            (`KismetSystemLibrary.Delay` 0.1)
            (set `self.Num` 0)
            (goto _label_2 :!via `Reset`)))))))

(event `self.StaticMesh.OnComponentBeginOverlap`
  (params (OverlappedComponent :type "PrimitiveComponent Object Reference") (OtherActor :type "Actor Object Reference") (OtherComp :type "PrimitiveComponent Object Reference") (OtherBodyIndex :type Integer) (bFromSweep :type Boolean) (SweepResult :type "HitResult Structure (by ref)")))

(event `self.Col.OnComponentEndOverlap`
  (params (OverlappedComponent :type "PrimitiveComponent Object Reference") (OtherActor :type "Actor Object Reference") (OtherComp :type "PrimitiveComponent Object Reference") (OtherBodyIndex :type Integer))
  (set `self.Other Comp` OtherComp)
  (`KismetSystemLibrary.K2_PauseTimerHandle` (`self.TimerHandle`))
  (`KismetSystemLibrary.MoveComponentTo` (`self.StaticMesh`) (`SplineComponent.GetLocationAtSplinePoint` (`self.Spline`) 0 "Local"))
  (`KismetSystemLibrary.Delay` 0.2)
  (goto _label :!via `Reset`))

(event `self.StaticMesh.OnComponentEndOverlap`
  (params (OverlappedComponent :type "PrimitiveComponent Object Reference") (OtherActor :type "Actor Object Reference") (OtherComp :type "PrimitiveComponent Object Reference") (OtherBodyIndex :type Integer)))

(fn `UserConstructionScript`)