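; BP_SlidingButtonOn is an interactable sliding button from the VR template, with a mesh constrained to a two-point spline.
; Overlapping its collision starts a looping timer that interpolates the mesh, with sweep, toward the closest segment point to its own location.
; Near the end point, a DoOnce issues a timer pause by function name.
; Ending overlap pauses the timer, moves the mesh back toward the start and re-arms the DoOnce.
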(event `self.Col.OnComponentBeginOverlap`
  (params (OverlappedComponent :type "PrimitiveComponent Object Reference") (OtherActor :type "Actor Object Reference") (OtherComp :type "PrimitiveComponent Object Reference") (OtherBodyIndex :type Integer) (bFromSweep :type Boolean) (SweepResult :type "HitResult Structure (by ref)"))
  (set `self.Other Comp` OtherComp)
  (bind _returnvalue (`KismetSystemLibrary.K2_SetTimerDelegate` (delegate `Update Draw Position`) 0.02 true))
  (set `self.TimerHandle` _returnvalue))

(event `Update Draw Position`
  (bind _spline (`self.Spline`))
  (bind _returnvalue (`SplineComponent.GetLocationAtSplinePoint` _spline 1 "World"))
  (bind _returnvalue_2 (`SceneComponent.K2_GetComponentLocation` (`self.StaticMesh`)))
  (bind _returnvalue_3 (`KismetMathLibrary.VInterpTo` _returnvalue_2 (`KismetMathLibrary.FindClosestPointOnSegment` _returnvalue_2 (`SplineComponent.GetLocationAtSplinePoint` _spline 0 "World") _returnvalue) (`KismetMathLibrary.FClamp` (* (`KismetSystemLibrary.K2_GetTimerElapsedTimeHandle` (`self.TimerHandle`)) 1.5)) 1.0))
  (`SceneComponent.K2_SetWorldLocation` (`self.StaticMesh`) _returnvalue_3 true false)
  (if (== _returnvalue_3 _returnvalue :`ErrorTolerance` 0.8)
    (`/Engine/EditorBlueprintResources/StandardMacros.DoOnce` false :!label _label
      (:`Completed`
        (`KismetSystemLibrary.K2_PauseTimer` null "Update Draw Position")))))

(event `self.StaticMesh.OnComponentBeginOverlap`
  (params (OverlappedComponent :type "PrimitiveComponent Object Reference") (OtherActor :type "Actor Object Reference") (OtherComp :type "PrimitiveComponent Object Reference") (OtherBodyIndex :type Integer) (bFromSweep :type Boolean) (SweepResult :type "HitResult Structure (by ref)")))

(event `self.Col.OnComponentEndOverlap`
  (params (OverlappedComponent :type "PrimitiveComponent Object Reference") (OtherActor :type "Actor Object Reference") (OtherComp :type "PrimitiveComponent Object Reference") (OtherBodyIndex :type Integer))
  (bind (_returnvalue_x _returnvalue_y _returnvalue_z) (`KismetMathLibrary.BreakVector` (`SplineComponent.GetLocationAtSplinePoint` (`self.Spline`) 0 "Local")))
  (set `self.Other Comp` OtherComp)
  (`KismetSystemLibrary.K2_PauseTimerHandle` (`self.TimerHandle`))
  (`KismetSystemLibrary.MoveComponentTo` (`self.StaticMesh`) (`KismetMathLibrary.MakeVector` 1.20838 _returnvalue_y _returnvalue_z) (struct))
  (`KismetSystemLibrary.Delay` 0.2)
  (goto _label :!via `Reset`))

(event `self.StaticMesh.OnComponentEndOverlap`
  (params (OverlappedComponent :type "PrimitiveComponent Object Reference") (OtherActor :type "Actor Object Reference") (OtherComp :type "PrimitiveComponent Object Reference") (OtherBodyIndex :type Integer)))

(fn `UserConstructionScript`)