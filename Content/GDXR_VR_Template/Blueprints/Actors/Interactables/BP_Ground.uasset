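; BP_Ground is a grabbable VR interactable that toggles a green ground activation state on other actors.
; On first-hand grab it snaps the hand to the left or right snap child actor, based on motion source.
; Grab and drop broadcast true or false to every BP_Ground_Interface actor, and drop also sets mesh physics simulation from StatePhys.
; Activation and StateOfPhys events are empty stubs.
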(event `self.Activation`
  (params (State :type Boolean))
  ;[1 1 1] has key card been activated.
)

(event `self.C_GrabComponent.FirstHandGrabbed`
  (params (`Motion Controller` :type "MotionControllerComponent Object Reference") (SkeltalMeshHand :type "SkeletalMeshComponent Object Reference") (`Motion Controller Aim` :type "MotionControllerComponent Object Reference"))
  (`|ExecutionSequence`
    (:`then_0`
      ;[1 1 1] Snap Hand to location
      (if (== (`MotionControllerComponent.MotionSource` `Motion Controller`) "Left")
        (message `/Game/GDXR_VR_Template/Blueprints/Interfaces/BPI_HandSnapping.SnapHandPosition` (`ChildActorComponent.ChildActor` (`self.SnapHandLeft`)) SkeltalMeshHand null)
        (else
          (message `/Game/GDXR_VR_Template/Blueprints/Interfaces/BPI_HandSnapping.SnapHandPosition` (`ChildActorComponent.ChildActor` (`self.SnapHandRight`)) SkeltalMeshHand null))))
    (:`then_1`
      (bind _outactors (`GameplayStatics.GetAllActorsWithInterface` "/Game/GDXR_VR_Template/Blueprints/Actors/Interactables/BP_Card/BP_Ground_Interface.BP_Ground_Interface_C"))
      (for _array_element _outactors
        (message `/Game/GDXR_VR_Template/Blueprints/Actors/Interactables/BP_Card/BP_Ground_Interface.GreenActivateGround` _array_element true)))))

(event `self.C_GrabComponent.FirstHandDropped`
  (params (`Original Hand Location` :type "Transform Structure") (`Motion Controller` :type "MotionControllerComponent Object Reference") (`Skeletal Mesh Hand` :type "SkeletalMeshComponent Object Reference"))
  (`|ExecutionSequence`
    (:`then_0`
      (if (stale `self.StateOfPhys` StatePhys)
        (`PrimitiveComponent.SetSimulatePhysics` (`self.StaticMesh`) true)
        (else
          (`PrimitiveComponent.SetSimulatePhysics` (`self.StaticMesh`) false))))
    (:`then_1`
      (bind _outactors (`GameplayStatics.GetAllActorsWithInterface` "/Game/GDXR_VR_Template/Blueprints/Actors/Interactables/BP_Card/BP_Ground_Interface.BP_Ground_Interface_C"))
      (for _array_element _outactors
        (message `/Game/GDXR_VR_Template/Blueprints/Actors/Interactables/BP_Card/BP_Ground_Interface.GreenActivateGround` _array_element false)))))

(event `self.StateOfPhys`
  (params (StatePhys :type Boolean)))

(fn `UserConstructionScript`)