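; VR interactable knife-disconnect handle that players grab and rotate to fire an activate event.
; Grabbing snaps the hand to a side-specific child actor and starts a looping timer that pitches the handle toward the controller using look-at and dot-product math.
; Nearly full rotation activates it once, while RequireRotation off skips rotation.
; Left-hand release also deactivates it and starts a timer, apparently easing the handle back; right-hand release only frees the hand.
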(event `self.C_GrabComponent.FirstHandGrabbed`
  (params (`Motion Controller` :type "MotionControllerComponent Object Reference") (SkeltalMeshHand :type "SkeletalMeshComponent Object Reference") (`Motion Controller Aim` :type "MotionControllerComponent Object Reference"))
  (bind _childactor (`ChildActorComponent.ChildActor` (`self.LeftHandSnap`)))
  (bind _childactor_2 (`ChildActorComponent.ChildActor` (`self.RightHandSnap`)))
  (bind _output_get (set `self.Motion Controller` `Motion Controller`))
  (bind _output_get_2 (set `self.Skeltal Mesh Hand` SkeltalMeshHand))
  (`KismetSystemLibrary.K2_SetTimerDelegate` (delegate `Update Rotation`) 0.02 true)
  (`self.HandleGrabbed` _output_get)
  (if (`self.Is on the Left  the door`)
    (if (== (`MotionControllerComponent.MotionSource` _output_get) "Left")
      (message `/Game/GDXR_VR_Template/Blueprints/Interfaces/BPI_HandSnapping.SnapHandPosition` _childactor _output_get_2 null)
      (else
        (message `/Game/GDXR_VR_Template/Blueprints/Interfaces/BPI_HandSnapping.SnapHandPosition` _childactor _output_get_2 null)))
    (elif (== (`MotionControllerComponent.MotionSource` _output_get) "Left")
      (message `/Game/GDXR_VR_Template/Blueprints/Interfaces/BPI_HandSnapping.SnapHandPosition` _childactor_2 _output_get_2 null)
      (else
        (message `/Game/GDXR_VR_Template/Blueprints/Interfaces/BPI_HandSnapping.SnapHandPosition` _childactor_2 _output_get_2 null)))))

(event `Update Rotation`
  (bind _handle (`self.handle`))
  (bind (_returnvalue_roll _returnvalue_pitch) (`KismetMathLibrary.BreakRotator` (`SceneComponent.K2_GetComponentRotation` _handle)))
  (bind (_returnvalue_roll_2 _returnvalue_pitch_2 _returnvalue_yaw) (`KismetMathLibrary.BreakRotator` (`KismetMathLibrary.FindLookAtRotation` (`SceneComponent.K2_GetComponentLocation` (`self.handle`)) (`SceneComponent.K2_GetComponentLocation` (`self.Motion Controller`)))))
  (if (`self.Require Rotation`)
    (`SceneComponent.K2_AddLocalRotation` _handle (`KismetMathLibrary.MakeRotator` 0.0 (* (`KismetMathLibrary.NormalizeAxis` (`KismetMathLibrary.Dot_VectorVector` (`KismetMathLibrary.GetUpVector` (`KismetMathLibrary.MakeRotator` _returnvalue_roll_2 (`KismetMathLibrary.ClampAngle` _returnvalue_pitch_2 0.0 90.0) _returnvalue_yaw)) (`KismetMathLibrary.GetUpVector` (`SceneComponent.K2_GetComponentRotation` (`self.handle`))))) 1.0)) false false)
    (if (>= _returnvalue_pitch 89.0)
      (`KismetSystemLibrary.K2_PauseTimer` null "Update Rotation")
      (`/Engine/EditorBlueprintResources/StandardMacros.DoOnce` false :!label _label
        (:`Completed`
          (`self.Activate` (`self.Motion Controller`) (`self.Skeltal Mesh Hand`) :!label _label_2))))
    (else
      (goto _label_2))))

(event `self.C_GrabComponent.FirstHandDropped`
  (params (`Original Hand Location` :type "Transform Structure") (`Motion Controller` :type "MotionControllerComponent Object Reference") (`Skeletal Mesh Hand` :type "SkeletalMeshComponent Object Reference"))
  (if (== (`MotionControllerComponent.MotionSource` `Motion Controller`) "Left")
    (message `/Game/GDXR_VR_Template/Blueprints/Interfaces/BPI_HandSnapping.ReleaseHandFromObject` (`ChildActorComponent.ChildActor` (`self.LeftHandSnap`)) `Motion Controller` `Skeletal Mesh Hand` `Original Hand Location`)
    (`KismetSystemLibrary.K2_PauseTimer` null "Update Rotation")
    (set `self.Motion Controller` null)
    (`self.Deactivate`)
    (bind _returnvalue (`KismetSystemLibrary.K2_SetTimerDelegate` (`|CreateDelegate` :!event `Rest Door Handle`) 0.02 true))
    (else
      (message `/Game/GDXR_VR_Template/Blueprints/Interfaces/BPI_HandSnapping.ReleaseHandFromObject` (`ChildActorComponent.ChildActor` (`self.RightHandSnap`)) `Motion Controller` `Skeletal Mesh Hand` `Original Hand Location`))))

(event `Rest Door Handle`
  (bind (_returnvalue_roll _returnvalue_pitch) (`KismetMathLibrary.BreakRotator` (`SceneComponent.K2_GetComponentRotation` (`self.handle`))))
  (bind _returnvalue (`KismetMathLibrary.FInterpTo` _returnvalue_pitch 0.0 5.0 5.0))
  (`SceneComponent.K2_SetWorldRotation` (`self.handle`) (`KismetMathLibrary.MakeRotator` 0.0 _returnvalue) false false)
  (if (> _returnvalue -0.1)
    (`KismetSystemLibrary.K2_PauseTimerHandle` (stale `self.C_GrabComponent.FirstHandDropped` _returnvalue))
    (goto _label :!via `Reset`)))

(fn `UserConstructionScript`)