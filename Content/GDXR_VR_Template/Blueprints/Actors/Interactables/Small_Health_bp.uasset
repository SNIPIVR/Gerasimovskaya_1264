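; Grabbable VR voltage indicator tool with selectable 110, 35 and 6 variants, despite the Small_Health name.
; Grabbing snaps the hand pose and shows a widget linked to this actor for up to 15 seconds, until dropped.
; Volt toggles the variant meshes.
; Tick pushes the active voltage to the TouchCable in ActorElectro, then mirrors its OnElectro and OnGreen flags as red light with sound and green light.
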(event `self.ReceiveBeginPlay`
  ;[1 1 1] Set Slot type
  (`|ExecutionSequence`
    (:`then_1`
      (bind _asukaz_widget (cast `/Game/StaticObject/VoltIndicator/Ukaz_widget` (`WidgetComponent.GetUserWidgetObject` (`self.Widget`))))
      (set `/Game/StaticObject/VoltIndicator/Ukaz_widget.ActorKey` self _asukaz_widget))))

(event `self.C_GrabComponent.FirstHandGrabbed`
  (params (`Motion Controller` :type "MotionControllerComponent Object Reference") (SkeltalMeshHand :type "SkeletalMeshComponent Object Reference") (`Motion Controller Aim` :type "MotionControllerComponent Object Reference"))
  (if (== (`MotionControllerComponent.MotionSource` `Motion Controller`) "Left")
    (message `/Game/GDXR_VR_Template/Blueprints/Interfaces/BPI_HandSnapping.SnapHandPosition` (`ChildActorComponent.ChildActor` (`self.HandLeft`)) SkeltalMeshHand null)
    (else
      (message `/Game/GDXR_VR_Template/Blueprints/Interfaces/BPI_HandSnapping.SnapHandPosition` (`ChildActorComponent.ChildActor` (`self.HandRight`)) SkeltalMeshHand null)))
  (`SceneComponent.SetVisibility` (`self.Widget`) true false)
  (`KismetSystemLibrary.Delay` 15.0)
  (`SceneComponent.SetVisibility` (`self.Widget`) false false)
  (`KismetSystemLibrary.Delay` 0.2))

(event `self.C_GrabComponent.FirstHandDropped`
  (params (`Original Hand Location` :type "Transform Structure") (`Motion Controller` :type "MotionControllerComponent Object Reference") (`Skeletal Mesh Hand` :type "SkeletalMeshComponent Object Reference"))
  (`SceneComponent.SetVisibility` (`self.Widget`) false false))

(event `self.ReceiveTick`
  (params (DeltaSeconds :type "Float (single-precision)"))
  (bind _greenlight (`self.GreenLight`))
  (bind _greenlight3 (`self.GreenLight3`))
  (bind _greenlight2 (`self.GreenLight2`))
  (bind _astouch_cable (cast `/Game/StaticObject/VoltIndicator/TouchCable` (`self.ActorElectro`)))
  (if (stale `/Game/StaticObject/VoltIndicator/UkazControl.Volt` `110`) :!label _label
    (set `/Game/StaticObject/VoltIndicator/TouchCable.110` true _astouch_cable)
    (set `/Game/StaticObject/VoltIndicator/TouchCable.35` false _astouch_cable)
    (set `/Game/StaticObject/VoltIndicator/TouchCable.6` false _astouch_cable)
    (`|ExecutionSequence`
      (:`then_0`
        (bind _onelectro_ (`/Game/StaticObject/VoltIndicator/TouchCable.OnElectro?` _astouch_cable))
        (if _onelectro_
          (`SceneComponent.SetVisibility` (`self.RedLight`) true false)
          (`ActorComponent.Activate` (`self.SoundUkaz`) false)
          (else
            (`SceneComponent.SetVisibility` (`self.RedLight`) false false)
            (`AudioComponent.Stop` (`self.SoundUkaz`)))))
      (:`then_1`
        (bind _ongreen (`/Game/StaticObject/VoltIndicator/TouchCable.OnGreen` _astouch_cable))
        (if _ongreen
          (`SceneComponent.SetVisibility` _greenlight true false)
          (else
            (`SceneComponent.SetVisibility` _greenlight false false)))))
    (elif (stale `/Game/StaticObject/VoltIndicator/UkazControl.Volt` `35`)
      (set `/Game/StaticObject/VoltIndicator/TouchCable.35` true _astouch_cable)
      (set `/Game/StaticObject/VoltIndicator/TouchCable.110` false _astouch_cable)
      (set `/Game/StaticObject/VoltIndicator/TouchCable.6` false _astouch_cable)
      (`|ExecutionSequence`
        (:`then_0`
          (if _onelectro_
            (`SceneComponent.SetVisibility` (`self.RedLight1`) true false)
            (`ActorComponent.Activate` (`self.SoundUkaz`) false)
            (else
              (`SceneComponent.SetVisibility` (`self.RedLight1`) false false)
              (`AudioComponent.Stop` (`self.SoundUkaz`)))))
        (:`then_1`
          (if _ongreen
            (`SceneComponent.SetVisibility` _greenlight3 true false)
            (else
              (`SceneComponent.SetVisibility` _greenlight3 false false)))))
      (elif (stale `/Game/StaticObject/VoltIndicator/UkazControl.Volt` `6`)
        (set `/Game/StaticObject/VoltIndicator/TouchCable.6` true _astouch_cable)
        (set `/Game/StaticObject/VoltIndicator/TouchCable.35` false _astouch_cable)
        (set `/Game/StaticObject/VoltIndicator/TouchCable.110` false _astouch_cable)
        (`|ExecutionSequence`
          (:`then_0`
            (if _onelectro_
              (`SceneComponent.SetVisibility` (`self.RedLight2`) true false)
              (`ActorComponent.Activate` (`self.SoundUkaz`) false)
              (else
                (`SceneComponent.SetVisibility` (`self.RedLight2`) false false)
                (`AudioComponent.Stop` (`self.SoundUkaz`)))))
          (:`then_1`
            (if _ongreen
              (`SceneComponent.SetVisibility` _greenlight2 true false)
              (else
                (`SceneComponent.SetVisibility` _greenlight2 false false)))))))))

(event `/Game/StaticObject/VoltIndicator/UkazControl.Volt`
  (params (`110` :type Boolean) (`35` :type Boolean) (`6` :type Boolean) (DelDop :type Boolean) (Dop :type Boolean))
  (`SceneComponent.SetVisibility` (`self.Ukaz110`) `110` false)
  (`SceneComponent.SetVisibility` (`self.Ukaz35`) `35` false)
  (`SceneComponent.SetVisibility` (`self.Ukaz6`) `6` false)
  (goto _label))

(fn `UserConstructionScript`)