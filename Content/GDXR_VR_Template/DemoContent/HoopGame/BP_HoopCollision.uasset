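; BP_HoopCollision is the scoring trigger for the hoop game in the VR template demo content.
; Any overlap on its cylinder increments the score, passes it to the hoop counter and spawns confetti Niagara at the cylinder's transform, destroying the previous effect first.
; An Activation event tells the same counter to start its timer message.
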(event `/Game/GDXR_VR_Template/Blueprints/Interfaces/BPI_PlayerInteractions.Activation`
  (params (State :type Boolean))
  (message `/Game/GDXR_VR_Template/DemoContent/HoopGame/BPI_HoopGame.Start Timer` (`self.BP_HoopCounter`)))

(event `self.Cylinder.OnComponentBeginOverlap`
  (params (OverlappedComponent :type "PrimitiveComponent Object Reference") (OtherActor :type "Actor Object Reference") (OtherComp :type "PrimitiveComponent Object Reference") (OtherBodyIndex :type Integer) (bFromSweep :type Boolean) (SweepResult :type "HitResult Structure (by ref)"))
  (bind _spawned_emmitter (`self.Spawned Emmitter`))
  (bind (_returnvalue_location _returnvalue_rotation _returnvalue_scale) (`KismetMathLibrary.BreakTransform` (`SceneComponent.K2_GetComponentToWorld` (`self.Cylinder`))))
  (bind _result (`/Engine/EditorBlueprintResources/StandardMacros.IncrementInt` (`self.CurrentScore`))
    (:`  `
      (`/Game/GDXR_VR_Template/DemoContent/HoopGame/BP_HoopCounterWidget.UpdateScore` (`self.BP_HoopCounter`) _result)
      (`/Engine/EditorBlueprintResources/StandardMacros.IsValid` _spawned_emmitter
        (:`Is Valid`
          (`ActorComponent.K2_DestroyComponent` _spawned_emmitter))
        (:`Is Not Valid`
          _))
      (bind _returnvalue (`NiagaraFunctionLibrary.SpawnSystemAtLocation` "/Game/GDXR_VR_Template/DemoContent/HoopGame/NS_Confetti.NS_Confetti" _returnvalue_location _returnvalue_rotation _returnvalue_scale))
      (set `self.Spawned Emmitter` _returnvalue))))

(fn `UserConstructionScript`)