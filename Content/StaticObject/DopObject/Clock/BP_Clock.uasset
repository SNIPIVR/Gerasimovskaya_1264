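; BP_Clock is a wall-time clock prop that also reacts to a laser.
; From BeginPlay, a one-second delay loop sets hour, minute and second hand yaw from the current system time, with the hour hand advancing by minutes.
; The first Box overlap by a component tagged "Lazer" flashes the PointLight briefly, gated by DoOnce with no reset.
; A separate ScriptPoint function sets the Point flag, with no caller in this file.
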(event `self.ReceiveBeginPlay`
  (bind (_year _month _day _hour _minute _second) (`KismetMathLibrary.BreakDateTime` (`KismetMathLibrary.Now`)))
  (`SceneComponent.K2_SetRelativeRotation` (`self.Clock_Hour`) (`KismetMathLibrary.MakeRotator` 0.0 0.0 (+ (* _hour 30.0) (* _minute 0.5))) false false :!label _label)
  (`SceneComponent.K2_SetRelativeRotation` (`self.Clock_Minutes`) (`KismetMathLibrary.MakeRotator` 0.0 0.0 (* _minute 6.0)) false false)
  (`SceneComponent.K2_SetRelativeRotation` (`self.Clock_Seconds`) (`KismetMathLibrary.MakeRotator` 0.0 0.0 (* _second 6.0)) false false)
  (`KismetSystemLibrary.Delay` 1.0)
  (goto _label))

(event `self.Box.OnComponentBeginOverlap`
  (params (OverlappedComponent :type "PrimitiveComponent Object Reference") (OtherActor :type "Actor Object Reference") (OtherComp :type "PrimitiveComponent Object Reference") (OtherBodyIndex :type Integer) (bFromSweep :type Boolean) (SweepResult :type "HitResult Structure (by ref)"))
  (if (`ActorComponent.ComponentHasTag` OtherComp "Lazer")
    (`/Engine/EditorBlueprintResources/StandardMacros.DoOnce` false
      (:`Completed`
        (`SceneComponent.SetVisibility` (`self.PointLight`) true false)
        (`KismetSystemLibrary.Delay` 0.5)
        (`SceneComponent.SetVisibility` (`self.PointLight`) false false)))))

(fn `ScriptPoint`
  (set `self.+Point` true))

(fn `UserConstructionScript`)