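; Grabbable telephone for scenario 8 that snaps the hand pose on pickup and plays up to three staged calls as timed audio chains.
; ChangeNumber flags select the call and clear when it finishes; dropping the handset stops all audio and halts the chain through StopCalling.
; The handset attaches to the Box socket at start and when leaving the box ungrabbed.
; The third call ends the scenario through BP_End, choosing the outcome from 03_04_TH1's IsWorkSeparator2.
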(event `self.ReceiveBeginPlay`
  (`|ExecutionSequence`
    (:`then_0`
      (`AudioComponent.Stop` (`self.Audio2`))
      (`AudioComponent.Stop` (`self.Audio4`))
      (`AudioComponent.Stop` (`self.Audio3`))
      (`AudioComponent.Stop` (`self.Audio6`))
      (`AudioComponent.Stop` (`self.Audio5`))
      (`AudioComponent.Stop` (`self.Audio13`))
      (`AudioComponent.Stop` (`self.Audio14`))
      (`AudioComponent.Stop` (`self.Audio15`))
      (`AudioComponent.Stop` (`self.Audio12`))
      (`AudioComponent.Stop` (`self.Audio17`))
      (`AudioComponent.Stop` (`self.Audio16`))
      (`AudioComponent.Stop` (`self.Audio8`))
      (`AudioComponent.Stop` (`self.Audio9`))
      (`AudioComponent.Stop` (`self.Audio10`))
      (`AudioComponent.Stop` (`self.Audio11`))
      (`AudioComponent.Stop` (`self.Audio7`))
      (`AudioComponent.Stop` (`self.Audio18`))
      (`AudioComponent.Stop` (`self.Audio19`))
      (`AudioComponent.Stop` (`self.Audio20`))
      (`AudioComponent.Stop` (`self.Audio21`))
      (`AudioComponent.Stop` (`self.Audio22`))
      (`AudioComponent.Stop` (`self.Audio23`))
      (`AudioComponent.Stop` (`self.Audio`))
      (`SceneComponent.K2_AttachToComponent` (`self.old_telephone__3__hanger`) (`self.Box`) "Phone_1" "SnapToTarget" "SnapToTarget" "KeepWorld" true :!label _label))))

(event `self.Box.OnComponentEndOverlap`
  (params (OverlappedComponent :type "PrimitiveComponent Object Reference") (OtherActor :type "Actor Object Reference") (OtherComp :type "PrimitiveComponent Object Reference") (OtherBodyIndex :type Integer))
  (if (not (`self.Grab?`))
    (goto _label)))

(event `self.C_GrabComponent.FirstHandGrabbed`
  (params (`Motion Controller` :type "MotionControllerComponent Object Reference") (SkeltalMeshHand :type "SkeletalMeshComponent Object Reference") (`Motion Controller Aim` :type "MotionControllerComponent Object Reference"))
  (bind _stop_calling (`self.Stop_Calling`))
  (bind _stop_calling_2 (`self.Stop_Calling`))
  (if (== (`MotionControllerComponent.MotionSource` `Motion Controller`) "Left")
    (message `/Game/GDXR_VR_Template/Blueprints/Interfaces/BPI_HandSnapping.SnapHandPosition` (`ChildActorComponent.ChildActor` (`self.HandLeft`)) SkeltalMeshHand null)
    (else
      (message `/Game/GDXR_VR_Template/Blueprints/Interfaces/BPI_HandSnapping.SnapHandPosition` (`ChildActorComponent.ChildActor` (`self.HandRight`)) SkeltalMeshHand null)))
  (`SceneComponent.SetRelativeScale3D` (`self.old_telephone__3__hanger`) (1.5 1.5 1.5))
  (set `self.Stop_Calling` false)
  (`|ExecutionSequence`
    (:`then_0`
      (set `self.Grab?` true)
      (if (`self.ChangeNumber`)
        (`ActorComponent.Activate` (`self.Audio`) false)
        (`KismetSystemLibrary.Delay` 29.0)
        (if (not (`self.Stop_Calling`))
          (`ActorComponent.Activate` (`self.Audio2`) false)
          (`KismetSystemLibrary.Delay` 26.0)
          (if (not (`self.Stop_Calling`))
            (`ActorComponent.Activate` (`self.Audio3`) false)
            (`KismetSystemLibrary.Delay` 10.5)
            (if (not (`self.Stop_Calling`))
              (`ActorComponent.Activate` (`self.Audio4`) false)
              (`KismetSystemLibrary.Delay` 4.5)
              (set `self.ChangeNumber` false)
              (set `self.Grab?` false))))))
    (:`then_1`
      (set `self.Grab?` true)
      (if (`self.ChangeNumber`)
        _
        (elif (`self.ChangeNumber_2`)
          (`ActorComponent.Activate` (`self.Audio5`) false)
          (`KismetSystemLibrary.Delay` 23.0)
          (if (not _stop_calling)
            (`ActorComponent.Activate` (`self.Audio6`) false)
            (`KismetSystemLibrary.Delay` 20.6)
            (if (not _stop_calling)
              (`ActorComponent.Activate` (`self.Audio7`) false)
              (`KismetSystemLibrary.Delay` 12.8)
              (if (not _stop_calling)
                (`ActorComponent.Activate` (`self.Audio8`) false)
                (`KismetSystemLibrary.Delay` 11.4)
                (if (not _stop_calling)
                  (`ActorComponent.Activate` (`self.Audio9`) false)
                  (`KismetSystemLibrary.Delay` 8.0)
                  (if (not _stop_calling)
                    (`ActorComponent.Activate` (`self.Audio10`) false)
                    (`KismetSystemLibrary.Delay` 11.0)
                    (if (not _stop_calling)
                      (`ActorComponent.Activate` (`self.Audio11`) false)
                      (`KismetSystemLibrary.Delay` 10.0)
                      (if (not _stop_calling)
                        (`ActorComponent.Activate` (`self.Audio12`) false)
                        (`KismetSystemLibrary.Delay` 2.0)
                        (set `self.ChangeNumber_2` false)
                        (set `self.Grab?` false)))))))))))
    (:`then_2`
      (set `self.Grab?` true)
      (if (`self.ChangeNumber`)
        _
        (elif (`self.ChangeNumber_2`)
          _
          (elif (`self.ChangeNumber_3`)
            (`ActorComponent.Activate` (`self.Audio13`) false)
            (`KismetSystemLibrary.Delay` 19.0)
            (if (not _stop_calling_2)
              (`ActorComponent.Activate` (`self.Audio14`) false)
              (`KismetSystemLibrary.Delay` 21.5)
              (if (not _stop_calling_2)
                (`ActorComponent.Activate` (`self.Audio15`) false)
                (set `self.ChangeNumber_3` false)
                (`KismetSystemLibrary.Delay` 6.0)
                (set `self.Grab?` false)
                (bind _asbp_end (cast `/Game/BP/Blueprints/UI/EndMenu/BP_End` (`self.BP END`)))
                (bind _as03_04_th1 (cast `/Game/BP/DisconnectKnives/03_04_TH1` (`self.03_04_TH1`)))
                (if (`/Game/BP/DisconnectKnives/03_04_TH1.IsWorkSeparator2?` _as03_04_th1)
                  (`/Game/BP/Blueprints/UI/EndMenu/BP_End.ScenarEnd` _asbp_end "NewEnumerator24")
                  (else
                    (`/Game/BP/Blueprints/UI/EndMenu/BP_End.ScenarEnd` _asbp_end "NewEnumerator14")))))))))))

(event `self.C_GrabComponent.FirstHandDropped`
  (params (`Original Hand Location` :type "Transform Structure") (`Motion Controller` :type "MotionControllerComponent Object Reference") (`Skeletal Mesh Hand` :type "SkeletalMeshComponent Object Reference"))
  (set `self.Grab?` false)
  (set `self.Stop_Calling` true)
  (`AudioComponent.Stop` (`self.Audio2`))
  (`AudioComponent.Stop` (`self.Audio4`))
  (`AudioComponent.Stop` (`self.Audio3`))
  (`AudioComponent.Stop` (`self.Audio6`))
  (`AudioComponent.Stop` (`self.Audio5`))
  (`AudioComponent.Stop` (`self.Audio13`))
  (`AudioComponent.Stop` (`self.Audio14`))
  (`AudioComponent.Stop` (`self.Audio15`))
  (`AudioComponent.Stop` (`self.Audio12`))
  (`AudioComponent.Stop` (`self.Audio17`))
  (`AudioComponent.Stop` (`self.Audio16`))
  (`AudioComponent.Stop` (`self.Audio8`))
  (`AudioComponent.Stop` (`self.Audio9`))
  (`AudioComponent.Stop` (`self.Audio10`))
  (`AudioComponent.Stop` (`self.Audio11`))
  (`AudioComponent.Stop` (`self.Audio7`))
  (`AudioComponent.Stop` (`self.Audio18`))
  (`AudioComponent.Stop` (`self.Audio19`))
  (`AudioComponent.Stop` (`self.Audio20`))
  (`AudioComponent.Stop` (`self.Audio21`))
  (`AudioComponent.Stop` (`self.Audio22`))
  (`AudioComponent.Stop` (`self.Audio23`))
  (`AudioComponent.Stop` (`self.Audio`)))

(event `self.Call2.OnComponentBeginOverlap`
  (params (OverlappedComponent :type "PrimitiveComponent Object Reference") (OtherActor :type "Actor Object Reference") (OtherComp :type "PrimitiveComponent Object Reference") (OtherBodyIndex :type Integer) (bFromSweep :type Boolean) (SweepResult :type "HitResult Structure (by ref)")))

(fn `UserConstructionScript`)