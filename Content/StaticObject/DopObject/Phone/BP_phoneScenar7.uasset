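; VR telephone for training scenario 7 that plays six scripted calls, then checks switchgear state for errors.
; Grabbing snaps the hand pose, and the released handset reattaches to its box when their overlap ends.
; Each grab runs any armed DoOnce call of timed audio clips, which arms the next after a delay.
; The last call tests switcher and equipment flags in turn, reporting the first failure through BP_End.ScenarEnd.
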(event `self.ReceiveBeginPlay`
  (`AudioComponent.Stop` (`self.Audio`))
  (`AudioComponent.Stop` (`self.Audio22`))
  (`AudioComponent.Stop` (`self.Audio4`))
  (`AudioComponent.Stop` (`self.Audio8`))
  (`AudioComponent.Stop` (`self.Audio7`))
  (`AudioComponent.Stop` (`self.Audio31`))
  (`AudioComponent.Stop` (`self.Audio30`))
  (`AudioComponent.Stop` (`self.Audio9`))
  (`AudioComponent.Stop` (`self.Audio6`))
  (`AudioComponent.Stop` (`self.Audio5`))
  (`AudioComponent.Stop` (`self.Audio21`))
  (`AudioComponent.Stop` (`self.Audio37`))
  (`AudioComponent.Stop` (`self.Audio36`))
  (`AudioComponent.Stop` (`self.Audio35`))
  (`AudioComponent.Stop` (`self.Audio34`))
  (`AudioComponent.Stop` (`self.Audio33`))
  (`AudioComponent.Stop` (`self.Audio26`))
  (`AudioComponent.Stop` (`self.Audio25`))
  (`AudioComponent.Stop` (`self.Audio24`))
  (`AudioComponent.Stop` (`self.Audio23`))
  (`AudioComponent.Stop` (`self.Audio2`))
  (`AudioComponent.Stop` (`self.Audio27`))
  (`AudioComponent.Stop` (`self.Audio32`))
  (`AudioComponent.Stop` (`self.Audio29`))
  (`AudioComponent.Stop` (`self.Audio28`))
  (`AudioComponent.Stop` (`self.Audio15`))
  (`AudioComponent.Stop` (`self.Audio14`))
  (`AudioComponent.Stop` (`self.Audio13`))
  (`AudioComponent.Stop` (`self.Audio12`))
  (`AudioComponent.Stop` (`self.Audio11`))
  (`AudioComponent.Stop` (`self.Audio20`))
  (`AudioComponent.Stop` (`self.Audio19`))
  (`AudioComponent.Stop` (`self.Audio16`))
  (`AudioComponent.Stop` (`self.Audio18`))
  (`AudioComponent.Stop` (`self.Audio17`))
  (`AudioComponent.Stop` (`self.Audio10`))
  (`AudioComponent.Stop` (`self.Audio3`))
  (`SceneComponent.K2_AttachToComponent` (`self.old_telephone__3__hanger`) (`self.Box`) "Phone_1" "SnapToTarget" "SnapToTarget" "KeepWorld" true :!label _label))

(event `self.Box.OnComponentEndOverlap`
  (params (OverlappedComponent :type "PrimitiveComponent Object Reference") (OtherActor :type "Actor Object Reference") (OtherComp :type "PrimitiveComponent Object Reference") (OtherBodyIndex :type Integer))
  (if (not (`self.Grab?`))
    (goto _label)))

(event `self.C_GrabComponent.FirstHandGrabbed`
  (params (`Motion Controller` :type "MotionControllerComponent Object Reference") (SkeltalMeshHand :type "SkeletalMeshComponent Object Reference") (`Motion Controller Aim` :type "MotionControllerComponent Object Reference"))
  (if (== (`MotionControllerComponent.MotionSource` `Motion Controller`) "Left")
    (message `/Game/GDXR_VR_Template/Blueprints/Interfaces/BPI_HandSnapping.SnapHandPosition` (`ChildActorComponent.ChildActor` (`self.HandLeft`)) SkeltalMeshHand null)
    (else
      (message `/Game/GDXR_VR_Template/Blueprints/Interfaces/BPI_HandSnapping.SnapHandPosition` (`ChildActorComponent.ChildActor` (`self.HandRight`)) SkeltalMeshHand null)))
  (`SceneComponent.SetRelativeScale3D` (`self.old_telephone__3__hanger`) (1.5 1.5 1.5))
  (`|ExecutionSequence`
    (:`then_0`
      (set `self.Grab?` true)
      (if (`self.ChangeNumber`)
        (`/Engine/EditorBlueprintResources/StandardMacros.DoOnce` false
          (:`Completed`
            (`ActorComponent.Activate` (`self.Audio`) false)
            (`KismetSystemLibrary.Delay` 41.0)
            (`ActorComponent.Activate` (`self.Audio2`) false)
            (`KismetSystemLibrary.Delay` 35.5)
            (`ActorComponent.Activate` (`self.Audio3`) false)
            (`KismetSystemLibrary.Delay` 40.0)
            (`ActorComponent.Activate` (`self.Audio4`) false)
            (`KismetSystemLibrary.Delay` 2.0)
            (`ActorComponent.Activate` (`self.Audio5`) false)
            (set `self.ChangeNumber` false)
            (set `self.Grab?` false)
            (`KismetSystemLibrary.Delay` 30.0)
            (set `self.ChangeNumber_2` true)))))
    (:`then_1`
      (set `self.Grab?` true)
      (if (`self.ChangeNumber_2`)
        (`/Engine/EditorBlueprintResources/StandardMacros.DoOnce` false
          (:`Completed`
            (`ActorComponent.Activate` (`self.Audio6`) false)
            (`KismetSystemLibrary.Delay` 47.5)
            (`ActorComponent.Activate` (`self.Audio7`) false)
            (`KismetSystemLibrary.Delay` 40.5)
            (`ActorComponent.Activate` (`self.Audio8`) false)
            (`KismetSystemLibrary.Delay` 7.0)
            (`ActorComponent.Activate` (`self.Audio9`) false)
            (`KismetSystemLibrary.Delay` 66.5)
            (`ActorComponent.Activate` (`self.Audio10`) false)
            (`KismetSystemLibrary.Delay` 77.5)
            (`ActorComponent.Activate` (`self.Audio11`) false)
            (`KismetSystemLibrary.Delay` 2.0)
            (`ActorComponent.Activate` (`self.Audio12`) false)
            (`KismetSystemLibrary.Delay` 2.3)
            (set `self.ChangeNumber_2` false)
            (set `self.Grab?` false)
            (`KismetSystemLibrary.Delay` 30.0)
            (set `self.ChangeNumber_3` true)))))
    (:`then_2`
      (set `self.Grab?` true)
      (if (`self.ChangeNumber_3`)
        (`/Engine/EditorBlueprintResources/StandardMacros.DoOnce` false
          (:`Completed`
            (`ActorComponent.Activate` (`self.Audio13`) false)
            (`KismetSystemLibrary.Delay` 78.0)
            (`ActorComponent.Activate` (`self.Audio14`) false)
            (`KismetSystemLibrary.Delay` 66.0)
            (`ActorComponent.Activate` (`self.Audio15`) false)
            (`KismetSystemLibrary.Delay` 7.0)
            (`ActorComponent.Activate` (`self.Audio16`) false)
            (`KismetSystemLibrary.Delay` 30.0)
            (`ActorComponent.Activate` (`self.Audio17`) false)
            (`KismetSystemLibrary.Delay` 36.5)
            (`ActorComponent.Activate` (`self.Audio18`) false)
            (`KismetSystemLibrary.Delay` 2.0)
            (`ActorComponent.Activate` (`self.Audio19`) false)
            (set `self.ChangeNumber_3` false)
            (set `self.Grab?` false)
            (`KismetSystemLibrary.Delay` 30.0)
            (set `self.ChangeNumber_4` true)))))
    (:`then_3`
      (set `self.Grab?` true)
      (if (`self.ChangeNumber_4`)
        (`/Engine/EditorBlueprintResources/StandardMacros.DoOnce` false
          (:`Completed`
            (`ActorComponent.Activate` (`self.Audio20`) false)
            (`KismetSystemLibrary.Delay` 31.5)
            (`ActorComponent.Activate` (`self.Audio21`) false)
            (`KismetSystemLibrary.Delay` 25.5)
            (`ActorComponent.Activate` (`self.Audio22`) false)
            (`KismetSystemLibrary.Delay` 7.0)
            (`ActorComponent.Activate` (`self.Audio23`) false)
            (`KismetSystemLibrary.Delay` 52.7)
            (`ActorComponent.Activate` (`self.Audio24`) false)
            (`KismetSystemLibrary.Delay` 57.5)
            (`ActorComponent.Activate` (`self.Audio25`) false)
            (`KismetSystemLibrary.Delay` 2.0)
            (`ActorComponent.Activate` (`self.Audio26`) false)
            (set `self.ChangeNumber_4` false)
            (set `self.Grab?` false)
            (`KismetSystemLibrary.Delay` 30.0)
            (set `self.ChangeNumber_5` true)))))
    (:`then_4`
      (set `self.Grab?` true)
      (if (`self.ChangeNumber_5`)
        (`/Engine/EditorBlueprintResources/StandardMacros.DoOnce` false
          (:`Completed`
            (`ActorComponent.Activate` (`self.Audio27`) false)
            (`KismetSystemLibrary.Delay` 28.5)
            (`ActorComponent.Activate` (`self.Audio28`) false)
            (`KismetSystemLibrary.Delay` 22.5)
            (`ActorComponent.Activate` (`self.Audio29`) false)
            (`KismetSystemLibrary.Delay` 16.5)
            (`ActorComponent.Activate` (`self.Audio30`) false)
            (`KismetSystemLibrary.Delay` 8.7)
            (`ActorComponent.Activate` (`self.Audio31`) false)
            (`KismetSystemLibrary.Delay` 14.0)
            (`ActorComponent.Activate` (`self.Audio32`) false)
            (`KismetSystemLibrary.Delay` 2.0)
            (`ActorComponent.Activate` (`self.Audio33`) false)
            (set `self.ChangeNumber_5` false)
            (set `self.Grab?` false)
            (`KismetSystemLibrary.Delay` 30.0)
            (set `self.ChangeNumber_6` true)))))
    (:`then_5`
      (set `self.Grab?` true)
      (if (`self.ChangeNumber_6`)
        (`/Engine/EditorBlueprintResources/StandardMacros.DoOnce` false
          (:`Completed`
            (`ActorComponent.Activate` (`self.Audio34`) false)
            (`KismetSystemLibrary.Delay` 17.5)
            (`ActorComponent.Activate` (`self.Audio35`) false)
            (`KismetSystemLibrary.Delay` 13.5)
            (`ActorComponent.Activate` (`self.Audio36`) false)
            (`KismetSystemLibrary.Delay` 7.0)
            (`ActorComponent.Activate` (`self.Audio37`) false)
            (set `self.ChangeNumber_6` false)
            (set `self.Grab?` false)
            (bind _asswitcher_3y_1_scenari_7 (cast `/Game/BP/Switcher/Scenar7/Switcher3Y_1_Scenari7` (`self.Switcher3Y_1_Scenari7`)))
            (if (`/Game/BP/Switcher/Scenar7/Switcher3Y_1_Scenari7.KRUN6PG` _asswitcher_3y_1_scenari_7)
              (bind _asswitcher_4y_5_scenari_7 (cast `/Game/BP/Switcher/Scenar7/Switcher4Y_5_Scenari7` (`self.Switcher4Y_5_Scenari7`)))
              (if (`/Game/BP/Switcher/Scenar7/Switcher4Y_5_Scenari7.RTN-2` _asswitcher_4y_5_scenari_7)
                (bind _asswitcher_4y_3_scenari_7 (cast `/Game/BP/Switcher/Scenar7/Switcher4Y_3_Scenari7` (`self.Switcher4Y_3_Scenari7`)))
                (if (`/Game/BP/Switcher/Scenar7/Switcher4Y_3_Scenari7.V110Alex` _asswitcher_4y_3_scenari_7)
                  (bind _asswitcher_4y_4_scenari_7 (cast `/Game/BP/Switcher/Scenar7/Switcher4Y_4_Scenari7` (`self.Switcher4Y_4_Scenari7`)))
                  (if (`/Game/BP/Switcher/Scenar7/Switcher4Y_4_Scenari7.LRAlexOFF` _asswitcher_4y_4_scenari_7)
                    (bind _as02_13_ice_break_alex (cast `/Game/BP/DisconnectKnives/02_13_IceBreakAlex` (`self.02_13_IceBreakAlex`)))
                    (if (`/Game/BP/DisconnectKnives/02_13_IceBreakAlex.RPGAlexActive` _as02_13_ice_break_alex)
                      (bind _askrun_arm1 (cast `/Game/OP_Dop/KRUN/KRUN_ARM1` (`self.KRUN_ARM1`)))
                      (if (`/Game/OP_Dop/KRUN/KRUN_ARM1.SHRYPGActive` _askrun_arm1)
                        (bind `_as22_blue_print_крун_якно` (cast `/Game/OP_Dop/KRUN/BP/22_BluePrint_КРУН_ЯКНО` (`self.22_BluePrint_КРУН_ЯКНО`)))
                        (if (not (`/Game/OP_Dop/KRUN/BP/22_BluePrint_КРУН_ЯКНО.V6YPGActive` `_as22_blue_print_крун_якно`))
                          (bind _asbp_end (cast `/Game/BP/Blueprints/UI/EndMenu/BP_End` (`self.BP_End`)))
                          (`/Game/BP/Blueprints/UI/EndMenu/BP_End.ScenarEnd` _asbp_end "NewEnumerator22"))
                        (else
                          (bind _asbp_end_2 (cast `/Game/BP/Blueprints/UI/EndMenu/BP_End` (`self.BP_End`)))
                          (`/Game/BP/Blueprints/UI/EndMenu/BP_End.ScenarEnd` _asbp_end_2 "NewEnumerator21")))
                      (else
                        (bind _asbp_end_3 (cast `/Game/BP/Blueprints/UI/EndMenu/BP_End` (`self.BP_End`)))
                        (`/Game/BP/Blueprints/UI/EndMenu/BP_End.ScenarEnd` _asbp_end_3 "NewEnumerator20")))
                    (else
                      (bind _asbp_end_4 (cast `/Game/BP/Blueprints/UI/EndMenu/BP_End` (`self.BP_End`)))
                      (`/Game/BP/Blueprints/UI/EndMenu/BP_End.ScenarEnd` _asbp_end_4 "NewEnumerator23")))
                  (else
                    (bind _asbp_end_5 (cast `/Game/BP/Blueprints/UI/EndMenu/BP_End` (`self.BP_End`)))
                    (`/Game/BP/Blueprints/UI/EndMenu/BP_End.ScenarEnd` _asbp_end_5 "NewEnumerator19")))
                (else
                  (bind _asbp_end_6 (cast `/Game/BP/Blueprints/UI/EndMenu/BP_End` (`self.BP_End`)))
                  (`/Game/BP/Blueprints/UI/EndMenu/BP_End.ScenarEnd` _asbp_end_6 "NewEnumerator18")))
              (else
                (bind _asbp_end_7 (cast `/Game/BP/Blueprints/UI/EndMenu/BP_End` (`self.BP_End`)))
                (`/Game/BP/Blueprints/UI/EndMenu/BP_End.ScenarEnd` _asbp_end_7 "NewEnumerator17")))))))))

(event `self.C_GrabComponent.FirstHandDropped`
  (params (`Original Hand Location` :type "Transform Structure") (`Motion Controller` :type "MotionControllerComponent Object Reference") (`Skeletal Mesh Hand` :type "SkeletalMeshComponent Object Reference"))
  (set `self.Grab?` false))

(event `self.Call1.OnComponentBeginOverlap`
  (params (OverlappedComponent :type "PrimitiveComponent Object Reference") (OtherActor :type "Actor Object Reference") (OtherComp :type "PrimitiveComponent Object Reference") (OtherBodyIndex :type Integer) (bFromSweep :type Boolean) (SweepResult :type "HitResult Structure (by ref)")))

(event `self.Call2.OnComponentBeginOverlap`
  (params (OverlappedComponent :type "PrimitiveComponent Object Reference") (OtherActor :type "Actor Object Reference") (OtherComp :type "PrimitiveComponent Object Reference") (OtherBodyIndex :type Integer) (bFromSweep :type Boolean) (SweepResult :type "HitResult Structure (by ref)")))

(fn `UserConstructionScript`)