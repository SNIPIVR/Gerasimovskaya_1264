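; Grabbable telephone for a scripted scenario that plays chained voice or sound sequences when the handset is picked up.
; On begin play it stops all audio and snaps the handset to its socket, re-snapping when the box overlap ends while not grabbed.
; Grabbing runs any of four one-shot, delay-timed audio chains enabled by ChangeNumber flags, each clearing its flag afterwards.
; The Call overlap events are empty and the flag-setting logic is disconnected.
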(event `self.ReceiveBeginPlay`
  (`|ExecutionSequence`
    (:`then_0`
      (`AudioComponent.Stop` (`self.Audio2`))
      (`AudioComponent.Stop` (`self.Audio4`))
      (`AudioComponent.Stop` (`self.Audio3`))
      (`AudioComponent.Stop` (`self.Audio6`))
      (`AudioComponent.Stop` (`self.Audio5`))
      (`AudioComponent.Stop` (`self.Audio13`))
      (`AudioComponent.Stop` (`self.Audio14`))
      (`AudioComponent.Stop` (`self.Audio15`))
      (`AudioComponent.Stop` (`self.Audio12`))
      (`AudioComponent.Stop` (`self.Audio17`))
      (`AudioComponent.Stop` (`self.Audio16`))
      (`AudioComponent.Stop` (`self.Audio8`))
      (`AudioComponent.Stop` (`self.Audio9`))
      (`AudioComponent.Stop` (`self.Audio10`))
      (`AudioComponent.Stop` (`self.Audio11`))
      (`AudioComponent.Stop` (`self.Audio7`))
      (`AudioComponent.Stop` (`self.Audio18`))
      (`AudioComponent.Stop` (`self.Audio19`))
      (`AudioComponent.Stop` (`self.Audio20`))
      (`AudioComponent.Stop` (`self.Audio21`))
      (`AudioComponent.Stop` (`self.Audio22`))
      (`AudioComponent.Stop` (`self.Audio23`))
      (`AudioComponent.Stop` (`self.Audio`))
      (`SceneComponent.K2_AttachToComponent` (`self.old_telephone__3__hanger`) (`self.Box`) "Phone_1" "SnapToTarget" "SnapToTarget" "KeepWorld" true :!label _label))))

(event `self.Box.OnComponentEndOverlap`
  (params (OverlappedComponent :type "PrimitiveComponent Object Reference") (OtherActor :type "Actor Object Reference") (OtherComp :type "PrimitiveComponent Object Reference") (OtherBodyIndex :type Integer))
  (if (not (`self.Grab?`))
    (goto _label)))

(event `self.GrabComponent.OnGrabbed`
  (`|ExecutionSequence`
    (:`then_0`
      (set `self.Grab?` true)
      (if (`self.ChangeNumber`)
        (`/Engine/EditorBlueprintResources/StandardMacros.DoOnce` false
          (:`Completed`
            (`ActorComponent.Activate` (`self.Audio`) false)
            (`KismetSystemLibrary.Delay` 22.5)
            (`ActorComponent.Activate` (`self.Audio2`) false)
            (`KismetSystemLibrary.Delay` 23.5)
            (`ActorComponent.Activate` (`self.Audio3`) false)
            (`KismetSystemLibrary.Delay` 1.5)
            (`ActorComponent.Activate` (`self.Audio4`) false)
            (`KismetSystemLibrary.Delay` 41.5)
            (`ActorComponent.Activate` (`self.Audio5`) false)
            (`KismetSystemLibrary.Delay` 44.5)
            (`ActorComponent.Activate` (`self.Audio6`) false)
            (set `self.ChangeNumber` false)
            (set `self.Grab?` false)))))
    (:`then_1`
      (set `self.Grab?` true)
      (if (`self.ChangeNumber_2`)
        (`/Engine/EditorBlueprintResources/StandardMacros.DoOnce` false
          (:`Completed`
            (`ActorComponent.Activate` (`self.Audio7`) false)
            (`KismetSystemLibrary.Delay` 46.5)
            (`ActorComponent.Activate` (`self.Audio8`) false)
            (`KismetSystemLibrary.Delay` 38.5)
            (`ActorComponent.Activate` (`self.Audio9`) false)
            (`KismetSystemLibrary.Delay` 12.5)
            (`ActorComponent.Activate` (`self.Audio10`) false)
            (`KismetSystemLibrary.Delay` 7.0)
            (`ActorComponent.Activate` (`self.Audio11`) false)
            (set `self.ChangeNumber_2` false)
            (set `self.Grab?` false)))))
    (:`then_2`
      (set `self.Grab?` true)
      (if (`self.ChangeNumber_3`)
        (`/Engine/EditorBlueprintResources/StandardMacros.DoOnce` false
          (:`Completed`
            (`ActorComponent.Activate` (`self.Audio12`) false)
            (`KismetSystemLibrary.Delay` 24.5)
            (`ActorComponent.Activate` (`self.Audio13`) false)
            (`KismetSystemLibrary.Delay` 21.5)
            (`ActorComponent.Activate` (`self.Audio14`) false)
            (`KismetSystemLibrary.Delay` 14.5)
            (`ActorComponent.Activate` (`self.Audio15`) false)
            (`KismetSystemLibrary.Delay` 12.5)
            (`ActorComponent.Activate` (`self.Audio16`) false)
            (`KismetSystemLibrary.Delay` 9.5)
            (`ActorComponent.Activate` (`self.Audio17`) false)
            (`KismetSystemLibrary.Delay` 13.5)
            (`ActorComponent.Activate` (`self.Audio18`) false)
            (`KismetSystemLibrary.Delay` 11.5)
            (`ActorComponent.Activate` (`self.Audio19`) false)
            (`KismetSystemLibrary.Delay` 1.5)
            (`ActorComponent.Activate` (`self.Audio20`) false)
            (set `self.ChangeNumber_3` false)
            (set `self.Grab?` false)))))
    (:`then_3`
      (set `self.Grab?` true)
      (if (`self.ChangeNumber_4`)
        (`/Engine/EditorBlueprintResources/StandardMacros.DoOnce` false
          (:`Completed`
            (`ActorComponent.Activate` (`self.Audio21`) false)
            (`KismetSystemLibrary.Delay` 19.5)
            (`ActorComponent.Activate` (`self.Audio22`) false)
            (`KismetSystemLibrary.Delay` 12.5)
            (`ActorComponent.Activate` (`self.Audio23`) false)
            (set `self.ChangeNumber_4` false)
            (set `self.Grab?` false)))))))

(event `self.GrabComponent.OnDropped`
  (set `self.Grab?` false))

(event `self.Call1.OnComponentBeginOverlap`
  (params (OverlappedComponent :type "PrimitiveComponent Object Reference") (OtherActor :type "Actor Object Reference") (OtherComp :type "PrimitiveComponent Object Reference") (OtherBodyIndex :type Integer) (bFromSweep :type Boolean) (SweepResult :type "HitResult Structure (by ref)")))

(event `self.Call2.OnComponentBeginOverlap`
  (params (OverlappedComponent :type "PrimitiveComponent Object Reference") (OtherActor :type "Actor Object Reference") (OtherComp :type "PrimitiveComponent Object Reference") (OtherBodyIndex :type Integer) (bFromSweep :type Boolean) (SweepResult :type "HitResult Structure (by ref)")))

(fn `UserConstructionScript`)