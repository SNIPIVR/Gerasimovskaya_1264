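; Scenario phone whose handset the player grabs to hear three staged calls, the last ending the scenario.
; Call1 overlap arms the first; its completion arms the second, while the third's flag is set outside this graph.
; Each call plays once as delayed audio clips; the third picks a BP_End ending from knife-related state.
; The handset snaps back to its socket when it leaves the box ungrabbed.
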(event `self.ReceiveBeginPlay`
  (`AudioComponent.Stop` (`self.Audio`))
  (`AudioComponent.Stop` (`self.Audio2`))
  (`AudioComponent.Stop` (`self.Audio4`))
  (`AudioComponent.Stop` (`self.Audio3`))
  (`AudioComponent.Stop` (`self.Audio6`))
  (`AudioComponent.Stop` (`self.Audio5`))
  (`AudioComponent.Stop` (`self.Audio10`))
  (`AudioComponent.Stop` (`self.Audio9`))
  (`AudioComponent.Stop` (`self.Audio8`))
  (`AudioComponent.Stop` (`self.Audio7`))
  (`SceneComponent.K2_AttachToComponent` (`self.old_telephone__3__hanger`) (`self.Box`) "Phone_1" "SnapToTarget" "SnapToTarget" "KeepWorld" true :!label _label))

(event `self.Box.OnComponentEndOverlap`
  (params (OverlappedComponent :type "PrimitiveComponent Object Reference") (OtherActor :type "Actor Object Reference") (OtherComp :type "PrimitiveComponent Object Reference") (OtherBodyIndex :type Integer))
  (if (not (`self.Grab?`))
    (goto _label)))

(event `self.GrabComponent.OnGrabbed`
  (`|ExecutionSequence`
    (:`then_0`
      (set `self.Grab?` true)
      (if (`self.ChangeNumber`)
        (`/Engine/EditorBlueprintResources/StandardMacros.DoOnce` false
          (:`Completed`
            (`ActorComponent.Activate` (`self.Audio`) false)
            (`KismetSystemLibrary.Delay` 17.0)
            (`ActorComponent.Activate` (`self.Audio2`) false)
            (`KismetSystemLibrary.Delay` 23.5)
            (`ActorComponent.Activate` (`self.Audio3`) false)
            (`KismetSystemLibrary.Delay` 12.5)
            (`ActorComponent.Activate` (`self.Audio4`) false)
            (`KismetSystemLibrary.Delay` 2.0)
            (set `self.ChangeNumber` false)
            (set `self.Grab?` false)
            (`KismetSystemLibrary.Delay` 5.0)
            (set `self.ChangeNumber_2` true)))))
    (:`then_1`
      (set `self.Grab?` true)
      (if (`self.ChangeNumber_2`)
        (`/Engine/EditorBlueprintResources/StandardMacros.DoOnce` false
          (:`Completed`
            (`ActorComponent.Activate` (`self.Audio5`) false)
            (`KismetSystemLibrary.Delay` 10.5)
            (`ActorComponent.Activate` (`self.Audio6`) false)
            (`KismetSystemLibrary.Delay` 11.5)
            (`ActorComponent.Activate` (`self.Audio7`) false)
            (`KismetSystemLibrary.Delay` 7.5)
            (`ActorComponent.Activate` (`self.Audio8`) false)
            (set `self.ChangeNumber_2` false)
            (set `self.Grab?` false)))))
    (:`then_2`
      (set `self.Grab?` true)
      (if (`self.ChangeNumber_3`)
        (`/Engine/EditorBlueprintResources/StandardMacros.DoOnce` false
          (:`Completed`
            (`ActorComponent.Activate` (`self.Audio9`) false)
            (`KismetSystemLibrary.Delay` 16.0)
            (`ActorComponent.Activate` (`self.Audio10`) false)
            (`KismetSystemLibrary.Delay` 10.5)
            (set `self.ChangeNumber_3` false)
            (set `self.Grab?` false)
            (bind _asbp_end (cast `/Game/BP/Blueprints/UI/EndMenu/BP_End` (`self.BP END`)))
            (bind _as3_1_a3 (cast `/Game/BP/DisconnectKnives/3_1_A3` (`self.3 1 A3`)))
            (if (`/Game/BP/DisconnectKnives/3_1_A3.WorkKnives?` _as3_1_a3)
              (bind _asdisconnect_knives (cast `/Game/BP/DisconnectKnives/DisconnectKnives` (`self.DisconectKnives`)))
              (if (not (`/Game/BP/DisconnectKnives/DisconnectKnives.IsWork?` _asdisconnect_knives))
                (`/Game/BP/Blueprints/UI/EndMenu/BP_End.ScenarEnd` _asbp_end "NewEnumerator4"))
              (else
                (`/Game/BP/Blueprints/UI/EndMenu/BP_End.ScenarEnd` _asbp_end "NewEnumerator3")))))))))

(event `self.GrabComponent.OnDropped`
  (set `self.Grab?` false))

(event `self.Call1.OnComponentBeginOverlap`
  (params (OverlappedComponent :type "PrimitiveComponent Object Reference") (OtherActor :type "Actor Object Reference") (OtherComp :type "PrimitiveComponent Object Reference") (OtherBodyIndex :type Integer) (bFromSweep :type Boolean) (SweepResult :type "HitResult Structure (by ref)"))
  (set `self.ChangeNumber` true)
  (set `PrimitiveComponent.bGenerateOverlapEvents` false (`self.Call1`)))

(event `self.Call2.OnComponentBeginOverlap`
  (params (OverlappedComponent :type "PrimitiveComponent Object Reference") (OtherActor :type "Actor Object Reference") (OtherComp :type "PrimitiveComponent Object Reference") (OtherBodyIndex :type Integer) (bFromSweep :type Boolean) (SweepResult :type "HitResult Structure (by ref)")))

(fn `UserConstructionScript`)