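; BP_Recorder is an in-world VR voice recorder, toggled when the VRPawn overlaps its sphere.
; Switching on activates AudioCapture and records a submix for a fixed duration, guarded by DoOnce against re-entry.
; The result exports as a timestamp-named SoundWave to a project subdirectory, then plays back immediately as 2D audio.
; Switching off only stops that playback audio, leaving any recording in progress running.
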(event `self.Sphere.OnComponentBeginOverlap`
  (params (OverlappedComponent :type "PrimitiveComponent Object Reference") (OtherActor :type "Actor Object Reference") (OtherComp :type "PrimitiveComponent Object Reference") (OtherBodyIndex :type Integer) (bFromSweep :type Boolean) (SweepResult :type "HitResult Structure (by ref)"))
  (bind _returnvalue (`KismetMathLibrary.Now`))
  (cast `/Game/VRTemplate/Blueprints/VRPawn` OtherActor)
  (if (`self.On?`)
    (set `self.On?` false)
    (`AudioComponent.Stop` (`self.Audio`))
    (else
      (set `self.On?` true)
      (`/Engine/EditorBlueprintResources/StandardMacros.DoOnce` false :!label _label
        (:`Completed`
          (`ActorComponent.Activate` (`self.AudioCapture`) false)
          (`AudioMixerBlueprintLibrary.StartRecordingOutput` 10.0 (`self.Submix to Record`))
          (`KismetSystemLibrary.Delay` 10.0)
          (bind _returnvalue_2 (`AudioMixerBlueprintLibrary.StopRecordingOutput` "SoundWave" (`KismetTextLibrary.Conv_TextToString` (`|FormatText` "{Year}{Hour}{Minute}{Second}" (`KismetMathLibrary.GetYear` _returnvalue) (`KismetMathLibrary.GetMinute` _returnvalue) (`KismetMathLibrary.GetSecond` _returnvalue) (`KismetMathLibrary.GetHour` _returnvalue))) (`KismetTextLibrary.Conv_TextToString` (`|FormatText` "{MeinDir}{SubDir}" (`KismetTextLibrary.Conv_StringToText` (`KismetSystemLibrary.GetProjectDirectory`)) (`self.SubDir`))) (`self.Submix to Record`) null))
          (bind _returnvalue_3 (`GameplayStatics.CreateSound2D` _returnvalue_2 1.0 1.0 0.0 null))
          (bind _output_get (set `self.Audio` _returnvalue_3))
          (`ActorComponent.Deactivate` (`self.AudioCapture`))
          (`/Engine/EditorBlueprintResources/StandardMacros.DoOnce` false :!label _label_2
            (:`Completed`
              (`AudioComponent.Play` _output_get 0.0)
              (`|ExecutionSequence`
                (:`then_0`
                  (goto _label_2 :!via `Reset`))
                (:`then_1`
                  (goto _label :!via `Reset`))))))))))

(fn `UserConstructionScript`)