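; VR grabbable telephone that plays scripted call dialogue when picked up, snapping a hand pose for the grabbing controller.
; ChangeNumber flags choose among three one-shot chains of delay-timed audio; Call1 overlap arms the first, whose completion sets ActivateTransformator.
; The handset attaches to its Box socket on BeginPlay and when an overlap ends while not grabbed.
; Dropping stops all audio but does not cancel pending delays.
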(event `self.ReceiveBeginPlay`
  (`AudioComponent.Stop` (`self.Audio`))
  (`AudioComponent.Stop` (`self.Audio2`))
  (`AudioComponent.Stop` (`self.Audio4`))
  (`AudioComponent.Stop` (`self.Audio3`))
  (`AudioComponent.Stop` (`self.Audio6`))
  (`AudioComponent.Stop` (`self.Audio5`))
  (`AudioComponent.Stop` (`self.Audio13`))
  (`AudioComponent.Stop` (`self.Audio14`))
  (`AudioComponent.Stop` (`self.Audio15`))
  (`AudioComponent.Stop` (`self.Audio12`))
  (`AudioComponent.Stop` (`self.Audio17`))
  (`AudioComponent.Stop` (`self.Audio16`))
  (`AudioComponent.Stop` (`self.Audio8`))
  (`AudioComponent.Stop` (`self.Audio9`))
  (`AudioComponent.Stop` (`self.Audio10`))
  (`AudioComponent.Stop` (`self.Audio11`))
  (`AudioComponent.Stop` (`self.Audio7`))
  (`SceneComponent.K2_AttachToComponent` (`self.old_telephone__3__hanger`) (`self.Box`) "Phone_1" "SnapToTarget" "SnapToTarget" "KeepWorld" true :!label _label))

(event `self.Box.OnComponentEndOverlap`
  (params (OverlappedComponent :type "PrimitiveComponent Object Reference") (OtherActor :type "Actor Object Reference") (OtherComp :type "PrimitiveComponent Object Reference") (OtherBodyIndex :type Integer))
  (if (not (`self.Grab?`))
    (goto _label)))

(event `self.C_GrabComponent.FirstHandGrabbed`
  (params (`Motion Controller` :type "MotionControllerComponent Object Reference") (SkeltalMeshHand :type "SkeletalMeshComponent Object Reference") (`Motion Controller Aim` :type "MotionControllerComponent Object Reference"))
  (if (== (`MotionControllerComponent.MotionSource` `Motion Controller`) "Left")
    (message `/Game/GDXR_VR_Template/Blueprints/Interfaces/BPI_HandSnapping.SnapHandPosition` (`ChildActorComponent.ChildActor` (`self.HandLeft`)) SkeltalMeshHand null)
    (else
      (message `/Game/GDXR_VR_Template/Blueprints/Interfaces/BPI_HandSnapping.SnapHandPosition` (`ChildActorComponent.ChildActor` (`self.HandRight`)) SkeltalMeshHand null)))
  (`|ExecutionSequence`
    (:`then_0`
      (set `self.Grab?` true)
      (if (`self.ChangeNumber`)
        (`/Engine/EditorBlueprintResources/StandardMacros.DoOnce` false
          (:`Completed`
            (`ActorComponent.Activate` (`self.Audio`) false)
            (`KismetSystemLibrary.Delay` 27.2)
            (`ActorComponent.Activate` (`self.Audio2`) false)
            (`KismetSystemLibrary.Delay` 24.2)
            (`ActorComponent.Activate` (`self.Audio3`) false)
            (`KismetSystemLibrary.Delay` 10.2)
            (`ActorComponent.Activate` (`self.Audio4`) false)
            (set `self.ChangeNumber` false)
            (set `self.Grab?` false)
            (set `self.ActivateTransformator` true)))))
    (:`then_1`
      (set `self.Grab?` true)
      (if (`self.ChangeNumber_2`)
        (`/Engine/EditorBlueprintResources/StandardMacros.DoOnce` false
          (:`Completed`
            (`ActorComponent.Activate` (`self.Audio5`) false)
            (`KismetSystemLibrary.Delay` 30.0)
            (`ActorComponent.Activate` (`self.Audio6`) false)
            (`KismetSystemLibrary.Delay` 24.5)
            (`ActorComponent.Activate` (`self.Audio7`) false)
            (`KismetSystemLibrary.Delay` 4.5)
            (`ActorComponent.Activate` (`self.Audio8`) false)
            (`KismetSystemLibrary.Delay` 19.5)
            (`ActorComponent.Activate` (`self.Audio9`) false)
            (`KismetSystemLibrary.Delay` 16.5)
            (`ActorComponent.Activate` (`self.Audio10`) false)
            (`KismetSystemLibrary.Delay` 15.5)
            (`ActorComponent.Activate` (`self.Audio11`) false)
            (`KismetSystemLibrary.Delay` 17.5)
            (`ActorComponent.Activate` (`self.Audio12`) false)
            (`KismetSystemLibrary.Delay` 19.5)
            (`ActorComponent.Activate` (`self.Audio13`) false)
            (`KismetSystemLibrary.Delay` 1.5)
            (`ActorComponent.Activate` (`self.Audio14`) false)
            (set `self.ChangeNumber_2` false)
            (set `self.Grab?` false)))))
    (:`then_2`
      (set `self.Grab?` true)
      (if (`self.ChangeNumber_3`)
        (`/Engine/EditorBlueprintResources/StandardMacros.DoOnce` false
          (:`Completed`
            (`ActorComponent.Activate` (`self.Audio15`) false)
            (`KismetSystemLibrary.Delay` 16.5)
            (`ActorComponent.Activate` (`self.Audio16`) false)
            (`KismetSystemLibrary.Delay` 10.5)
            (`ActorComponent.Activate` (`self.Audio17`) false)
            (set `self.ChangeNumber_3` false)
            (set `self.Grab?` false)))))))

(event `self.C_GrabComponent.FirstHandDropped`
  (params (`Original Hand Location` :type "Transform Structure") (`Motion Controller` :type "MotionControllerComponent Object Reference") (`Skeletal Mesh Hand` :type "SkeletalMeshComponent Object Reference"))
  (set `self.Grab?` false)
  (`AudioComponent.Stop` (`self.Audio`))
  (`AudioComponent.Stop` (`self.Audio2`))
  (`AudioComponent.Stop` (`self.Audio4`))
  (`AudioComponent.Stop` (`self.Audio3`))
  (`AudioComponent.Stop` (`self.Audio6`))
  (`AudioComponent.Stop` (`self.Audio5`))
  (`AudioComponent.Stop` (`self.Audio13`))
  (`AudioComponent.Stop` (`self.Audio14`))
  (`AudioComponent.Stop` (`self.Audio15`))
  (`AudioComponent.Stop` (`self.Audio12`))
  (`AudioComponent.Stop` (`self.Audio17`))
  (`AudioComponent.Stop` (`self.Audio16`))
  (`AudioComponent.Stop` (`self.Audio8`))
  (`AudioComponent.Stop` (`self.Audio9`))
  (`AudioComponent.Stop` (`self.Audio10`))
  (`AudioComponent.Stop` (`self.Audio11`))
  (`AudioComponent.Stop` (`self.Audio7`)))

(event `self.Call1.OnComponentBeginOverlap`
  (params (OverlappedComponent :type "PrimitiveComponent Object Reference") (OtherActor :type "Actor Object Reference") (OtherComp :type "PrimitiveComponent Object Reference") (OtherBodyIndex :type Integer) (bFromSweep :type Boolean) (SweepResult :type "HitResult Structure (by ref)"))
  (set `self.ChangeNumber` true)
  (set `PrimitiveComponent.bGenerateOverlapEvents` false (`self.Call1`)))

(fn `UserConstructionScript`)