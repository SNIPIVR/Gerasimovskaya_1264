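; VR telephone prop for a scenario, playing one of two scripted calls when the handset is grabbed.
; Grabbing snaps the matching hand onto the handset, which returns to its socket when it leaves the box ungrabbed.
; Call1 and Call2 overlaps arm the calls, each a one-shot chain of delayed audio clips.
; After the second call, nested checks on knife, disconnect and ground-handle actors choose the ending passed to BP_End.
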(event `self.ReceiveBeginPlay`
  (`AudioComponent.Stop` (`self.Audio`))
  (`AudioComponent.Stop` (`self.Audio2`))
  (`AudioComponent.Stop` (`self.Audio4`))
  (`AudioComponent.Stop` (`self.Audio3`))
  (`AudioComponent.Stop` (`self.Audio6`))
  (`AudioComponent.Stop` (`self.Audio5`))
  (`SceneComponent.K2_AttachToComponent` (`self.old_telephone__3__hanger`) (`self.Box`) "Phone_1" "SnapToTarget" "SnapToTarget" "KeepWorld" true :!label _label))

(event `self.Call1.OnComponentBeginOverlap`
  (params (OverlappedComponent :type "PrimitiveComponent Object Reference") (OtherActor :type "Actor Object Reference") (OtherComp :type "PrimitiveComponent Object Reference") (OtherBodyIndex :type Integer) (bFromSweep :type Boolean) (SweepResult :type "HitResult Structure (by ref)"))
  (set `self.ChangeNumber` true)
  (set `PrimitiveComponent.bGenerateOverlapEvents` false (`self.Call1`)))

(event `self.Box.OnComponentEndOverlap`
  (params (OverlappedComponent :type "PrimitiveComponent Object Reference") (OtherActor :type "Actor Object Reference") (OtherComp :type "PrimitiveComponent Object Reference") (OtherBodyIndex :type Integer))
  (if (not (`self.Grab?`))
    (goto _label)))

(event `self.Call2.OnComponentBeginOverlap`
  (params (OverlappedComponent :type "PrimitiveComponent Object Reference") (OtherActor :type "Actor Object Reference") (OtherComp :type "PrimitiveComponent Object Reference") (OtherBodyIndex :type Integer) (bFromSweep :type Boolean) (SweepResult :type "HitResult Structure (by ref)"))
  (set `self.ChangeNumber_2` true)
  (set `self.ChangeNumber` false)
  (set `PrimitiveComponent.bGenerateOverlapEvents` false (`self.Call2`)))

(event `self.C_GrabComponent.FirstHandGrabbed`
  (params (`Motion Controller` :type "MotionControllerComponent Object Reference") (SkeltalMeshHand :type "SkeletalMeshComponent Object Reference") (`Motion Controller Aim` :type "MotionControllerComponent Object Reference"))
  (if (== (`MotionControllerComponent.MotionSource` `Motion Controller`) "Left")
    (message `/Game/GDXR_VR_Template/Blueprints/Interfaces/BPI_HandSnapping.SnapHandPosition` (`ChildActorComponent.ChildActor` (`self.HandLeft`)) SkeltalMeshHand null)
    (else
      (message `/Game/GDXR_VR_Template/Blueprints/Interfaces/BPI_HandSnapping.SnapHandPosition` (`ChildActorComponent.ChildActor` (`self.HandRight`)) SkeltalMeshHand null)))
  (`SceneComponent.SetRelativeScale3D` (`self.old_telephone__3__hanger`) (1.5 1.5 1.5))
  (`|ExecutionSequence`
    (:`then_0`
      (set `self.Grab?` true)
      (if (`self.ChangeNumber`)
        (`/Engine/EditorBlueprintResources/StandardMacros.DoOnce` false
          (:`Completed`
            (`ActorComponent.Activate` (`self.Audio`) false)
            (`KismetSystemLibrary.Delay` 16.0)
            (`ActorComponent.Activate` (`self.Audio2`) false)
            (`KismetSystemLibrary.Delay` 12.5)
            (`ActorComponent.Activate` (`self.Audio3`) false)
            (`KismetSystemLibrary.Delay` 11.5)
            (`ActorComponent.Activate` (`self.Audio4`) false)
            (set `self.ChangeNumber` false)
            (set `self.Grab?` false)))))
    (:`then_1`
      (set `self.Grab?` true)
      (if (`self.ChangeNumber_2`)
        (`/Engine/EditorBlueprintResources/StandardMacros.DoOnce` false
          (:`Completed`
            (`ActorComponent.Activate` (`self.Audio5`) false)
            (`KismetSystemLibrary.Delay` 16.0)
            (`ActorComponent.Activate` (`self.Audio6`) false)
            (`KismetSystemLibrary.Delay` 11.0)
            (set `self.ChangeNumber_2` false)
            (set `self.Grab?` false)
            (bind _asbp_end (cast `/Game/BP/Blueprints/UI/EndMenu/BP_End` (`self.BP END`)))
            (bind _as3_1_a3 (cast `/Game/BP/DisconnectKnives/3_1_A3` (`self.3 1 A3`)))
            (if (`/Game/BP/DisconnectKnives/3_1_A3.WorkKnives?` _as3_1_a3)
              (bind _asdisconnect_knives (cast `/Game/BP/DisconnectKnives/DisconnectKnives` (`self.DisconectKnives`)))
              (if (`/Game/BP/DisconnectKnives/DisconnectKnives.IsWork?` _asdisconnect_knives)
                (bind _ashandle_ground (cast `/Game/cupboard/Ground_Handle/Handle_Ground` (`self.Handle_Ground`)))
                (if (`/Game/cupboard/Ground_Handle/Handle_Ground.EndScenar` _ashandle_ground)
                  (`/Game/BP/Blueprints/UI/EndMenu/BP_End.ScenarEnd` _asbp_end "NewEnumerator24")
                  (else
                    (`/Game/BP/Blueprints/UI/EndMenu/BP_End.ScenarEnd` _asbp_end "NewEnumerator5")))
                (else
                  (`/Game/BP/Blueprints/UI/EndMenu/BP_End.ScenarEnd` _asbp_end "NewEnumerator4")))
              (else
                (`/Game/BP/Blueprints/UI/EndMenu/BP_End.ScenarEnd` _asbp_end "NewEnumerator3")))))))))

(event `self.C_GrabComponent.FirstHandDropped`
  (params (`Original Hand Location` :type "Transform Structure") (`Motion Controller` :type "MotionControllerComponent Object Reference") (`Skeletal Mesh Hand` :type "SkeletalMeshComponent Object Reference"))
  (set `self.Grab?` false))

(fn `UserConstructionScript`)